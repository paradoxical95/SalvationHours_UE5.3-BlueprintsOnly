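; Base weapon actor for the player's M4 and Glock, configured from DT_WeaponInfo by switch index.
; Socket-snapped sights, suppressor, grip, flashlight and laser are gated by per-weapon flags and restored from an async save load on switching to the rifle.
; Optics set the active view socket and FOV, with Acog scope toggling delegated to its child actor.
; Events drive firing and reload animations, suppressor-aware sound, shell ejection, smoke and muzzle flash.
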(event Custom|Event_EjectBulletShell
  (bind _weaponmesh (Variables|Default|GetWeaponMesh))
  (bind _socket_ejectshells (Variables|SOCKETS|GetSocket_EjectShells))
  (bind _returnvalue (Utilities|String|StringToName _socket_ejectshells))
  (bind _returnvalue_2 (Transformation|GetSocketTransform _weaponmesh _returnvalue "RTS_World"))
  ;[1 1 1] Bullet Shell Ejection
  (bind _returnvalue_3 (Game|SpawnActorfromClass "/Game/_Main/Blueprints/BulletStuff/BP_BulletShell.BP_BulletShell_C" (Math|Transform|MakeTransform (.location _returnvalue_2) (.rotation _returnvalue_2) (select (== (Variables|Default|GetWeaponSwitch) 1) "0.750000,0.750000,0.754000" (.scale _returnvalue_2))) "Undefined" "OverrideRootScale" self 0))
  (Physics|SetSimulatePhysics (Variables|/Game/_Main/Blueprints/BulletStuff/BP_BulletShell.BP_BulletShell_C|GetShell_Mesh _returnvalue_3) true)
  (Physics|AddImpulse (Variables|/Game/_Main/Blueprints/BulletStuff/BP_BulletShell.BP_BulletShell_C|GetShell_Mesh _returnvalue_3) (+ (* (Math|Vector|GetForwardVector (Variables|/Game/_Main/Blueprints/BulletStuff/BP_BulletShell.BP_BulletShell_C|GetShell_Mesh _returnvalue_3)) (Math|Random|RandomFloatinRange 1.0 3.0)) (* (Math|Vector|GetRightVector (Variables|/Game/_Main/Blueprints/BulletStuff/BP_BulletShell.BP_BulletShell_C|GetShell_Mesh _returnvalue_3)) (Math|Random|RandomFloatinRange -3.0 -1e+01))) "None" false)
  (Utilities|FlowControl|Delay 5.0)
  (Actor|DestroyActor _returnvalue_3))

(event Custom|Event_PlayFireMontageWeapon
  ;[1 1 1] Sound and Montage
  (Components|Animation|PlayAnimation (Variables|Default|GetWeaponMesh) (Utilities|Struct|BreakS_WeaponInfo (Variables|STRUCTS|GetWeaponInfo)) false))

(event Custom|Event_PlayWeaponFireSound
  (bind _returnvalue (Transformation|GetActorLocation))
  (bind _weaponinfo (Variables|STRUCTS|GetWeaponInfo))
  (bind (_weaponfiresound _weaponfiresuppressedsound) (Utilities|Struct|BreakS_WeaponInfo _weaponinfo))
  ;[1 1 1] Sound and Montage
  (if (not (Variables|Default|GetSuppressorAttached?))
    (Audio|PlaySoundatLocation _weaponfiresound _returnvalue "0, 0, 0" 1.0 1.0 0.0 0 0 0 0)
    (else
      (Audio|PlaySoundatLocation _weaponfiresuppressedsound _returnvalue "0, 0, 0" 1.0 1.0 0.0 0 0 0 0))))

(event Custom|Event_SpawnBarrelSmoke
  (bind _barrelsmoke_ns (Variables|Default|GetBarrelSmoke_NS))
  ;[1 1 1] Barrel Smoke
  (Transformation|AttachComponentToComponent _barrelsmoke_ns (Variables|Default|GetWeaponMesh) (Utilities|String|StringToName (Variables|SOCKETS|GetSocket_Shooting)) "SnapToTarget" "SnapToTarget" "SnapToTarget" true)
  (Components|Activation|Activate _barrelsmoke_ns false)
  (Utilities|FlowControl|Delay 5.0)
  (Components|Activation|Deactivate _barrelsmoke_ns))

(event Custom|Event_SpawnBurstSmoke
  (bind _burstsmoke_ns (Variables|Default|GetBurstSmoke_NS))
  ;[1 1 1] Burst Smoke
  (Transformation|AttachComponentToComponent _burstsmoke_ns (Variables|Default|GetWeaponMesh) (Utilities|String|StringToName (Variables|SOCKETS|GetSocket_SmokeBurst)) "SnapToTarget" "SnapToTarget" "SnapToTarget" true)
  (Components|Activation|Activate _burstsmoke_ns false)
  (Utilities|FlowControl|Delay 1.5)
  (Components|Activation|Deactivate _burstsmoke_ns))

(event Custom|Event_SpawnMuzzleFlash
  (bind _weaponmesh (Variables|Default|GetWeaponMesh))
  (bind _muzzleflashlight (Variables|Default|GetMuzzleFlashLight))
  (bind _socket_muzzleflash (Variables|SOCKETS|GetSocket_MuzzleFlash))
  (bind _returnvalue (Utilities|String|StringToName _socket_muzzleflash))
  (bind _returnvalue_2 (Transformation|GetSocketTransform _weaponmesh _returnvalue "RTS_World"))
  ;[1 1 1] MuzzleFlash
  (Transformation|AttachComponentToComponent _muzzleflashlight (Variables|Default|GetWeaponMesh) (Utilities|String|StringToName (Variables|SOCKETS|GetSocket_MuzzleFlash)) "SnapToTarget" "SnapToTarget" "SnapToTarget" true)
  (Rendering|SetVisibility _muzzleflashlight true false)
  (Utilities|FlowControl|Delay 0.15)
  (Rendering|SetVisibility _muzzleflashlight false false)
  (Effects|SpawnEmitteratLocation "/Game/MilitaryWeapDark/FX/P_AssaultRifle_MuzzleFlash.P_AssaultRifle_MuzzleFlash" (.location _returnvalue_2) (.rotation _returnvalue_2)))

(event Custom|Event_PlayReloadMontageWeapon
  (bind _weaponinfo (Variables|STRUCTS|GetWeaponInfo))
  (bind _weaponreloadmontage (Utilities|Struct|BreakS_WeaponInfo _weaponinfo))
  ;[1 1 1] Sound and Montage
  (Utilities|IsValid _weaponreloadmontage
    (:Is%20Valid
      (Components|Animation|PlayAnimation (Variables|Default|GetWeaponMesh) _weaponreloadmontage false))))

(event Custom|Event_HideMagOnWeapon
  (params (MagVisibility :type Boolean))
  ;[1 1 1] Sound and Montage
  (Rendering|SetVisibility (Variables|Default|GetMagazine) MagVisibility false))

(event Custom|Event_LoadRifleStuff
  ;[0.2344 0.1055 0.1266] Event_Load Rifle Attachments
  (bind _returnvalue (SaveGame|CreateSaveGameObject "/Game/_Main/Blueprints/SaveGame/BP_SaveGame_SalvationHours.BP_SaveGame_SalvationHours_C"))
  (bind _output_get (Variables|Default|SetSaveGameInstance _returnvalue))
  (bind _returnvalue_2 (SaveGame|DoesSaveGameExist (Variables|/Game/_Main/Blueprints/SaveGame/BP_SaveGame_SalvationHours.BP_SaveGame_SalvationHours_C|GetSaveSlot_WeaponData _output_get)))
  (if _returnvalue_2
    (bind _savegame (|AsyncLoadGamefromSlot (Variables|/Game/_Main/Blueprints/SaveGame/BP_SaveGame_SalvationHours.BP_SaveGame_SalvationHours_C|GetSaveSlot_WeaponData _output_get))
      (:Completed
        (bind _asbp_save_game_salvation_hours (Utilities|Casting|CastToBP_SaveGame_SalvationHours _savegame))
        (Variables|ENUMs|SetOpticsEnum (.Optic%20Name (Default|GetSavedWeaponData _asbp_save_game_salvation_hours)))
        (CallFunction|UpdateWeaponOptics)
        (CallFunction|AttachCanted (.Canted%20Attached? (Default|GetSavedWeaponData _asbp_save_game_salvation_hours)) false)
        (CallFunction|AttachSuppressor (.Suppressor%20Attached? (Default|GetSavedWeaponData _asbp_save_game_salvation_hours)))
        (if (.Vertical%20Grip%20Attached? (Default|GetSavedWeaponData _asbp_save_game_salvation_hours))
          (CallFunction|AttachVerticalGrip))
        (if (.FlashlightAttached? (Default|GetSavedWeaponData _asbp_save_game_salvation_hours))
          (CallFunction|AttachFlashlight))
        (if (.LaserLightAttached? (Default|GetSavedWeaponData _asbp_save_game_salvation_hours))
          (CallFunction|AttachLaserLight))))))

(event EventBeginPlay
  (CallFunction|PrepareWeaponData false) ; for setting the struct + mesh
  (Variables|ENUMs|SetFiringMode "NewEnumerator0")
  (Collision|SetCollisionEnabled (Variables|Default|GetWeaponMesh) "NoCollision")
  (Rendering|SetVisibility (Variables|Default|GetVerticalGrip) false false)
  (if (Utilities|Struct|BreakS_WeaponInfo (Variables|STRUCTS|GetWeaponInfo))
    (CallFunction|AttachOptictoWeapon (Variables|SOCKETS|GetSocket_Attach_IronSight) (Variables|SOCKETS|GetSocket_View_IronSight) (Variables|Default|GetIronSight) (Variables|FOV|Get1x_FOV))
    (else
      (Variables|SOCKETS|SetCurrentActiveSocket (Variables|SOCKETS|GetSocket_View_IronSight)))))

(fn ConstructionScript)

(fn UpdateWeaponOptics
  (bind _returnvalue (Components|GetOwner))
  (bind _weaponinfo (Variables|STRUCTS|GetWeaponInfo))
  (bind (_ironsightallowed_ _holoallowed_ _reddotallowed_ _acogscopeallowed_) (Utilities|Struct|BreakS_WeaponInfo _weaponinfo))
  (if (Actor|ActorHasTag _returnvalue "Jack")
    (bind _weaponoptic (Class|BPIntJack|SetDesiredOptic(Message) _returnvalue))
    (bind _output_get (Variables|ENUMs|SetOpticsEnum _weaponoptic))
    (switch Utilities|FlowControl|Switch|SwitchonE_Optics _output_get
      (:NewEnumerator0
        (if _ironsightallowed_
          (CallFunction|AttachOptictoWeapon (Variables|SOCKETS|GetSocket_Attach_IronSight) (Variables|SOCKETS|GetSocket_View_IronSight) (Variables|Default|GetIronSight) (Variables|FOV|Get1x_FOV)) ; IronSight
        ))
      (:NewEnumerator1
        (if _holoallowed_
          (CallFunction|AttachOptictoWeapon (Variables|SOCKETS|GetSocket_Attach_Holo) (Variables|SOCKETS|GetSocket_View_Holo) (Variables|Default|GetHolo) (Variables|FOV|Get1x_FOV)) ; Holo
        ))
      (:NewEnumerator2
        (if _reddotallowed_
          (CallFunction|AttachOptictoWeapon (Variables|SOCKETS|GetSocket_Attach_RedDot) (Variables|SOCKETS|GetSocket_View_RedDot) (Variables|Default|GetRedDot) (Variables|FOV|Get1x_FOV)) ; Red Dot
        ))
      (:NewEnumerator3
        (if _acogscopeallowed_ ; because of Struct Update
          (CallFunction|AttachOptictoWeapon (Variables|SOCKETS|GetSocket_Attach_Acog) (Variables|SOCKETS|GetSocket_View_Acog) (Variables|Default|GetAcog) (Variables|FOV|GetAcog_FOV)) ; Acog
        )))))

(fn AttachOptictoWeapon
  (params (AttachSocketName :type String) (ViewSocketName :type String) (Target%20Optic%20Actor :type Scene%20Component%20Object%20Reference) (NewFOV_ForOptic :type Float%20%28double-precision%29))
  (Variables|SOCKETS|SetCurrentActiveSocket ViewSocketName)
  (Variables|FOV|SetNewFOV_ForOptic NewFOV_ForOptic)
  (Utilities|IsValid Target%20Optic%20Actor
    (:Is%20Valid
      (Rendering|SetVisibility Target%20Optic%20Actor true false)
      (Transformation|AttachComponentToComponent Target%20Optic%20Actor (Variables|Default|GetWeaponMesh) (Utilities|String|StringToName AttachSocketName) "SnapToTarget" "SnapToTarget" "SnapToTarget" true)
      (if (Components|ComponentHasTag Target%20Optic%20Actor "Holo")
        (Rendering|SetVisibility (Variables|Default|GetAcog) false false)
        (elif (Components|ComponentHasTag Target%20Optic%20Actor "RedDot")
          (Rendering|SetVisibility (Variables|Default|GetHolo) false false)
          (elif (Components|ComponentHasTag Target%20Optic%20Actor "Acog")
            (Rendering|SetVisibility (Variables|Default|GetHolo) false false)
            (elif (Components|ComponentHasTag Target%20Optic%20Actor "IronSight")
              (Rendering|SetVisibility (Variables|Default|GetHolo) false false))))))))

(fn AttachCanted
  (params (Attach? :type Boolean) (SwitchSocket :type Boolean))
  (if (Utilities|Struct|BreakS_WeaponInfo (Variables|STRUCTS|GetWeaponInfo))
    (if Attach?
      (Variables|FOV|SetNewFOV_ForOptic 2e+01)
      (Transformation|AttachComponentToComponent (Variables|Default|GetCantedSight) (Variables|Default|GetWeaponMesh) (Utilities|String|StringToName (Variables|SOCKETS|GetSocket_Attach_Canted)) "SnapToTarget" "SnapToTarget" "SnapToTarget" true)
      (Rendering|SetVisibility (Variables|Default|GetCantedSight) true false)
      (Variables|Default|SetCantedAttached? true)
      (else
        (Rendering|SetVisibility (Variables|Default|GetCantedSight) false false)
        (Variables|Default|SetCantedAttached? false)))
    (if SwitchSocket
      (Variables|SOCKETS|SetCurrentActiveSocket (Variables|SOCKETS|GetSocket_View_Canted))
      (else
        (Variables|SOCKETS|SetCurrentActiveSocket (Variables|SOCKETS|GetCurrentActiveSocket))
        (Variables|FOV|SetNewFOV_ForOptic 1e+01)))))

(fn AttachSuppressor
  (params (EnableSuppressor :type Boolean))
  (bind _output_get (Variables|Default|SetSuppressorAttached? EnableSuppressor))
  (Transformation|AttachComponentToComponent (Variables|Default|GetSuppressor) (Variables|Default|GetWeaponMesh) (Utilities|String|StringToName (Variables|SOCKETS|GetSocket_Attach_Suppressor)) "SnapToTarget" "SnapToTarget" "SnapToTarget" true)
  (Rendering|SetVisibility (Variables|Default|GetSuppressor) _output_get false))

(fn AttachVerticalGrip
  (if (not (Rendering|IsVisible (Variables|Default|GetVerticalGrip)))
    (if (Utilities|Struct|BreakS_WeaponInfo (Variables|STRUCTS|GetWeaponInfo))
      (Transformation|AttachComponentToComponent (Variables|Default|GetVerticalGrip) (Variables|Default|GetWeaponMesh) (Utilities|String|StringToName (Variables|SOCKETS|GetSocket_Attach_VerticalGrip)) "SnapToTarget" "SnapToTarget" "SnapToTarget" true)
      (Rendering|SetVisibility (Variables|Default|GetVerticalGrip) true false)
      (Variables|Default|SetIsVerticalGripAttached? true))))

(fn AttachFlashlight
  (bind _flashlight (Variables|Default|GetFlashlight))
  (if (Utilities|Struct|BreakS_WeaponInfo (Variables|STRUCTS|GetWeaponInfo))
    (Transformation|AttachComponentToComponent _flashlight (Variables|Default|GetWeaponMesh) (Utilities|String|StringToName (Variables|SOCKETS|GetSocket_Attach_Flashlight)) "SnapToTarget" "SnapToTarget" "SnapToTarget" true)
    (Rendering|SetVisibility _flashlight true false)
    (Variables|Default|SetFlashlightAttached? true)))

(fn AttachLaserLight
  (bind _laserlight (Variables|Default|GetLaserLight))
  (if (Utilities|Struct|BreakS_WeaponInfo (Variables|STRUCTS|GetWeaponInfo))
    (Transformation|AttachComponentToComponent _laserlight (Variables|Default|GetWeaponMesh) (Utilities|String|StringToName (Variables|SOCKETS|GetSocket_Attach_LaserLight)) "SnapToTarget" "SnapToTarget" "SnapToTarget" true)
    (Rendering|SetVisibility _laserlight true false)
    (Variables|Default|SetLaserLightAttached? true)))

(fn PrepareWeaponData
  (params (ForWeaponSwitching? :type Boolean))
  (bind _magazine (Variables|Default|GetMagazine))
  (bind _returnvalue (Utilities|GetDataTableRow "/Game/_Main/Blueprints/DataTables/DT_WeaponInfo.DT_WeaponInfo" (Utilities|Array|Get(acopy) (Variables|Default|GetRowName_DT) (Variables|Default|GetWeaponSwitch)))
    (:then
      (bind _output_get (Variables|STRUCTS|SetWeaponInfo _returnvalue))
      (Components|SkinnedMesh|SetSkinnedAssetandUpdate (Variables|Default|GetWeaponMesh) (.WeaponMesh (Utilities|Struct|BreakS_WeaponInfo _output_get)) false)
      ;[0.2344 0.2344 0.2344 1 12] MagazineBP
      (bind _asbp_magazine (Utilities|Casting|CastToBP_Magazine (Variables|/Script/Engine.ChildActorComponent|GetChildActor _magazine)))
      (Variables|Default|SetMagazineBP_Ref _asbp_magazine)
      (Transformation|AttachComponentToComponent _magazine (Variables|Default|GetWeaponMesh) (Utilities|String|StringToName (Variables|SOCKETS|GetSocket_Magazine)) "SnapToTarget" "SnapToTarget" "SnapToTarget" true)
      (Default|EventSetMagazineMesh (Variables|Default|GetMagazineBP_Ref) (.MagazineMesh (Utilities|Struct|BreakS_WeaponInfo _output_get)))
      (if (== (Variables|Default|GetWeaponSwitch) 1)
        (Rendering|SetVisibility (Variables|Default|GetVerticalGrip) false false)
        (Variables|SOCKETS|SetCurrentActiveSocket (Variables|SOCKETS|GetSocket_View_IronSight))
        (Variables|FOV|SetNewFOV_ForOptic 5.0) ; -5 offset value now\nso no more 85 here
        (Variables|Default|SetIsVerticalGripAttached? false)
        (elif ForWeaponSwitching?
          (CallFunction|EventLoadRifleStuff))))))

(fn ScopeinOutToggle
  (params (IsInADS? :type Boolean) (ScopeInMode :type E_ScopeInMode%20Enum :default "NewEnumerator0") (IsCantedOn? :type Boolean))
  (bind _acog (Variables|Default|GetAcog))
  (if (not IsCantedOn?)
    (bind _output_get (Variables|Default|SetScope%20in%20Mode ScopeInMode))
    (if (.AcogScopeAllowed? (Utilities|Struct|BreakS_WeaponInfo (Variables|STRUCTS|GetWeaponInfo)))
      (if (Rendering|IsVisible _acog)
        (bind _asbp_c_acog (Utilities|Casting|CastToBP_C_Acog (Variables|/Script/Engine.ChildActorComponent|GetChildActor _acog)))
        (Default|ScopeinOut _asbp_c_acog IsInADS? _output_get)
        (switch Utilities|FlowControl|Switch|SwitchonE_ScopeInMode _output_get ; bcz of this I save performance\nSCC2D only visible when Aiming in PIP\nelse its hidden
          (:NewEnumerator0
            (CallFunction|UpdateSocketandFOV (Variables|SOCKETS|GetSocket_View_Acog) (Variables|FOV|GetAcog_FOV))))))))

(fn RemoveAttachments
  (params (Attachment%20Name :type E_WeaponAttachments%20Enum :default "NewEnumerator0"))
  (switch Utilities|FlowControl|Switch|SwitchonE_WeaponAttachments Attachment%20Name
    (:NewEnumerator0
      (CallFunction|AttachCanted false false)
      (Variables|Default|SetCantedAttached? false)
      (Development|PrintString "CantedRemoved"))
    (:NewEnumerator1
      (Rendering|SetVisibility (Variables|Default|GetVerticalGrip) false false)
      (Variables|Default|SetIsVerticalGripAttached? false)
      (Development|PrintString "Vertical Grip Removed"))
    (:NewEnumerator2
      (Rendering|SetVisibility (Variables|Default|GetSuppressor) false false)
      (Variables|Default|SetSuppressorAttached? false)
      (Development|PrintString "Suppressor Removed"))
    (:NewEnumerator3
      (Rendering|SetVisibility (Variables|Default|GetFlashlight) false false)
      (Variables|Default|SetFlashlightAttached? false)
      (Development|PrintString "Flashlight Removed"))
    (:NewEnumerator4
      (Rendering|SetVisibility (Variables|Default|GetLaserLight) false false)
      (Variables|Default|SetLaserLightAttached? false)
      (Development|PrintString "Laser Removed"))))

(fn UpdateSocketandFOV
  (params (CurrentActiveSocket :type String) (NewFOV_ForOptic :type Float%20%28double-precision%29))
  (Variables|SOCKETS|SetCurrentActiveSocket CurrentActiveSocket)
  (Variables|FOV|SetNewFOV_ForOptic NewFOV_ForOptic))

(fn ReplenishWeaponAmmo
  (bind _returnvalue (Utilities|GetDataTableRow "/Game/_Main/Blueprints/DataTables/DT_WeaponInfo.DT_WeaponInfo" (Utilities|Array|Get(acopy) (Variables|Default|GetRowName_DT) (Variables|Default|GetWeaponSwitch)))
    (:then
      (Utilities|Struct|SetmembersinS_WeaponInfo (Variables|STRUCTS|GetWeaponInfo) (.MaxAmmo (Utilities|Struct|BreakS_WeaponInfo _returnvalue)) (.CurrentAmmo (Utilities|Struct|BreakS_WeaponInfo _returnvalue)) (.Magazine1Ammo (Utilities|Struct|BreakS_WeaponInfo _returnvalue)) (.Magazine2Ammo (Utilities|Struct|BreakS_WeaponInfo _returnvalue)) (.Magazine3Ammo (Utilities|Struct|BreakS_WeaponInfo _returnvalue))))))

(fn ToggleFlashlight
  (params (Toggle? :type Boolean))
  (if (Variables|Default|GetFlashlightAttached?)
    (bind _asbp_flashlight_barrel (Utilities|Casting|CastToBP_Flashlight_Barrel (Variables|/Script/Engine.ChildActorComponent|GetChildActor (Variables|Default|GetFlashlight))))
    (Default|ToggleFlashlight _asbp_flashlight_barrel Toggle?)))

(fn ToggleLaserLight
  (params (Toggle? :type Boolean))
  (if (Variables|Default|GetLaserLightAttached?)
    (bind _asbp_laser_light_barrel (Utilities|Casting|CastToBP_LaserLight_Barrel (Variables|/Script/Engine.ChildActorComponent|GetChildActor (Variables|Default|GetLaserLight))))
    (Default|ToggleLaser _asbp_laser_light_barrel Toggle?)))