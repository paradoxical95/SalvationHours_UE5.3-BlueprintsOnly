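; BP_TRBX_PlayCutScene is a trigger box, named for playing cutscenes, that is currently unfinished and plays nothing.
; ChapterSegmentStatus, intended to be called by the GameInstance, stores paused, complete and ongoing segment flags.
; Overlap checks for the "Jack" tag but leads nowhere.
; Disconnected logic would resume voice-over through the GameInstance when paused and not ongoing, then disable collision for one-time use, alongside debug prints.
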(event EventBeginPlay)

(event Collision|EventActorBeginOverlap
  (params (OtherActor :type Actor%20Object%20Reference))
  (if (Actor|ActorHasTag OtherActor "Jack")
    _))

(event EventChapterSegmentStatus
  (params (SegmentPaused? :type Boolean) (SegmentComplete? :type Boolean) (SegmentOnGoing? :type Boolean) (ChapterDataStruct :type S%20Chapter%20Segment%20Data%20Structure))
  (bind _output_get (Variables|Default|SetSegment%20Paused? SegmentPaused?))
  (bind _output_get_2 (Variables|Default|SetSegment%20Complete? SegmentComplete?))
  (bind _output_get_3 (Variables|Default|SetSegment%20on%20Going? SegmentOnGoing?)))

(fn ConstructionScript)