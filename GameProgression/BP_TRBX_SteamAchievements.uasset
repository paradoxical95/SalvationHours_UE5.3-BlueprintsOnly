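; Trigger volume actor that unlocks one Steam achievement, chosen by its AchievementName enum, when the actor tagged "Jack" lingers inside.
; On BeginPlay it reads achievement data through the GameInstance and removes itself if that achievement is already unlocked.
; Overlap runs a looping one-second timer whose count persists across exits.
; After about five seconds total, it sends the unlock message to the GameInstance, then destroys itself.
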(event OnComponentBeginOverlap(CollisionComponent)
  (params (OverlappedComponent :type Primitive%20Component%20Object%20Reference) (OtherActor :type Actor%20Object%20Reference) (OtherComp :type Primitive%20Component%20Object%20Reference) (OtherBodyIndex :type Integer) (bFromSweep :type Boolean) (SweepResult :type Hit%20Result%20Structure%20%28by%20ref%29))
  (if (Actor|ActorHasTag OtherActor "Jack")
    (Variables|Default|SetIsColliding? true)
    (bind _returnvalue (Utilities|Time|SetTimerbyEvent (delegate Custom|CE_CheckAndUnlockAchievement) 1.0 true))
    (Variables|Default|SetTimerHandle _returnvalue)))

(event OnComponentEndOverlap(CollisionComponent)
  (params (OverlappedComponent :type Primitive%20Component%20Object%20Reference) (OtherActor :type Actor%20Object%20Reference) (OtherComp :type Primitive%20Component%20Object%20Reference) (OtherBodyIndex :type Integer))
  (if (Actor|ActorHasTag OtherActor "Jack")
    (Variables|Default|SetIsColliding? false)
    (Utilities|Time|ClearandInvalidateTimerbyHandle (Variables|Default|GetTimerHandle))))

(event Custom|CE_CheckAndUnlockAchievement
  (if (Variables|Default|GetIsColliding?)
    (bind _output_get (Variables|Default|SetTempInt (+ (Variables|Default|GetTempInt) 1)))
    (if (> _output_get 4)
      (Development|PrintString (Utilities|String|Append "Achievement Unclocked -> " (Utilities|String|ToString(Name) (Utilities|Select :Index (Variables|Default|GetAchievementName) :NewEnumerator0 "Arrival" :NewEnumerator1 "Annex" :NewEnumerator2 "Ambush" :NewEnumerator3 "FastHands" :NewEnumerator4 "WeaponsFree" :NewEnumerator5 "Counterplay" :NewEnumerator6 "Wounds" :NewEnumerator7 "UpCloseAndPersonal" :NewEnumerator8 "NoEasterEgg" :NewEnumerator9 "Prophet" :NewEnumerator10 "NoDeaths" :NewEnumerator11 "TenDeaths"))))
      (Utilities|Time|ClearandInvalidateTimerbyHandle (Variables|Default|GetTimerHandle))
      (Variables|Default|SetIsColliding? false)
      (Class|BPIntGameInstance|GIUnlockSteamAchievements(Message) (Game|GetGameInstance) (Variables|Default|GetAchievementName))
      (Utilities|FlowControl|Delay 2.0)
      (Actor|DestroyActor))))

(event EventBeginPlay
  (bind _achievementdata (Class|BPIntGameInstance|GIFetchAchievementData(Message) (Game|GetGameInstance)))
  (if (.Unlocked? (Utilities|Struct|BreakS_SteamAchievements (Utilities|Array|Get(acopy) _achievementdata (Utilities|Select :Index (Variables|Default|GetAchievementName) :NewEnumerator0 0 :NewEnumerator1 1 :NewEnumerator2 2 :NewEnumerator3 3 :NewEnumerator4 4 :NewEnumerator5 5 :NewEnumerator6 6 :NewEnumerator7 7 :NewEnumerator8 8 :NewEnumerator9 9 :NewEnumerator10 10 :NewEnumerator11 11))))
    (Utilities|FlowControl|Delay 3.0)
    (Actor|DestroyActor)))

(fn ConstructionScript)