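; Trigger box that resumes a paused voice-over segment when the player character or vehicle overlaps it.
; The GameInstance supplies paused, complete and ongoing segment states, and a flag chooses whether the Vehicle or Jack actor tag triggers it.
; When paused and not ongoing, it calls the GameInstance to resume the VO, then disables its collision so it fires once per session, with debug printing.
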(event EventBeginPlay)

(event Collision|EventActorBeginOverlap
  (params (OtherActor :type Actor%20Object%20Reference))
  (if (select (Variables|Default|GetResumeViaVehicle?) (Actor|ActorHasTag OtherActor "Vehicle") (Actor|ActorHasTag OtherActor "Jack"))
    ;[0.1035 0.2344 0.2157 1 13] Then Check the variables provided by GameInstance
    (if (Variables|Default|GetSegment%20Paused?)
      (if (not (Variables|Default|GetSegment%20on%20Going?))
        (Class|BPIntGameInstance|GIResumeVOAfterPause(Message) (Game|GetGameInstance))
        (Collision|SetCollisionEnabled (Variables|Default|GetCollisionComponent) "NoCollision") ; bcz of this, one TBox can only fire once during one session
        (Development|PrintString (Utilities|String|Append "Resumed via Trigger Box - 
" (Utilities|GetDisplayName self)) true true "(R=1.000000,G=0.000000,B=0.581583,A=1.000000)" 5.0)))))

(event EventChapterSegmentStatus
  (params (SegmentPaused? :type Boolean) (SegmentComplete? :type Boolean) (SegmentOnGoing? :type Boolean) (ChapterDataStruct :type S%20Chapter%20Segment%20Data%20Structure))
  (bind _output_get (Variables|Default|SetSegment%20Paused? SegmentPaused?))
  (bind _output_get_2 (Variables|Default|SetSegment%20Complete? SegmentComplete?))
  (bind _output_get_3 (Variables|Default|SetSegment%20on%20Going? SegmentOnGoing?)))

(fn ConstructionScript)