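; Chapter 6 gun pickup that appears as either Drew's pistol or Jim's rifle, chosen by a flag and previewed through the construction script.
; A sphere overlap toggles the interact prompt for the Jack-tagged actor and marks it in range.
; The PickupsCH6Guns event, when in range, notifies the GameInstance so progression resumes once both are picked, plays the ammo sound, hides the mesh and destroys itself after a delay.
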(event OnComponentBeginOverlap(Sphere)
  (params (OverlappedComponent :type Primitive%20Component%20Object%20Reference) (OtherActor :type Actor%20Object%20Reference) (OtherComp :type Primitive%20Component%20Object%20Reference) (OtherBodyIndex :type Integer) (bFromSweep :type Boolean) (SweepResult :type Hit%20Result%20Structure%20%28by%20ref%29))
  (if (Actor|ActorHasTag OtherActor "Jack")
    (Class|BPIntJack|ToggleInteractPromptPlayer(Message) OtherActor true)
    (Variables|Default|SetInRange? true)))

(event OnComponentEndOverlap(Sphere)
  (params (OverlappedComponent :type Primitive%20Component%20Object%20Reference) (OtherActor :type Actor%20Object%20Reference) (OtherComp :type Primitive%20Component%20Object%20Reference) (OtherBodyIndex :type Integer))
  (if (Actor|ActorHasTag OtherActor "Jack")
    (Class|BPIntJack|ToggleInteractPromptPlayer(Message) OtherActor false)
    (Variables|Default|SetInRange? false)))

(event EventBeginPlay
  (bind _drewpistol_ (Variables|Default|GetDrewPistol?))
  (Rendering|SetVisibility (Variables|Default|GetDrew_Pistol) _drewpistol_ false)
  (Rendering|SetVisibility (Variables|Default|GetJim_Rifle) (not _drewpistol_) false))

(event EventPickupsCH6Guns
  (if (Variables|Default|GetInRange?)
    (Class|BPIntGameInstance|GIPickupGunsCH6(Message) (Game|GetGameInstance)) ; Notify the GI \nSo resume only when both are picked
    (if (Variables|Default|GetDrewPistol?)
      (Audio|PlaySound2D "/Game/MilitaryWeapDark/Sound/Pistol/Wavs/Pistol_AmmoPickup.Pistol_AmmoPickup" 1.0 1.0 0.0 0 0)
      (Rendering|SetVisibility (Variables|Default|GetDrew_Pistol) false false)
      (else
        (Audio|PlaySound2D "/Game/MilitaryWeapDark/Sound/Rifle/Wavs/Rifle_AmmoPickup.Rifle_AmmoPickup" 1.0 1.0 0.0 0 0)
        (Rendering|SetVisibility (Variables|Default|GetJim_Rifle) false false)))
    (Utilities|FlowControl|Delay 5.0)
    (Actor|DestroyActor)))

(fn ConstructionScript
  (bind _drewpistol_ (Variables|Default|GetDrewPistol?))
  (Rendering|SetVisibility (Variables|Default|GetDrew_Pistol) _drewpistol_ false)
  (Rendering|SetVisibility (Variables|Default|GetJim_Rifle) (not _drewpistol_) false))

(fn FetchArrowsfromVehicles
  (params (Seat :type E_VehicleSeat%20Enum :default "NewEnumerator0"))
  (return "0, 0, 0" "0, 0, 0"))

(fn GetVehicleNameandLoc
  (return "NewEnumerator0" "0, 0, 0" "0, 0, 0"))

(fn IsVehicleMoving?
  (return false))

(fn ObtainTrunkArrowsPickup
  (params (Seat%281-6%29 :type Integer))
  (return "0, 0, 0" "0, 0, 0"))

(fn PlayerDependentLight?
  (return false))