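; Blueprint Interface for the Game Instance, declaring the calls that other objects use to reach game-wide progression and persistence.
; Progression calls cover chapters and segments, tasks, dialogue, soundtrack, level loading, enemy spawning and tracking, chapter-specific pickups and events, and Steam achievements.
; Other calls pass player, NPC, vehicle and spline references, save and load world data, and save or fetch visual, audio, control and upscaler settings.
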(fn GetPlayerRef
  (params (JackRef :type Character%20Object%20Reference)))

(fn GetNPCRef
  (params (NPC_Character :type Character%20Object%20Reference) (NPC_CharacterName :type E_CharacterNames%20Enum :default "NewEnumerator0")))

(fn GISetChapterandSegment
  (params (ChapterNumber :type E_ChapterNumber%20Enum :default "NewEnumerator0") (CH1_Seg :type E_Chapter1_Segments%20Enum :default "NewEnumerator2") (CH2_Seg :type E_Chapter2_Segments%20Enum :default "NewEnumerator6") (CH3_Seg :type E_Chapter3_Segments%20Enum :default "NewEnumerator6") (CH4_Seg :type E_Chapter4_Segments%20Enum :default "NewEnumerator15") (CH5_Seg :type E_Chapter5_Segments%20Enum :default "NewEnumerator15") (CH6_Seg :type E_Chapter6_Segments%20Enum :default "NewEnumerator15")))

(fn GIPlayDialoguesActual)

(fn GIResumeVOAfterPause)

(fn GITaskUpdate
  (params (Completed? :type Boolean) (TaskNumber :type Integer)))

(fn GetVehicleRef
  (params (VehicleRef :type Actor%20Object%20Reference) (VehicleType :type E_VehicleName%20Enum :default "NewEnumerator0")))

(fn GIGetSplineReferencesfromLevel
  (params (SplineRef :type BP%20Spline%20Vehicle%20Object%20Reference) (ChapterNumber :type E_ChapterNumber%20Enum :default "NewEnumerator0") (Ch1%20Seg :type E_Chapter1_Segments%20Enum :default "NewEnumerator2") (Ch2%20Seg :type E_Chapter2_Segments%20Enum :default "NewEnumerator6") (Ch3%20Seg :type E_Chapter3_Segments%20Enum :default "NewEnumerator6") (Ch4%20Seg :type E_Chapter4_Segments%20Enum :default "NewEnumerator15") (Ch5%20Seg :type E_Chapter5_Segments%20Enum :default "NewEnumerator15") (Ch6%20Seg :type E_Chapter6_Segments%20Enum :default "NewEnumerator15")))

(fn GITransferSplineDatatoVehicle
  (params (WhichVehicle :type E_VehicleName%20Enum :default "NewEnumerator0")))

(fn GISmoothLoadLevel
  (params (LevelSelector :type Integer)))

(fn GISpawnEnemiesatLocation
  (params (SpawnTargetPoint :type Target%20Point%20Object%20Reference) (Amount :type Integer) (MovementTargetPoints :type Array%20of%20Target%20Point%20Object%20References)))

(fn GITrackDeadEnemies
  (params (Amount :type Integer)))

(fn GICH4PickupBag
  (params (DuffelBagPicked? :type Boolean)))

(fn GICH4PickupHDD
  (params (HardDrivePicked? :type Boolean)))

(fn GITrackDestroyedAnnexLights)

(fn GILaserLassoSeqDone)

(fn GIPickupGunsCH6)

(fn GIPickupBelongingsCH6)

(fn GIPickupMilitaryBagCH6)

(fn GIShowCurrentTaskforPlayer
  (params (Toggle? :type Boolean)))

(fn GISaveGameWorldData)

(fn GILoadGameWorldData)

(fn GIAutoSaveData
  (params (SaveVehicleLoc? :type Boolean) (SavePoint :type E_SavePoints%20Enum :default "NewEnumerator0") (Map :type E_LevelMap%20Enum :default "NewEnumerator0")))

(fn GIFetchChapterSegment
  (return ""))

(fn GISaveNPCLocData
  (params (NPC_Name :type E_CharacterNames%20Enum :default "NewEnumerator0") (NPC_Location :type Vector) (NPC_Rotation :type Rotator)))

(fn GIResetSavesforNewGame)

(fn GIResumeAfterDeath
  (params (ResumeFromDeath :type Boolean)))

(fn GIFetchCurrentTaskText
  (return ""))

(fn GISaveDataVisuals
  (params (SoftwareLumen? :type Boolean)))

(fn GIFetchDataVisuals
  (return false))

(fn GILoadAllDataMaster)

(fn GIFetchDataAudio
  (return 0.0 0.0 0.0 0.0))

(fn GIFetchDataControls
  (return "NewEnumerator0" false false 0.0 0.0 0.0 0.0 0.0 0.0 false false))

(fn GISaveDataAudio
  (params (AmbientVol :type Float%20%28double-precision%29) (EffectsVol :type Float%20%28double-precision%29) (MusicVol :type Float%20%28double-precision%29) (DialogueVol :type Float%20%28double-precision%29)))

(fn GISaveDataControls
  (params (Difficulty :type E_GameDifficulty%20Enum :default "NewEnumerator0") (X_Invert? :type Boolean) (Y_Invert? :type Boolean) (MouseXSens :type Float%20%28double-precision%29) (MouseYSens :type Float%20%28double-precision%29) (FOV :type Float%20%28double-precision%29) (ACOG_Sens :type Float%20%28double-precision%29) (Gamepad_Horz_Sens :type Float%20%28double-precision%29) (Gamepad_Vert_Sens :type Float%20%28double-precision%29) (Gamepad_Vert_Invert :type Boolean) (WereThumbsticksFlipped? :type Boolean)))

(fn GIChangeSoundtrackState
  (params (SoundtrackState? :type E_SoundtrackStateChange%20Enum :default "NewEnumerator0") (OnlyTogglePlaying? :type Boolean) (ChangeTrackTo :type E_SoundtrackList%20Enum :default "NewEnumerator0")))

(fn GISaveAllStuff)

(fn GISaveDataUpscalers
  (params (UpscalerDataTotal :type S%20Upscaler%20Data%20Total%20Structure)))

(fn GIFetchDataUpscalers
  (return ""))

(fn GIUnlockSteamAchievements
  (params (AchievementName :type E_SteamAchievementsName%20Enum :default "NewEnumerator0")))

(fn GIFetchAchievementData
  (return 0))