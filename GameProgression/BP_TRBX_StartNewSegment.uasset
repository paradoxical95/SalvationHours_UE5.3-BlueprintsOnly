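; Trigger box that starts a configured chapter segment when the player or a vehicle overlaps it.
; The GameInstance pushes segment status and chapter data to it.
; If the current segment is complete and CheckForPreviousChSeg confirms the hard-coded predecessor, it sets the new segment through the GameInstance, plays dialogue and hides Objective-tagged actors.
; It then disables its collision to fire once, until a reset event re-enables it.
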(event Custom|Check_And_Update_ObjMarker
  (bind _chsegstruct (Class|BPIntGameInstance|GIFetchChapterSegment(Message) (Game|GetGameInstance)))
  (if (Utilities|Enum|Equal(Enum) (.ChapterNumber? (Utilities|Struct|BreakS_ChapterSegmentData _chsegstruct)) (Variables|ProgressionVariables|GetChapterNumber))
    (switch Utilities|FlowControl|Switch|SwitchonE_ChapterNumber (Variables|ProgressionVariables|GetChapterNumber)
      (:NewEnumerator0
        (if (Utilities|Enum|Equal(Enum) (Variables|ProgressionVariables|GetChapter1_Segment) (.CH1_Segment (Utilities|Struct|BreakS_ChapterSegmentData _chsegstruct)))
          _))
      (:NewEnumerator1
        (if (Utilities|Enum|Equal(Enum) (.CH2_Segment (Utilities|Struct|BreakS_ChapterSegmentData _chsegstruct)) (Variables|ProgressionVariables|GetChapter2_Segment))
          _))
      (:NewEnumerator2
        (if (Utilities|Enum|Equal(Enum) (.CH3_Segment (Utilities|Struct|BreakS_ChapterSegmentData _chsegstruct)) (Variables|ProgressionVariables|GetChapter3_Segment))
          _))
      (:NewEnumerator3
        (if (Utilities|Enum|Equal(Enum) (.CH4_Segment (Utilities|Struct|BreakS_ChapterSegmentData _chsegstruct)) (Variables|ProgressionVariables|GetChapter4_Segment))
          _))
      (:NewEnumerator4
        (if (Utilities|Enum|Equal(Enum) (.CH5_Segment (Utilities|Struct|BreakS_ChapterSegmentData _chsegstruct)) (Variables|ProgressionVariables|GetChapter5_Segment))
          _)))))

(event Custom|Event_Reset_TRBX_ChapterStarters
  (Collision|SetCollisionEnabled (Variables|Default|GetCollisionComponent) "QueryOnly") ; resetting if need be.\nCreated for Ch4Seg3/4 load from save + Ch4Seg11 reset from death
)

(event EventBeginPlay)

(event Collision|EventActorBeginOverlap
  (params (OtherActor :type Actor%20Object%20Reference))
  (bind _returnvalue (Game|GetGameInstance))
  (bind _chapter6_segment (Variables|ProgressionVariables|GetChapter6_Segment))
  (bind _startviavehicle_ (Variables|Default|GetStartViaVehicle?))
  (bind _chapternumber (Variables|ProgressionVariables|GetChapterNumber))
  (bind _chapter1_segment (Variables|ProgressionVariables|GetChapter1_Segment))
  (bind _chapter2_segment (Variables|ProgressionVariables|GetChapter2_Segment))
  (bind _chapter3_segment (Variables|ProgressionVariables|GetChapter3_Segment))
  (bind _chapter4_segment (Variables|ProgressionVariables|GetChapter4_Segment))
  (bind _chapter5_segment (Variables|ProgressionVariables|GetChapter5_Segment))
  (if (select _startviavehicle_ (Actor|ActorHasTag OtherActor "Vehicle") (Actor|ActorHasTag OtherActor "Jack"))
    (Development|PrintString (select _startviavehicle_ "Vehicle Triggered" "Player Triggered"))
    ;[0.1035 0.2344 0.2157 1 13] Then Check the variables provided by GameInstance
    (if (Variables|Default|GetSegment%20Complete?)
      (if (not (Variables|Default|GetSegment%20on%20Going?))
        (if (CallFunction|CheckforPreviousChSeg)
          (Class|BPIntGameInstance|GISetChapterandSegment(Message) _returnvalue _chapternumber _chapter1_segment _chapter2_segment _chapter3_segment _chapter4_segment _chapter5_segment _chapter6_segment) ; Prime the dialogues
          (Class|BPIntGameInstance|GIPlayDialoguesActual(Message) _returnvalue) ; Play them for Real
          (Development|PrintString (Utilities|String|Append "TRBX Starts -> 
" (Utilities|String|EnumtoString _chapternumber) " 
" (Utilities|String|EnumtoString _chapter1_segment) " 
" (Utilities|String|EnumtoString _chapter2_segment) " 
" (Utilities|String|EnumtoString _chapter3_segment) " 
" (Utilities|String|EnumtoString _chapter4_segment) " 
" (Utilities|String|EnumtoString _chapter5_segment) " 
" (Utilities|String|EnumtoString _chapter6_segment)) true true "(R=1.000000,G=0.249614,B=0.000000,A=1.000000)" 3.0)
          (Collision|SetCollisionEnabled (Variables|Default|GetCollisionComponent) "NoCollision") ; bcz of this, one TBox can only fire once during one session
          (Utilities|Time|ClearandInvalidateTimerbyHandle (Variables|Default|GetTimer))
          ;[1 1 1] This will hide the ObjMarker after triggering the Seg/Ch
          ; No worries since the level BP will un-hide when it updates the marker
          ; there's only 1 object in Benghazi
          (bind _outactors (Actor|GetAllActorswithTag "Objective"))
          (for _array_element _outactors
            (Rendering|SetActorHiddenInGame _array_element true))
          (else
            (Development|PrintString "Chapters Seg 
Don't Match  
For this TRBX" true true "(R=1.000000,G=0.254694,B=0.000000,A=1.000000)" 3.0)))))
    (else
      (Development|PrintString "Collided With NONE"))))

(event EventChapterSegmentStatus
  (params (SegmentPaused? :type Boolean) (SegmentComplete? :type Boolean) (SegmentOnGoing? :type Boolean) (ChapterDataStruct :type S%20Chapter%20Segment%20Data%20Structure))
  (Variables|Default|SetSegment%20Paused? SegmentPaused?)
  (Variables|Default|SetSegment%20Complete? SegmentComplete?)
  (Variables|Default|SetSegment%20on%20Going? SegmentOnGoing?)
  (Variables|Default|SetChapter%20Data%20Struct ChapterDataStruct))

(fn ConstructionScript)

(fn CheckforPreviousChSeg
  (bind _chapter_data_struct (Variables|Default|GetChapter%20Data%20Struct))
  (bind _chapter_data_struct_2 (Variables|Default|GetChapter%20Data%20Struct))
  (bind _chapter_data_struct_3 (Variables|Default|GetChapter%20Data%20Struct))
  (bind _chapter_data_struct_4 (Variables|Default|GetChapter%20Data%20Struct))
  (bind _chapter_data_struct_5 (Variables|Default|GetChapter%20Data%20Struct))
  (bind _chapter_data_struct_6 (Variables|Default|GetChapter%20Data%20Struct))
  (bind _chapter_data_struct_7 (Variables|Default|GetChapter%20Data%20Struct))
  (bind _chapter_data_struct_8 (Variables|Default|GetChapter%20Data%20Struct))
  (bind _chapter_data_struct_9 (Variables|Default|GetChapter%20Data%20Struct))
  (bind _chapter_data_struct_10 (Variables|Default|GetChapter%20Data%20Struct))
  (bind _chapter_data_struct_11 (Variables|Default|GetChapter%20Data%20Struct))
  (bind _chapter_data_struct_12 (Variables|Default|GetChapter%20Data%20Struct))
  (bind _chapter_data_struct_13 (Variables|Default|GetChapter%20Data%20Struct))
  (bind _chapter_data_struct_14 (Variables|Default|GetChapter%20Data%20Struct))
  (bind (_ch5_segment _chapternumber_) (Utilities|Struct|BreakS_ChapterSegmentData _chapter_data_struct))
  (bind (_ch1_segment _chapternumber__2) (Utilities|Struct|BreakS_ChapterSegmentData _chapter_data_struct_9))
  (bind (_ch4_segment _chapternumber__3) (Utilities|Struct|BreakS_ChapterSegmentData _chapter_data_struct_11))
  (bind (_ch5_segment_2 _chapternumber__4) (Utilities|Struct|BreakS_ChapterSegmentData _chapter_data_struct_12))
  (bind (_ch2_segment _chapternumber__5) (Utilities|Struct|BreakS_ChapterSegmentData _chapter_data_struct_13))
  (bind (_ch2_segment_2 _chapternumber__6) (Utilities|Struct|BreakS_ChapterSegmentData _chapter_data_struct_14))
  (bind (_ch2_segment_3 _chapternumber__7) (Utilities|Struct|BreakS_ChapterSegmentData _chapter_data_struct_2))
  (bind (_ch2_segment_4 _chapternumber__8) (Utilities|Struct|BreakS_ChapterSegmentData _chapter_data_struct_3))
  (bind (_ch3_segment _chapternumber__9) (Utilities|Struct|BreakS_ChapterSegmentData _chapter_data_struct_4))
  (bind (_ch3_segment_2 _chapternumber__10) (Utilities|Struct|BreakS_ChapterSegmentData _chapter_data_struct_5))
  (bind (_ch4_segment_2 _chapternumber__11) (Utilities|Struct|BreakS_ChapterSegmentData _chapter_data_struct_6))
  (bind (_ch4_segment_3 _chapternumber__12) (Utilities|Struct|BreakS_ChapterSegmentData _chapter_data_struct_7))
  (bind (_ch4_segment_4 _chapternumber__13) (Utilities|Struct|BreakS_ChapterSegmentData _chapter_data_struct_8))
  (bind (_ch4_segment_5 _chapternumber__14) (Utilities|Struct|BreakS_ChapterSegmentData _chapter_data_struct_10))
  (switch Utilities|FlowControl|Switch|SwitchonE_ChapterNumber (Variables|ProgressionVariables|GetChapterNumber) ; The ones set Externally via Level
    (:NewEnumerator0
      ;[1 1 1] Ch1
      (switch Utilities|FlowControl|Switch|SwitchonE_Chapter1_Segments (Variables|ProgressionVariables|GetChapter1_Segment)
        (:NewEnumerator0
          (return true))
        (:NewEnumerator1
          (if (Utilities|Enum|Equal(Enum) _chapternumber__2 "NewEnumerator0")
            (if (Utilities|Enum|Equal(Enum) _ch1_segment "NewEnumerator0")
              (return true)
              (else
                _)))
          (return false))))
    (:NewEnumerator1
      ;[1 1 1] Ch2
      (switch Utilities|FlowControl|Switch|SwitchonE_Chapter2_Segments (Variables|ProgressionVariables|GetChapter2_Segment)
        (:NewEnumerator1
          (if (Utilities|Enum|Equal(Enum) _chapternumber__5 (Variables|ProgressionVariables|GetChapterNumber))
            (if (Utilities|Enum|Equal(Enum) _ch2_segment "NewEnumerator0")
              (return true)
              (else
                _)))
          (return false))
        (:NewEnumerator2
          (if (Utilities|Enum|Equal(Enum) _chapternumber__6 (Variables|ProgressionVariables|GetChapterNumber))
            (if (Utilities|Enum|Equal(Enum) _ch2_segment_2 "NewEnumerator1")
              (return true)
              (else
                _)))
          (return false))
        (:NewEnumerator4
          (if (Utilities|Enum|Equal(Enum) _chapternumber__7 (Variables|ProgressionVariables|GetChapterNumber))
            (if (Utilities|Enum|Equal(Enum) _ch2_segment_3 "NewEnumerator3")
              (return true)
              (else
                _)))
          (return false))))
    (:NewEnumerator2
      ;[1 1 1] Ch3
      (switch Utilities|FlowControl|Switch|SwitchonE_Chapter3_Segments (Variables|ProgressionVariables|GetChapter3_Segment)
        (:NewEnumerator0
          (if (Utilities|Enum|Equal(Enum) _chapternumber__8 "NewEnumerator1")
            (if (Utilities|Enum|Equal(Enum) _ch2_segment_4 "NewEnumerator5")
              (return true)
              (else
                _)))
          (return false))
        (:NewEnumerator3
          (if (Utilities|Enum|Equal(Enum) _chapternumber__9 "NewEnumerator2")
            (if (Utilities|Enum|Equal(Enum) _ch3_segment "NewEnumerator2")
              (return true)
              (else
                _)))
          (return false))))
    (:NewEnumerator3
      ;[1 1 1] Ch4
      (switch Utilities|FlowControl|Switch|SwitchonE_Chapter4_Segments (Variables|ProgressionVariables|GetChapter4_Segment)
        (:NewEnumerator0
          (if (Utilities|Enum|Equal(Enum) _chapternumber__10 "NewEnumerator2")
            (if (Utilities|Enum|Equal(Enum) _ch3_segment_2 "NewEnumerator3")
              (return true)
              (else
                _)))
          (return false))
        (:NewEnumerator1
          (if (Utilities|Enum|Equal(Enum) _chapternumber__11 "NewEnumerator3")
            (if (Utilities|Enum|Equal(Enum) _ch4_segment_2 "NewEnumerator0")
              (return true)
              (else
                _)))
          (return false))
        (:NewEnumerator4
          (if (Utilities|Enum|Equal(Enum) _chapternumber__12 "NewEnumerator3")
            (if (Utilities|Enum|Equal(Enum) _ch4_segment_3 "NewEnumerator3")
              (return true)
              (else
                _)))
          (return false))
        (:NewEnumerator5
          (if (Utilities|Enum|Equal(Enum) _chapternumber__13 "NewEnumerator3")
            (if (Utilities|Enum|Equal(Enum) _ch4_segment_4 "NewEnumerator4")
              (return true)
              (else
                _)))
          (return false))
        (:NewEnumerator6
          (if (Utilities|Enum|Equal(Enum) _chapternumber__14 "NewEnumerator3")
            (if (Utilities|Enum|Equal(Enum) _ch4_segment_5 "NewEnumerator5")
              (return true)
              (else
                _)))
          (return false))
        (:NewEnumerator12
          (if (Utilities|Enum|Equal(Enum) _chapternumber__3 "NewEnumerator3")
            (if (Utilities|Enum|Equal(Enum) _ch4_segment "NewEnumerator11")
              (return true)
              (else
                _)))
          (return false))))
    (:NewEnumerator4
      ;[1 1 1] Ch5
      (switch Utilities|FlowControl|Switch|SwitchonE_Chapter5_Segments (Variables|ProgressionVariables|GetChapter5_Segment)
        (:NewEnumerator1
          (if (Utilities|Enum|Equal(Enum) _chapternumber__4 "NewEnumerator4")
            (if (Utilities|Enum|Equal(Enum) _ch5_segment_2 "NewEnumerator0")
              (return true)
              (else
                _)))
          (return false))
        (:NewEnumerator3
          (if (Utilities|Enum|Equal(Enum) _chapternumber_ "NewEnumerator4")
            (if (Utilities|Enum|Equal(Enum) _ch5_segment "NewEnumerator2")
              (return true)
              (else
                _)))
          (return false))))))