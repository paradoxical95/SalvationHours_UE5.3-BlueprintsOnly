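; Male "CaseOff" NPC that randomizes shirt and jeans colors on BeginPlay through dynamic materials, then attaches to its assigned chair, if any.
; Modular body parts follow the main mesh as leader pose.
; Their cull distance is set at spawn and again when the draw-distance event fires.
; Order updates show the vest in chapters 5 and 6, and a getter exposes its evacuation vehicle and seat.
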(event Custom|ChangeDrawDistance_CO
  (params (DrawDistance :type Float%20%28single-precision%29))
  (Variables|Default|SetDrawDistanceLOD DrawDistance)
  (Class|PrimitiveComponent|SetCullDistance (Variables|Default|GetTorso) (Variables|Default|GetDrawDistanceLOD)))

(event EventBeginPlay
  (bind _chairtosit (Variables|Default|GetChairToSit))
  (|CallParentFunction)
  (bind _returnvalue (Rendering|Material|CreateDynamicMaterialInstance (Variables|Default|GetTorso) 0 "/Game/MetaHumans/CaseOfficer_1/Materials/Shirt/Male/M_m_top_shirt.M_m_top_shirt" "None" :!class /Script/Engine.PrimitiveComponent))
  (Rendering|Material|SetVectorParameterValue _returnvalue "diffuse_color_1" (Utilities|Array|Get(acopy) (Variables|Default|GetShirtColor) (Math|Random|RandomIntegerinRange 0 7)) :!class /Script/Engine.MaterialInstanceDynamic)
  (bind _returnvalue_2 (Rendering|Material|CreateDynamicMaterialInstance (Variables|Default|GetLegs) 0 "/Game/MetaHumans/CaseOfficer_1/Materials/Jeans/M_btm_jeans_nrm.M_btm_jeans_nrm" "None" :!class /Script/Engine.PrimitiveComponent))
  (Rendering|Material|SetVectorParameterValue _returnvalue_2 "diffuse_color_1" (Utilities|Array|Get(acopy) (Variables|Default|GetPantColor) (Math|Random|RandomIntegerinRange 0 2)) :!class /Script/Engine.MaterialInstanceDynamic)
  (Utilities|IsValid _chairtosit
    (:Is%20Valid
      (Class|BPIntActorProps|AttachtoChair(Message) _chairtosit false self))
    (:Is%20Not%20Valid
      _))
  (Class|PrimitiveComponent|SetCullDistance (Variables|Default|GetTorso) (Variables|Default|GetDrawDistanceLOD)))

(fn ConstructionScript
  (|CallParentFunction)
  (Components|SkinnedMesh|SetLeaderPoseComponent (Variables|Default|GetTorso) (Variables|Character|GetMesh) false false))

(fn NPCOrdersUpdated
  (|CallParentFunction)
  (switch Utilities|FlowControl|Switch|SwitchonE_ChapterNumber (Variables|Default|GetChapter%20Number)
    (:NewEnumerator4
      _)
    (:NewEnumerator5
      _))
  (Rendering|SetVisibility (Variables|Default|GetVest) true false))

(fn NPCCOEVACVehicleandSeat
  (return (Variables|Default|GetEVAC_Vehicle) (Variables|Default|GetSeatDuringEVAC)))