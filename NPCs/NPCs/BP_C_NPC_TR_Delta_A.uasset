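; Character Blueprint for a Delta variant NPC that assembles a modular body with tactical gear.
; The construction script makes the feet, legs, torso and face follow the main mesh's pose through leader pose components.
; On BeginPlay, after the parent logic, it shows the balaclava, visor, vest, helmet and weapon mesh.
; It then gives the balaclava a dynamic material instance with the camouflage texture as its base.
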(event EventBeginPlay
  (bind _balaclava (Variables|Default|GetBalaclava))
  (|CallParentFunction)
  (Rendering|SetVisibility _balaclava true false)
  (bind _returnvalue (Rendering|Material|CreateDynamicMaterialInstance _balaclava 0 "/Game/_Main/Assets/Tactical/Mat/Balaclava_Mat.Balaclava_Mat" "None" :!class /Script/Engine.PrimitiveComponent))
  (Rendering|Material|SetTextureParameterValue _returnvalue "BaseTex" "/Game/_Main/Assets/Tactical/Tex/Camouflage_Texture.Camouflage_Texture"))

(event Collision|EventActorBeginOverlap
  (params (OtherActor :type Actor%20Object%20Reference)))

(event EventTick
  (params (DeltaSeconds :type Float%20%28single-precision%29)))

(fn ConstructionScript
  (|CallParentFunction)
  (Components|SkinnedMesh|SetLeaderPoseComponent (Variables|Default|GetFeet) (Variables|Character|GetMesh) false false))