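; Blueprint for the NPC Phillip, a modular character with separate face and body meshes plus helmet, vest and pistol props.
; The construction script makes legs, torso and feet follow the main mesh's pose, and BeginPlay snaps the helmet to a face socket.
; An event plays optional face and body montages.
; The NPC orders event is empty, and the chapter-segment logic for gear visibility is unconnected.
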(event EventBeginPlay
  (|CallParentFunction)
  (Transformation|AttachComponentToComponent (Variables|Default|GetDelta_Helmet) (Variables|Default|GetFace) "Delta_Helmet" "SnapToTarget" "SnapToTarget" "SnapToTarget" true) ; WORKS !! EVEN WITH FACE ANIMS
)

(event EventPlayNPCAnimsOnly
  (params (FaceAnim :type Anim%20Montage%20Object%20Reference) (BodyAnim :type Anim%20Montage%20Object%20Reference))
  ;[0.09893 0.2031 0.1807] Playing Anims only
  ; For all NPCs
  (Utilities|FlowControl|Sequence
    (:then_0
      (Utilities|IsValid FaceAnim
        (:Is%20Valid
          (Animation|Montage|PlayMontage (Variables|Default|GetFace) FaceAnim))))
    (:then_1
      (Utilities|IsValid BodyAnim
        (:Is%20Valid
          (Animation|Montage|PlayMontage (Variables|Character|GetMesh) BodyAnim))))))

(event EventEventUpdateNPCOrders)

(fn ConstructionScript
  (|CallParentFunction)
  (Components|SkinnedMesh|SetLeaderPoseComponent (Variables|Default|GetLegs) (Variables|Character|GetMesh) false false))