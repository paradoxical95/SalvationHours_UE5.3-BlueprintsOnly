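; Blueprint for the NPC Ric, a MetaHuman character with a night-vision helmet attached to a socket on the Face mesh at BeginPlay.
; The construction script makes Feet, Legs and Torso follow the body mesh's pose.
; One event plays optional face and body montages, while another toggles soot by swapping color textures on dynamic face and body materials.
; Material slots, source materials and textures are hard-coded for this particular MetaHuman.
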(event EventBeginPlay
  (|CallParentFunction)
  ;[1 0.08327 0.09322] Necessary Code
  ; for GRS only
  (Transformation|AttachComponentToComponent (Variables|Default|GetNV_Helmet_SM) (Variables|Default|GetFace) "NV_Helmet" "SnapToTarget" "SnapToTarget" "SnapToTarget" true) ; WORKS !! EVEN WITH FACE ANIMS
)

(event EventPlayNPCAnimsOnly
  (params (FaceAnim :type Anim%20Montage%20Object%20Reference) (BodyAnim :type Anim%20Montage%20Object%20Reference))
  ;[0.09893 0.2031 0.1807] Playing Anims only
  ; For all NPCs
  (Utilities|FlowControl|Sequence
    (:then_0
      (Utilities|IsValid FaceAnim
        (:Is%20Valid
          (Animation|Montage|PlayMontage (Variables|Default|GetFace) FaceAnim))))
    (:then_1
      (Utilities|IsValid BodyAnim
        (:Is%20Valid
          (Animation|Montage|PlayMontage (Variables|Character|GetMesh) BodyAnim))))))

(event EventNPCToggleFaceSootTexture
  (params (ToggleSootTex? :type Boolean))
  ;[0.1354 0.1354 0.1354] Face Black Soot Texture Code
  (bind _returnvalue (Rendering|Material|CreateDynamicMaterialInstance (Variables|Default|GetFace) 11 "/Game/MetaHumans/Ric/Face/Materials/Baked/MI_HeadSynthesized_Baked_LOD2.MI_HeadSynthesized_Baked_LOD2" "None" :!class /Script/Engine.PrimitiveComponent)) ; This varies from MH to MH\nCheck Index as well as Source Mat
  (Rendering|Material|SetTextureParameterValue _returnvalue "Color_MAIN" (select ToggleSootTex? "/Game/MetaHumans/Drew/Face/FaceColor_MAIN_LOD1_Soot.FaceColor_MAIN_LOD1_Soot" "/Game/MetaHumans/Drew/Face/FaceColor_MAIN_LOD1.FaceColor_MAIN_LOD1")) ; This parameter remains same
  ;[0.2031 0.2031 0.2031] For Arms Soot Texture
  (bind _returnvalue_2 (Rendering|Material|CreateDynamicMaterialInstance (Variables|Character|GetMesh) 0 "/Game/MetaHumans/Ric/Materials/M_BodySynthesized.M_BodySynthesized" "None" :!class /Script/Engine.PrimitiveComponent)) ; This varies from MH to MH
  (Rendering|Material|SetTextureParameterValue _returnvalue_2 "Color_MAIN" (select ToggleSootTex? "/Game/MetaHumans/Ric/Body/BodyBaseColor_Soot.BodyBaseColor_Soot" "/Game/MetaHumans/Ric/Body/BodyBaseColor.BodyBaseColor")) ; This parameter remains same
)

(fn ConstructionScript
  (|CallParentFunction)
  (Components|SkinnedMesh|SetLeaderPoseComponent (Variables|Default|GetFeet) (Variables|Character|GetMesh) false false))