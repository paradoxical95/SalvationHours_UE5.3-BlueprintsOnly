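; Libyan soldier NPC Blueprint that dresses and arms a modular character, extending a parent NPC class.
; Construction makes the body parts follow the main Mesh's pose.
; BeginPlay shows an AK-style rifle, randomizes shirt colors and applies camouflage to the balaclava through dynamic materials, sets cull distances and flags LMG mounting.
; Two prep events clear that flag and set combat state for either a rifle-carrying soldier or an unarmed-looking suspect with a flip phone.
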(event Custom|Event_LibyanSusMan_Prep
  (Rendering|SetVisibility (Variables|Default|GetWeapon_SM) false false)
  (Variables|Default|SetLMG_Mounting? false)
  (Variables|Default|SetCombatState "NewEnumerator1")
  (Rendering|SetVisibility (Variables|Default|GetFlipPhone) true false)
  (Utilities|FlowControl|Delay 2e+01))

(event EventBeginPlay
  (bind _weapon_sm (Variables|Default|GetWeapon_SM))
  (bind _shirtcolorvalue (Variables|Default|GetShirtColorValue))
  (bind _outitem (Utilities|Array|Random _shirtcolorvalue))
  (|CallParentFunction)
  (Rendering|SetVisibility _weapon_sm true false)
  (Components|StaticMesh|SetStaticMesh _weapon_sm "/Game/FPS_Weapon_Bundle/Weapons/Meshes/Ka47/SM_KA47.SM_KA47")
  (Rendering|SetVisibility (Variables|Default|GetOptic) false false)
  (bind _returnvalue (Rendering|Material|CreateDynamicMaterialInstance (Variables|Default|GetTorso) 0 "/Game/MetaHumans/LibyanSoldier/Materials/Crewneckt/Male/M_m_top_crewneckt_nrm.M_m_top_crewneckt_nrm" "None" :!class /Script/Engine.PrimitiveComponent))
  (Rendering|Material|SetVectorParameterValue _returnvalue "diffuse_color_1" _outitem :!class /Script/Engine.MaterialInstanceDynamic)
  (Rendering|Material|SetVectorParameterValue _returnvalue "diffuse_color_2" _outitem :!class /Script/Engine.MaterialInstanceDynamic)
  (Variables|Default|SetLMG_Mounting? true)
  (bind _returnvalue_2 (Rendering|Material|CreateDynamicMaterialInstance (Variables|Default|GetBalaclava) 0 "/Game/_Main/Assets/Tactical/Mat/Balaclava_Mat.Balaclava_Mat" "None" :!class /Script/Engine.PrimitiveComponent))
  (Rendering|Material|SetTextureParameterValue _returnvalue_2 "BaseTex" "/Game/_Main/Assets/Tactical/Tex/Camouflage_Texture.Camouflage_Texture")
  (Class|PrimitiveComponent|SetCullDistance (Variables|Default|GetTorso) (Variables|Default|GetDrawDistanceLOD)))

(event EventPrepLibyanSoldier
  (bind _weapon_sm (Variables|Default|GetWeapon_SM))
  (Rendering|SetVisibility _weapon_sm true false)
  (Variables|Default|SetLMG_Mounting? false)
  (Variables|Default|SetCombatState "NewEnumerator2")
  (Transformation|AttachComponentToComponent _weapon_sm (Variables|Character|GetMesh) "Rifle_AK47" "SnapToTarget" "SnapToTarget" "SnapToTarget" true))

(fn ConstructionScript
  (|CallParentFunction)
  (Components|SkinnedMesh|SetLeaderPoseComponent (Variables|Default|GetTorso) (Variables|Character|GetMesh) false false))