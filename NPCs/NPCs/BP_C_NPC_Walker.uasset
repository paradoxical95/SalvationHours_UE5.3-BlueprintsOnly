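; BP_C_NPC_Walker is an NPC character blueprint with a modular body that extends a parent class's construction and BeginPlay logic.
; The construction script makes Torso, Legs and Feet follow the body Mesh through leader pose.
; BeginPlay creates a dynamic shirt material on the Torso and sets two fixed diffuse colors.
; PlayNPCAnimsOnly plays optional montages on Face and body Mesh separately, skipping any invalid one.
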(event EventBeginPlay
  (|CallParentFunction)
  (bind _returnvalue (Rendering|Material|CreateDynamicMaterialInstance (Variables|Default|GetTorso) 0 "/Game/MetaHumans/Walker/Materials/Shirt/Male/M_m_top_shirt.M_m_top_shirt" "None" :!class /Script/Engine.PrimitiveComponent))
  (Rendering|Material|SetVectorParameterValue _returnvalue "diffuse_color_1" "(R=0.196078,G=0.168627,B=0.145098,A=1.000000)" :!class /Script/Engine.MaterialInstanceDynamic)
  (Rendering|Material|SetVectorParameterValue _returnvalue "diffuse_color_2" "(R=0.070588,G=0.152941,B=0.250980,A=1.000000)" :!class /Script/Engine.MaterialInstanceDynamic))

(event EventPlayNPCAnimsOnly
  (params (FaceAnim :type Anim%20Montage%20Object%20Reference) (BodyAnim :type Anim%20Montage%20Object%20Reference))
  ;[0.09893 0.2031 0.1807] Playing Anims only
  ; For all NPCs
  (Utilities|FlowControl|Sequence
    (:then_0
      (Utilities|IsValid FaceAnim
        (:Is%20Valid
          (Animation|Montage|PlayMontage (Variables|Default|GetFace) FaceAnim))))
    (:then_1
      (Utilities|IsValid BodyAnim
        (:Is%20Valid
          (Animation|Montage|PlayMontage (Variables|Character|GetMesh) BodyAnim))))))

(fn ConstructionScript
  (|CallParentFunction)
  (Components|SkinnedMesh|SetLeaderPoseComponent (Variables|Default|GetTorso) (Variables|Character|GetMesh) false false))