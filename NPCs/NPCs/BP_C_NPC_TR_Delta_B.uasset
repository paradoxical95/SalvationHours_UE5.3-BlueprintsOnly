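; Delta B variant NPC Blueprint that sets up the look of a modular character in tactical gear over casual clothing.
; The construction script makes feet, legs, torso and face follow the main mesh pose.
; After parent BeginPlay, it shows the balaclava, visor, vest, helmet and weapon.
; It then creates dynamic materials to choose a camo or black balaclava and tint the shirt and jeans from color variables.
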(event EventBeginPlay
  (bind _balaclava (Variables|Default|GetBalaclava))
  (bind _shirtcolorvalue (Variables|Default|GetShirtColorValue))
  (bind _pantcolorvalue (Variables|Default|GetPantColorValue))
  (|CallParentFunction)
  (Rendering|SetVisibility _balaclava true false)
  (bind _returnvalue (Rendering|Material|CreateDynamicMaterialInstance _balaclava 0 "/Game/_Main/Assets/Tactical/Mat/Balaclava_Mat.Balaclava_Mat" "None" :!class /Script/Engine.PrimitiveComponent))
  (Rendering|Material|SetTextureParameterValue _returnvalue "BaseTex" (select (Variables|Default|GetBalaclavaCamo?) "/Game/_Main/Assets/Tactical/Tex/Camouflage_Texture.Camouflage_Texture" "/Game/_Main/Assets/Tactical/Tex/black_Balaclave__0.black_Balaclave__0"))
  (bind _returnvalue_2 (Rendering|Material|CreateDynamicMaterialInstance (Variables|Default|GetTorso) 0 "/Game/MetaHumans/TripoliDelta/Materials/Crewneckt/Male/M_m_top_crewneckt_nrm.M_m_top_crewneckt_nrm" "None" :!class /Script/Engine.PrimitiveComponent))
  (Rendering|Material|SetVectorParameterValue _returnvalue_2 "diffuse_color_1" _shirtcolorvalue :!class /Script/Engine.MaterialInstanceDynamic)
  (Rendering|Material|SetVectorParameterValue _returnvalue_2 "diffuse_color_2" _shirtcolorvalue :!class /Script/Engine.MaterialInstanceDynamic)
  (bind _returnvalue_3 (Rendering|Material|CreateDynamicMaterialInstance (Variables|Default|GetLegs) 0 "/Game/MetaHumans/TripoliDelta/Materials/Jeans/M_btm_jeans_nrm.M_btm_jeans_nrm" "None" :!class /Script/Engine.PrimitiveComponent))
  (Rendering|Material|SetVectorParameterValue _returnvalue_3 "diffuse_color_1" _pantcolorvalue :!class /Script/Engine.MaterialInstanceDynamic)
  (Rendering|Material|SetVectorParameterValue _returnvalue_3 "diffuse_color_2" _pantcolorvalue :!class /Script/Engine.MaterialInstanceDynamic))

(fn ConstructionScript
  (|CallParentFunction)
  (Components|SkinnedMesh|SetLeaderPoseComponent (Variables|Default|GetFeet) (Variables|Character|GetMesh) false false))