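; Jim NPC character Blueprint, a child class that plays montage animations on a modular body and separate face mesh.
; On BeginPlay it shows the night-vision helmet, vest and weapon meshes, then snaps the helmet to a Face socket so it works with facial animation.
; The construction script makes feet, legs and torso follow the body mesh pose.
; PlayNPCAnimsOnly plays optional face and body montages on their respective meshes.
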(event EventBeginPlay
  (|CallParentFunction)
  (Rendering|SetVisibility (Variables|Default|GetNV_Helmet_SM) true false)
  ;[1 0.08327 0.09322] Necessary Code
  ; for GRS only
  (Transformation|AttachComponentToComponent (Variables|Default|GetNV_Helmet_SM) (Variables|Default|GetFace) "NV_Helmet" "SnapToTarget" "SnapToTarget" "SnapToTarget" true) ; WORKS !! EVEN WITH FACE ANIMS
)

(event EventPlayNPCAnimsOnly
  (params (FaceAnim :type Anim%20Montage%20Object%20Reference) (BodyAnim :type Anim%20Montage%20Object%20Reference))
  ;[0.09893 0.2031 0.1807] Playing Anims only
  ; For all NPCs
  (Utilities|FlowControl|Sequence
    (:then_0
      (Utilities|IsValid FaceAnim
        (:Is%20Valid
          (Animation|Montage|PlayMontage (Variables|Default|GetFace) FaceAnim))))
    (:then_1
      (Utilities|IsValid BodyAnim
        (:Is%20Valid
          (Animation|Montage|PlayMontage (Variables|Character|GetMesh) BodyAnim))))))

(fn ConstructionScript
  (|CallParentFunction)
  (Components|SkinnedMesh|SetLeaderPoseComponent (Variables|Default|GetFeet) (Variables|Character|GetMesh) false false))