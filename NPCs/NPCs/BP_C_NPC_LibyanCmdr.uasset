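; BP_C_NPC_LibyanCmdr is a Libyan commander NPC Blueprint that extends a parent class with its own weapon setup and modular body.
; The construction script runs the parent's, then makes the feet, legs, face and torso follow the main Mesh through leader pose.
; On BeginPlay, after the parent's logic, it shows the weapon mesh, assigns the SM_KA_Val_Y model and hides the optic.
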(event EventBeginPlay
  (bind _weapon_sm (Variables|Default|GetWeapon_SM))
  (|CallParentFunction)
  (Rendering|SetVisibility _weapon_sm true false)
  (Components|StaticMesh|SetStaticMesh _weapon_sm "/Game/FPS_Weapon_Bundle/Weapons/Meshes/KA_Val/SM_KA_Val_Y.SM_KA_Val_Y")
  (Rendering|SetVisibility (Variables|Default|GetOptic) false false))

(event Collision|EventActorBeginOverlap
  (params (OtherActor :type Actor%20Object%20Reference)))

(event EventTick
  (params (DeltaSeconds :type Float%20%28single-precision%29)))

(fn ConstructionScript
  (|CallParentFunction)
  (Components|SkinnedMesh|SetLeaderPoseComponent (Variables|Default|GetFeet) (Variables|Character|GetMesh) false false))