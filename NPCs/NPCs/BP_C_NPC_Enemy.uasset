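; Armed enemy NPC with randomized clothing and face coverings, which shoots at the player (tag "Jack") and sometimes at "GRS" pawns.
; A game instance event sends it along waypoints with AIMoveTo, then enables pawn sensing and random crouching.
; Shots are camera line traces with random pitch error, difficulty-based player damage, cosmetic effects and timed reloads.
; On death it spawns a decal, reports to the game instance and destroys itself after a delay.
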(event OnSeePawn(PawnSensing)
  (params (Pawn :type Pawn%20Object%20Reference))
  (bind _returnvalue (Transformation|GetActorLocation Pawn))
  (bind _weapon_sm (Variables|Default|GetWeapon_SM))
  (bind _npc_camera (Variables|Default|GetNPC_Camera))
  (bind _burstsmoke_ns (Variables|Default|GetBurstSmoke_NS))
  (bind _returnvalue_2 (Transformation|GetSocketTransform _weapon_sm "Fire" "RTS_World"))
  (bind _returnvalue_3 (Transformation|GetWorldTransform _npc_camera))
  (bind _returnvalue_4 (Math|Rotator|FindLookatRotation (.location _returnvalue_3) _returnvalue))
  ;[0.3438 0.04793 0] Activating Enemy
  (if (not (Variables|Default|GetIsDead?))
    (if (Variables|Default|GetActivateEnemy?)
      (if (Actor|ActorHasTag Pawn "Jack")
        (Transformation|SetWorldRotation _npc_camera (Math|Rotator|MakeRotator (.roll _returnvalue_4) (+ (.pitch _returnvalue_4) (Math|Random|RandomFloatinRange 0.45 2.25)) (.yaw _returnvalue_4)) false false :!label _label)
        (bind _outhit (Collision|LineTraceByChannel (.location _returnvalue_3) (+ (.location _returnvalue_3) (* (Math|Vector|GetForwardVector (.rotation _returnvalue_3)) 5e+03)) "TraceTypeQuery2" false 0 "None" true "(R=1.000000,G=0.000000,B=0.000000,A=1.000000)" "(R=0.000000,G=1.000000,B=0.000000,A=1.000000)" 0.1))
        (Utilities|IsValid (.HitActor (Collision|BreakHitResult _outhit))
          (:Is%20Valid
            (if (Actor|ActorHasTag (.HitActor (Collision|BreakHitResult _outhit)) "Jack")
              (if (Variables|Default|GetCanFire?)
                (Game|Damage|ApplyDamage (.HitActor (Collision|BreakHitResult _outhit)) (Variables|Default|GetDamageValue) 0 self) ; Apply Damage to Player
                (if (Math|Random|RandomBoolwithWeight 0.2) :!label _label_2
                  (Game|SpawnActorfromClass "/Game/_Main/Blueprints/Weapons_BP/BP_BulletProjectile.BP_BulletProjectile_C" (Math|Transform|MakeTransform (.location _returnvalue_2) (.rotation _returnvalue_2) "1.000000,1.000000,1.000000") "Undefined" "MultiplyWithRoot" 0 0))
                (Transformation|AttachComponentToComponent _burstsmoke_ns (Variables|Default|GetWeapon_SM) "Fire" "SnapToTarget" "SnapToTarget" "SnapToTarget" true)
                (Components|Activation|Activate _burstsmoke_ns false)
                (Utilities|FlowControl|Delay 0.25)
                (Components|Activation|Deactivate _burstsmoke_ns)
                (if (Math|Random|RandomBoolwithWeight 0.15)
                  (Audio|SpawnSoundAttached "/Game/_Main/Blueprints/NPCs/AudioFX/Enemy_Attack_VO_Cue.Enemy_Attack_VO_Cue" (Variables|Character|GetMesh) "None" "0, 0, 0" "0, 0, 0" "KeepRelativeOffset" false 0.8 1.0 0.0 "/Game/_Main/Blueprints/NPCs/AudioFX/NPC_VO_SoundAttenuation.NPC_VO_SoundAttenuation" "/Game/_Main/Blueprints/NPCs/AudioFX/BP_SoundConcurrency.BP_SoundConcurrency"))
                (if (Math|Random|RandomBoolwithWeight 0.9)
                  (Utilities|LightFlicker)
                  (Audio|SpawnSoundAttached "/Game/Warfare_SFX_Bundle/Gun_Sound_Essentials/Enemy_AK_Rifle_Cue.Enemy_AK_Rifle_Cue" (Variables|Character|GetMesh) "None" "0, 0, 0" "0, 0, 0" "KeepRelativeOffset" false 1.0 1.0 0.0 "/Game/_Main/Blueprints/NPCs/AudioFX/Enemy_Rifle_Attenuation.Enemy_Rifle_Attenuation" "/Game/_Main/Blueprints/NPCs/AudioFX/BP_SoundConcurrency.BP_SoundConcurrency"))
                (bind _result (Math|Integer|IncrementInt (Variables|Default|GetFiringCount))
                  (:%20%20
                    (if (<= _result 30)
                      (Variables|Default|SetCanFire? false)
                      (Utilities|FlowControl|Delay (Math|Random|RandomFloatinRange 0.1 1.75)) ; random delay between shots
                      (Variables|Default|SetCanFire? true)
                      (if (Math|Random|RandomBoolwithWeight 0.5)
                        (Utilities|FlowControl|Sequence
                          (:then_0
                            (Utilities|FlowControl|DoOnce false) ; enters at Reset
                          )
                          (:then_1
                            (Utilities|FlowControl|DoOnce false) ; enters at Reset
                          )))
                      (else
                        (Variables|Default|SetFiringCount 0)
                        (Variables|Default|SetCanFire? false)
                        (Variables|Default|SetPlayingAnim true)
                        (Variables|Default|SetIsNPC_Reloading? true)
                        (Utilities|FlowControl|Delay 4.5)
                        (Variables|Default|SetIsNPC_Reloading? false)
                        (Variables|Default|SetPlayingAnim false)
                        (Variables|Default|SetCanFire? true))))))
              (else
                (if (Math|Random|RandomBoolwithWeight 0.05) :!label _label_3
                  (Audio|SpawnSoundatLocation "/Game/Warfare_SFX_Bundle/Bullet_Impacts_Flybys_Pro/Wavs/Concrete/ConcreteImpact_Bullets_Cue.ConcreteImpact_Bullets_Cue" (.ImpactPoint (Collision|BreakHitResult _outhit)) "0, 0, 0" 0.8 1.0 0.0 "/Game/_Main/Blueprints/NPCs/AudioFX/NPC_VO_SoundAttenuation.NPC_VO_SoundAttenuation" "/Game/_Main/Blueprints/NPCs/AudioFX/BP_SoundConcurrency.BP_SoundConcurrency")
                  (goto _label_2)
                  (else
                    (goto _label_2)))))))
        (elif (Variables|Default|GetShootGRS?) ; randomly choosing.\nNot always
          (if (Actor|ActorHasTag Pawn "GRS")
            (goto _label)
            (else
              (goto _label_3)))
          (else
            (goto _label_3)))))))

(event Custom|HandleCrouchRandom
  ;[0.3438 0.04793 0] Activating Enemy
  (Variables|Default|SetIsCrouched? (Math|Random|RandomBoolwithWeight 0.35))
  (Variables|Default|SetShootGRS? (Math|Random|RandomBoolwithWeight 0.5)))

(event EventBeginPlay
  (bind _balaclava_color (Variables|Default|GetBalaclava_Color))
  (bind _outitem (Utilities|Array|Random _balaclava_color))
  (|CallParentFunction)
  (Rendering|SetVisibility (select (Math|Random|RandomBoolwithWeight 0.65) (Variables|Default|GetBalaclava) (Variables|Default|GetBandana)) true false)
  (bind _returnvalue (Rendering|Material|CreateDynamicMaterialInstance (Variables|Default|GetTorso) 0 "/Game/MetaHumans/Enemy/Materials/Crewneckt/Male/M_m_top_crewneckt_nrm.M_m_top_crewneckt_nrm" "None" :!class /Script/Engine.PrimitiveComponent))
  (Rendering|Material|SetVectorParameterValue _returnvalue "diffuse_color_1" (.OutItem (Utilities|Array|Random (Variables|Default|GetShirtColor_1))) :!class /Script/Engine.MaterialInstanceDynamic)
  (Rendering|Material|SetVectorParameterValue _returnvalue "diffuse_color_2" (.OutItem (Utilities|Array|Random (Variables|Default|GetShirtColor_2))) :!class /Script/Engine.MaterialInstanceDynamic)
  (bind _returnvalue_2 (Rendering|Material|CreateDynamicMaterialInstance (Variables|Default|GetLegs) 0 "/Game/MetaHumans/Enemy/Materials/Cargopants/M_btm_cargopants.M_btm_cargopants" "None" :!class /Script/Engine.PrimitiveComponent))
  (Rendering|Material|SetVectorParameterValue _returnvalue_2 "diffuse_color_1" (.OutItem (Utilities|Array|Random (Variables|Default|GetPantsColor))) :!class /Script/Engine.MaterialInstanceDynamic)
  (bind _returnvalue_3 (Rendering|Material|CreateDynamicMaterialInstance (Variables|Default|GetBandana) 0 "/Game/_Main/Assets/Tactical/Mat/Bandana_MI.Bandana_MI" "None" :!class /Script/Engine.PrimitiveComponent))
  (Rendering|Material|SetVectorParameterValue _returnvalue_3 "Color" _outitem :!class /Script/Engine.MaterialInstanceDynamic)
  (bind _returnvalue_4 (Rendering|Material|CreateDynamicMaterialInstance (Variables|Default|GetBalaclava) 0 "/Game/_Main/Assets/Tactical/Mat/Balaclava_MI.Balaclava_MI" "None" :!class /Script/Engine.PrimitiveComponent))
  (Rendering|Material|SetVectorParameterValue _returnvalue_4 "Color" _outitem :!class /Script/Engine.MaterialInstanceDynamic)
  (Rendering|SetVisibility (Variables|Default|GetWeapon_SM) (Variables|Default|GetWeaponVisible?) false)
  (Class|PrimitiveComponent|SetCullDistance (Variables|Character|GetMesh) (Variables|Default|GetDrawDistance))
  (Class|PawnSensingComponent|SetSensingUpdatesEnabled (Variables|Default|GetPawnSensing) false)
  (bind _gamedifficulty (Class|BPIntGameInstance|GIFetchDataControls(Message) (Game|GetGameInstance)))
  (Variables|Default|SetDamageValue (Utilities|Select :Index _gamedifficulty :NewEnumerator0 1.25 :NewEnumerator1 2.25) :!pinned true) ; Set Game Difficulty based\nDamage Value
)

(event Game|Damage|EventAnyDamage
  (params (Damage :type Float%20%28single-precision%29) (DamageType :type Damage%20Type%20Object%20Reference) (InstigatedBy :type Controller%20Object%20Reference) (DamageCauser :type Actor%20Object%20Reference))
  ;[1 1 1] Take Damage Event
  (if (not (Variables|Default|GetIsDead?))
    (bind _output_get (Variables|Default|SetHealth (- (Variables|Default|GetHealth) Damage)))
    (if (<= _output_get 0.0)
      (AI|Navigation|StopMovement (AI|GetAIController self)) ; SPAWN BLOOD FX ?
      (Class|PawnSensingComponent|SetSensingUpdatesEnabled (Variables|Default|GetPawnSensing) false)
      (Variables|Default|SetActivateEnemy? false)
      (Utilities|Time|ClearandInvalidateTimerbyHandle (Variables|Default|GetCrouchEventTimer))
      (Variables|Default|SetIsCrouched? false)
      (Variables|Default|SetIsNPC_Reloading? false)
      (Variables|Default|SetIsDead? true)
      (bind _returnvalue (Game|SpawnActorfromClass "/Game/_Main/Blueprints/Decals_Custom/BP_QuixelDecals.BP_QuixelDecals_C" (Math|Transform|MakeTransform (Transformation|GetWorldLocation (Variables|Default|GetFeet)) "0, 0, 0" "1.000000,1.000000,1.000000") "AlwaysSpawn" "MultiplyWithRoot" 0 2 21 0.5 0.5 0))
      (Class|BPIntGameInstance|GITrackDeadEnemies(Message) (Game|GetGameInstance) 1)
      (Collision|SetCollisionEnabled (Variables|Character|GetMesh) "NoCollision")
      (Rendering|SetVisibility (Variables|Default|GetNPCIndicatorSprite) false false)
      (Utilities|FlowControl|Delay 12.0)
      (Actor|DestroyActor)
      (Actor|DestroyActor _returnvalue))))

(event EventNPCActivateEnemyEvent
  (params (TP%20Array :type Array%20of%20Target%20Point%20Object%20References))
  (bind _enemyendlocationradius (Variables|Default|GetEnemyEndLocationRadius))
  (bind _returnvalue (* _enemyendlocationradius -1.0))
  (bind _returnvalue_2 (Math|Random|RandomFloatinRange _returnvalue _enemyendlocationradius))
  ;[0.3438 0.04793 0] Activating Enemy
  (if (not (Variables|Default|GetIsDead?))
    (if (not (Variables|Default|GetActivateEnemy?))
      (Variables|Default|SetHead_LookAt_Value 0.35)
      (Variables|/Script/Engine.CharacterMovementComponent|SetMaxWalkSpeed (Variables|Character|GetCharacterMovement) 4e+02)
      (Utilities|IsValid (Utilities|Array|Get(acopy) TP%20Array (Variables|Default|GetTP_Counter)) :!label _label
        (:Is%20Valid
          (AI|AIMoveTo self "0, 0, 0" (Utilities|Array|Get(acopy) TP%20Array (Variables|Default|GetTP_Counter)) 65.0 false
            (:OnSuccess
              (Math|Integer|IncrementInt (Variables|Default|GetTP_Counter)
                (:%20%20
                  (Variables|Default|SetEnemyFailCount 0)
                  (goto _label))))
            (:OnFail
              (bind _result (Math|Integer|IncrementInt (Variables|Default|GetEnemyFailCount) :!label _label_2)
                (:%20%20
                  (if (> _result 3)
                    (Math|Integer|DecrementInt (Variables|Default|GetTP_Counter)
                      (:%20%20
                        (AI|AIMoveTo self "0, 0, 0" (Utilities|Array|Get(acopy) TP%20Array (Variables|Default|GetTP_Counter)) 85.0 false
                          (:OnSuccess
                            (Math|Integer|IncrementInt (Variables|Default|GetTP_Counter)
                              (:%20%20
                                _)))
                          (:OnFail
                            (goto _label_2)))))
                    (else
                      (goto _label))))))))
        (:Is%20Not%20Valid
          _))
      (Transformation|SetActorLocation (Math|Vector|MakeVector (+ (.x (Transformation|GetActorLocation (Utilities|Array|Get(acopy) TP%20Array (- (Variables|Default|GetTP_Counter) 1)))) _returnvalue_2) (+ (.y (Transformation|GetActorLocation (Utilities|Array|Get(acopy) TP%20Array (- (Variables|Default|GetTP_Counter) 1)))) _returnvalue_2) (.z (Transformation|GetActorLocation))) false false)
      (Class|PawnSensingComponent|SetSensingUpdatesEnabled (Variables|Default|GetPawnSensing) true)
      (Variables|Default|SetTP_Counter 0)
      (Utilities|FlowControl|Delay 1.0)
      (Variables|Default|SetActivateEnemy? true) ; This allows the Pawn Sensing to actually work
      (Variables|Default|SetEnemyFailCount 0)
      (bind _returnvalue_3 (Utilities|Time|SetTimerbyEvent (delegate Custom|HandleCrouchRandom) 5.0 true))
      (Variables|Default|SetCrouchEventTimer _returnvalue_3))))

(fn ConstructionScript
  (|CallParentFunction)
  (Components|SkinnedMesh|SetLeaderPoseComponent (Variables|Default|GetFeet) (Variables|Character|GetMesh) false false))