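; MetaHuman-based NPC character Blueprint (DC) with modular body parts and a night-vision helmet.
; Construction makes feet, torso and legs follow the body mesh's pose, and BeginPlay snaps the helmet to a face socket.
; An event plays optional face and body montages on their respective meshes.
; A soot toggle creates dynamic materials for face and body, swapping clean and sooty color textures, with slots and source materials specific to this MetaHuman.
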(event EventBeginPlay
  (|CallParentFunction)
  ;[1 0.08327 0.09322] Necessary Code
  ; for GRS only
  (Transformation|AttachComponentToComponent (Variables|Default|GetNV_Helmet_SM) (Variables|Default|GetFace) "NV_Helmet" "SnapToTarget" "SnapToTarget" "SnapToTarget" true) ; WORKS !! EVEN WITH FACE ANIMS
)

(event Collision|EventActorBeginOverlap
  (params (OtherActor :type Actor%20Object%20Reference)))

(event EventTick
  (params (DeltaSeconds :type Float%20%28single-precision%29)))

(event EventPlayNPCAnimsOnly
  (params (FaceAnim :type Anim%20Montage%20Object%20Reference) (BodyAnim :type Anim%20Montage%20Object%20Reference))
  (Utilities|FlowControl|Sequence
    (:then_0
      (Utilities|IsValid FaceAnim
        (:Is%20Valid
          (Animation|Montage|PlayMontage (Variables|Default|GetFace) FaceAnim))))
    (:then_1
      (Utilities|IsValid BodyAnim
        (:Is%20Valid
          (Animation|Montage|PlayMontage (Variables|Character|GetMesh) BodyAnim))))))

(event EventNPCToggleFaceSootTexture
  (params (ToggleSootTex? :type Boolean))
  ;[0.1354 0.1354 0.1354] Face Black Soot Texture Code
  (bind _returnvalue (Rendering|Material|CreateDynamicMaterialInstance (Variables|Default|GetFace) 11 "/Game/MetaHumans/DC/Face/Materials/Baked/MI_HeadSynthesized_Baked_LOD2.MI_HeadSynthesized_Baked_LOD2" "None" :!class /Script/Engine.PrimitiveComponent)) ; This varies from MH to MH\nCheck Index as well as Source Mat
  (Rendering|Material|SetTextureParameterValue _returnvalue "Color_MAIN" (select ToggleSootTex? "/Game/MetaHumans/DC/Face/FaceColor_MAIN_LOD_Soot.FaceColor_MAIN_LOD_Soot" "/Game/MetaHumans/DC/Face/FaceColor_MAIN_LOD.FaceColor_MAIN_LOD")) ; This parameter remains same
  ;[0.2031 0.2031 0.2031] For Arms Soot Texture
  (bind _returnvalue_2 (Rendering|Material|CreateDynamicMaterialInstance (Variables|Character|GetMesh) 0 "/Game/MetaHumans/DC/Materials/M_BodySynthesized.M_BodySynthesized" "None" :!class /Script/Engine.PrimitiveComponent)) ; This varies from MH to MH
  (Rendering|Material|SetTextureParameterValue _returnvalue_2 "Color_MAIN" (select ToggleSootTex? "/Game/MetaHumans/DC/Body/BodyBaseColor_Soot.BodyBaseColor_Soot" "/Game/MetaHumans/DC/Body/BodyBaseColor.BodyBaseColor")) ; This parameter remains same
)

(fn ConstructionScript
  (|CallParentFunction)
  (Components|SkinnedMesh|SetLeaderPoseComponent (Variables|Default|GetFeet) (Variables|Character|GetMesh) false false))