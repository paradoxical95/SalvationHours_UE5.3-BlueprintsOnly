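; Blueprint for Chester, an NPC built on a parent NPC class and assembled from modular body meshes.
; Construction makes the feet, legs, torso and face follow the main mesh's pose as leader.
; On BeginPlay he attaches to his assigned chair through a message call and hides his weapon mesh.
; When NPC orders update, his vest is made visible for Chapters 5 and 6.
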(event EventBeginPlay
  (|CallParentFunction)
  (Class|BPIntActorProps|AttachtoChair(Message) (Variables|Default|GetChairToSit) false self)
  (Rendering|SetVisibility (Variables|Default|GetWeapon_SM) false true))

(fn ConstructionScript
  (|CallParentFunction)
  (Components|SkinnedMesh|SetLeaderPoseComponent (Variables|Default|GetFeet) (Variables|Character|GetMesh) false false))

(fn NPCOrdersUpdated
  (|CallParentFunction)
  (switch Utilities|FlowControl|Switch|SwitchonE_ChapterNumber (Variables|Default|GetChapter%20Number)
    (:NewEnumerator4
      _)
    (:NewEnumerator5
      _))
  (Rendering|SetVisibility (Variables|Default|GetVest) true false))