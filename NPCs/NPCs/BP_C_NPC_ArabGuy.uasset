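; NPC Blueprint for an Arab man, with a scripted Chapter 5 voice-over scene.
; Construction makes legs, feet and torso follow the main mesh's pose; BeginPlay tints the torso through a dynamic material and switches off pawn sensing.
; Events play optional face and body montages, or run the timed Arabic dialogue, raising a scene flag until the audio fades out.
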(event Custom|Event_ArabGuySeq
  (bind _vo_audio (Variables|Default|GetVO_Audio))
  (Audio|Components|Audio|SetSound _vo_audio "/Game/_Main/VO/NPC/ArabMen/ArabMan_Ch5Seg2_Arabic.ArabMan_Ch5Seg2_Arabic")
  (Audio|Components|Audio|Play _vo_audio 0.0)
  (Variables|Default|SetArabGuy_Ch5Scene true)
  (Utilities|FlowControl|Delay 1e+01)
  (Audio|Components|Audio|FadeOut (Variables|Default|GetVO_Audio) 0.55 0.0 "Linear" :!class /Script/Engine.AudioComponent)
  (Variables|Default|SetArabGuy_Ch5Scene false))

(event EventBeginPlay
  (bind _pawnsensing (Variables|Default|GetPawnSensing))
  (|CallParentFunction)
  (bind _returnvalue (Rendering|Material|CreateDynamicMaterialInstance (Variables|Default|GetTorso) 0 "/Game/MetaHumans/ArabKid/Materials/Crewneckt/Male/M_m_top_crewneckt_nrm.M_m_top_crewneckt_nrm" "None" :!class /Script/Engine.PrimitiveComponent))
  (Rendering|Material|SetVectorParameterValue _returnvalue "diffuse_color_1" "(R=0.172357,G=0.257127,B=0.307292,A=1.000000)" :!class /Script/Engine.MaterialInstanceDynamic)
  (Rendering|Material|SetVectorParameterValue _returnvalue "diffuse_color_2" "(R=0.229167,G=0.204670,B=0.098919,A=1.000000)" :!class /Script/Engine.MaterialInstanceDynamic)
  (Class|PawnSensingComponent|SetSensingUpdatesEnabled _pawnsensing false)
  (Components|Activation|Deactivate _pawnsensing))

(event EventPlayNPCAnimsOnly
  (params (FaceAnim :type Anim%20Montage%20Object%20Reference) (BodyAnim :type Anim%20Montage%20Object%20Reference))
  (Utilities|FlowControl|Sequence
    (:then_0
      (Utilities|IsValid FaceAnim
        (:Is%20Valid
          (Animation|Montage|PlayMontage 0 FaceAnim))))
    (:then_1
      (Utilities|IsValid BodyAnim
        (:Is%20Valid
          (Animation|Montage|PlayMontage (Variables|Character|GetMesh) BodyAnim))))))

(fn ConstructionScript
  (|CallParentFunction)
  (Components|SkinnedMesh|SetLeaderPoseComponent (Variables|Default|GetLegs) (Variables|Character|GetMesh) false false))