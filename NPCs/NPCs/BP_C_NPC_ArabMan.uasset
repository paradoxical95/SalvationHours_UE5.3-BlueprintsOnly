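; BP_C_NPC_ArabMan is an NPC Blueprint with a modular body that plays face and body animation montages on request.
; The construction script makes the Feet, Torso and Legs meshes follow the main Mesh as leader pose.
; BeginPlay tints the torso's crew-neck shirt grey through a dynamic material instance.
; PlayNPCAnimsOnly plays each valid montage on its component, Face or Mesh.
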(event EventBeginPlay
  (|CallParentFunction)
  (bind _returnvalue (Rendering|Material|CreateDynamicMaterialInstance (Variables|Default|GetTorso) 0 "/Game/MetaHumans/ArabMan/Materials/Crewneckt/Male/M_m_top_crewneckt_nrm.M_m_top_crewneckt_nrm" "None" :!class /Script/Engine.PrimitiveComponent))
  (Rendering|Material|SetVectorParameterValue _returnvalue "diffuse_color_1" "(R=0.307292,G=0.307292,B=0.307292,A=1.000000)" :!class /Script/Engine.MaterialInstanceDynamic)
  (Rendering|Material|SetVectorParameterValue _returnvalue "diffuse_color_2" "(R=0.229167,G=0.229167,B=0.229167,A=1.000000)" :!class /Script/Engine.MaterialInstanceDynamic))

(event Collision|EventActorBeginOverlap
  (params (OtherActor :type Actor%20Object%20Reference)))

(event EventTick
  (params (DeltaSeconds :type Float%20%28single-precision%29)))

(event EventPlayNPCAnimsOnly
  (params (FaceAnim :type Anim%20Montage%20Object%20Reference) (BodyAnim :type Anim%20Montage%20Object%20Reference))
  (Utilities|FlowControl|Sequence
    (:then_0
      (Utilities|IsValid FaceAnim
        (:Is%20Valid
          (Animation|Montage|PlayMontage (Variables|Default|GetFace) FaceAnim))))
    (:then_1
      (Utilities|IsValid BodyAnim
        (:Is%20Valid
          (Animation|Montage|PlayMontage (Variables|Character|GetMesh) BodyAnim))))))

(fn ConstructionScript
  (|CallParentFunction)
  (Components|SkinnedMesh|SetLeaderPoseComponent (Variables|Default|GetFeet) (Variables|Character|GetMesh) false false))