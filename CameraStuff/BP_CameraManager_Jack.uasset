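; Player camera manager for BP_Jack that drives first-person aim-down-sights view and camera sway.
; BlueprintUpdateCamera uses ADSAlpha to blend location from FPCamera toward the primary weapon's active socket, adjusted along its forward axis by a dot product.
; The same alpha narrows the clamped base FOV by the optic's offset.
; Tick interpolates mouse-driven sway, clamped tighter in ADS, which is added in control-rotation space.
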(event Custom|Event_CameraSway
  ;[1 1 1] Camera Sway Event
  (Utilities|IsValid (Variables|Default|GetJack_Ref)
    (:Is%20Valid
      (Variables|Default|SetSwayOffset (Math|Interpolation|VInterpTo (Variables|Default|GetSwayOffset) "0, 0, 0" (Utilities|Time|GetWorldDeltaSeconds) 8.0))
      (Variables|Default|SetSwayOffset (Math|Interpolation|VInterpTo (Variables|Default|GetSwayOffset) (Math|Vector|SelectVector (Utilities|SwayADS) (Utilities|SwayIdle) (Variables|/Game/_Main/Blueprints/BP_Jack.BP_Jack_C|GetIsInADS? (Variables|Default|GetJack_Ref))) (Utilities|Time|GetWorldDeltaSeconds) 5.0)))))

(event Custom|UpdateCamFOV
  (params (NewFOV :type Float%20%28single-precision%29))
  (Variables|Default|SetNewCameraBaseFOV (Math|Float|Clamp(Float) NewFOV 6e+01 1.2e+02)))

(event EventBeginPlay
  (bind _asbp_jack (Utilities|Casting|CastToBP_Jack (Game|GetPlayerCharacter 0)))
  (Variables|Default|SetJack_Ref _asbp_jack))

(event EventTick
  (params (DeltaSeconds :type Float%20%28single-precision%29))
  (CallFunction|EventCameraSway))

(fn ConstructionScript)

(fn BlueprintUpdateCamera
  (params (CameraTarget :type Actor%20Object%20Reference))
  (bind _jack_ref (Variables|Default|GetJack_Ref))
  (bind _newcamerabasefov (Variables|Default|GetNewCameraBaseFOV))
  (bind _jack_ref_2 (Variables|Default|GetJack_Ref))
  (bind _fpcamera (Variables|/Game/_Main/Blueprints/BP_Jack.BP_Jack_C|GetFPCamera _jack_ref_2))
  (bind _ads_alpha (Variables|/Game/_Main/Blueprints/BP_Jack.BP_Jack_C|GetADS_Alpha _jack_ref))
  (bind _weapon_primary (Variables|/Game/_Main/Blueprints/BP_Jack.BP_Jack_C|GetWeapon_Primary _jack_ref_2))
  (bind _returnvalue (Transformation|GetWorldLocation _fpcamera))
  (bind _currentactivesocket (Variables|/Game/_Main/Blueprints/Weapons_BP/BP_WeaponBase.BP_WeaponBase_C|GetCurrentActiveSocket _weapon_primary))
  (bind _weaponmesh (Variables|/Game/_Main/Blueprints/Weapons_BP/BP_WeaponBase.BP_WeaponBase_C|GetWeaponMesh _weapon_primary))
  (bind _returnvalue_2 (Utilities|String|StringToName _currentactivesocket))
  (bind _returnvalue_3 (Transformation|GetSocketTransform _weaponmesh _returnvalue_2 "RTS_World"))
  (bind (_location _rotation) (Math|Transform|BreakTransform _returnvalue_3))
  (bind _returnvalue_4 (Math|Vector|GetForwardVector _rotation))
  (bind _returnvalue_5 (- _returnvalue _location))
  (Utilities|IsValid (Variables|Default|GetJack_Ref)
    (:Is%20Valid
      (Utilities|IsValid _weapon_primary
        (:Is%20Valid
          (Variables|Default|SetFinalCamRot (Pawn|GetControlRotation _jack_ref :!class /Script/Engine.Pawn))
          (Variables|Default|SetFinalCamLoc (+ (Math|Vector|RotateVector (Variables|Default|GetSwayOffset) (Variables|Default|GetFinalCamRot)) (Math|Vector|Lerp(Vector) _returnvalue (- _location (* _returnvalue_4 (* (Math|Vector|DotProduct (Math|Vector|Normalize _returnvalue_5 0.0) _returnvalue_4) (/ (Math|Vector|VectorLength _returnvalue_5) 2.5e+03)))) _ads_alpha)))
          (return (Variables|Default|GetFinalCamLoc) (Variables|Default|GetFinalCamRot) (Math|Float|Lerp _newcamerabasefov (- _newcamerabasefov (Variables|/Game/_Main/Blueprints/Weapons_BP/BP_WeaponBase.BP_WeaponBase_C|GetNewFOV_ForOptic _weapon_primary)) _ads_alpha) true))))
    (:Is%20Not%20Valid
      (Development|PrintString "Ahhhhhh" true true "(R=0.000000,G=0.000000,B=0.000000,A=1.000000)" 1e+01))))