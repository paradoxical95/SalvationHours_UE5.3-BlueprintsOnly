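; BP_Menu3D is a main menu actor that hosts a 3D widget and links to other menus that the player's view can move between.
; On BeginPlay it binds to its Menu3DWidget's transition event and disables its own collision.
; A transition request looks up the index in LinkedMenus, moves collision from this actor to the target menu, and eases the player's view target over to it.
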(event Custom|Event_TransitionTo
  (params (NewMenu :type BP%20Menu%203D%20Object%20Reference))
  (Collision|SetActorEnableCollision false)
  (Collision|SetActorEnableCollision NewMenu true)
  (Game|Player|SetViewTargetwithBlend (Game|GetPlayerController 0) NewMenu 1.355 "VTBlend_EaseInOut" 1.8 false))

(event Custom|OnTransitionBetweenMenus
  (params (MenuIndex :type Integer))
  (bind _linkedmenus (Variables|Default|GetLinkedMenus))
  (if (Utilities|Array|IsValidIndex _linkedmenus MenuIndex)
    (CallFunction|EventTransitionto (Utilities|Array|Get(acopy) _linkedmenus MenuIndex))))

(event EventBeginPlay
  (bind _asmenu_3dwidget (Utilities|Casting|CastToMenu3DWidget (UserInterface|GetUserWidgetObject (Variables|Default|GetWidget))))
  (EventDispatchers|BindEventtoTransitiontoLinkedMenu _asmenu_3dwidget (delegate Custom|OnTransitionBetweenMenus))
  (Collision|SetActorEnableCollision false))

(fn ConstructionScript)