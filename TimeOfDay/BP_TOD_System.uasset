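; Time-of-day Blueprint meant to rotate sun and moon lights for a day-night cycle, but its main logic is not connected to Tick or any other event.
; That logic advances a Clock function, which converts scaled rotation into hours and minutes from a 12:00 start.
; Sun pitch thresholds, gated by DoOnce nodes, play or reverse a Transition timeline that blends sun and skylight intensity.
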(event EventBeginPlay)

(event EventTick
  (params (DeltaSeconds :type Float%20%28single-precision%29)))

(fn ConstructionScript)

(fn Clock
  (params (Delta :type Float%20%28double-precision%29))
  (bind _output_get (Variables|Default|SetTick (+ (* Delta 2.4e+02) (Variables|Default|GetTick)))) ; increments througout
  (bind _output_get_2 (Variables|Default|SetTime (Math|Timespan|MakeTimespan 0 12 0 (Math|Float|Truncate _output_get))))
  (Variables|Default|SetCurrentHours (.Hours (Math|Timespan|BreakTimespan _output_get_2)))
  (Variables|Default|SetCurrentMinutes (.Minutes (Math|Timespan|BreakTimespan _output_get_2)))
  (Utilities|IsValid 0))