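; Black soot decal Blueprint with a selectable texture, sort order and scale.
; On BeginPlay, a custom event creates a dynamic material instance, sets one of two soot textures, then applies the sort order and Y/Z scale with a fixed thin X depth.
; The Construction Script's uniform-scaling logic and setup call are disconnected, so they never run.
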(event Custom|Event_SetDecalData
  (bind _decal (Variables|Default|GetDecal))
  (bind _returnvalue (Rendering|Material|CreateDynamicMaterialInstance _decal :!class /Script/Engine.DecalComponent))
  (Rendering|Material|SetTextureParameterValue _returnvalue "Texture" (Utilities|Select :Index (Variables|Default|GetTextureSelector) :Option%200 "/Game/_Main/Blueprints/Decals_Custom/DecalTex/BlackSoot_1.BlackSoot_1" :Option%201 "/Game/_Main/Blueprints/Decals_Custom/DecalTex/BlackSoot_3.BlackSoot_3"))
  (Class|DecalComponent|SetSortOrder _decal (Variables|Default|GetDecalSortOrder))
  (Transformation|SetRelativeScale3D _decal (Math|Vector|MakeVector 0.1 (Variables|Default|GetDecalScale_Y) (Variables|Default|GetDecalScale_Z))))

(event EventBeginPlay
  (CallFunction|EventSetDecalData))

(fn ConstructionScript)