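; Procedural boundary wall Blueprint: a single door flanked by repeated wall sections, with a switchable lamp.
; The construction script applies the selected door mesh and material, then uses a macro to build right and left runs as instanced static meshes; unconnected logic for further sides remains.
; BeginPlay re-randomizes the door's look.
; ToggleLighting switches the point light and lamp emissive after a random delay, staggering changes.
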(event EventBeginPlay
  (bind _door (Variables|Default|GetDoor))
  (Components|StaticMesh|SetStaticMesh _door (.OutItem (Utilities|Array|Random (Variables|Default|GetDoorMeshes))))
  (Rendering|Material|SetMaterial _door 0 (.OutItem (Utilities|Array|Random (Variables|Default|GetDoorMaterials)))))

(event EventToggleLighting
  (params (Enable? :type Boolean))
  ;[1 1 1] New Code
  (if Enable?
    (Utilities|FlowControl|Delay (Math|Random|RandomFloatinRange 0.5 2.5))
    (Rendering|SetVisibility (Variables|Default|GetPointLight) true false)
    (bind _returnvalue (Rendering|Material|CreateDynamicMaterialInstance (Variables|Default|GetLamp) 0 "/Game/_Main/Assets/Props/OtherProps/Sketchfab/Mat/CeilingLamp_Classic.CeilingLamp_Classic" "None" :!class /Script/Engine.PrimitiveComponent))
    (Rendering|Material|SetScalarParameterValue _returnvalue "Emissive" 15.0 :!class /Script/Engine.MaterialInstanceDynamic)
    (else
      (Utilities|FlowControl|Delay (Math|Random|RandomFloatinRange 0.5 2.5))
      (Rendering|SetVisibility (Variables|Default|GetPointLight) false false)
      (bind _returnvalue_2 (Rendering|Material|CreateDynamicMaterialInstance (Variables|Default|GetLamp) 0 "/Game/_Main/Assets/Props/OtherProps/Sketchfab/Mat/CeilingLamp_Classic.CeilingLamp_Classic" "None" :!class /Script/Engine.PrimitiveComponent))
      (Rendering|Material|SetScalarParameterValue _returnvalue_2 "Emissive" 0.5 :!class /Script/Engine.MaterialInstanceDynamic))))

(fn ConstructionScript
  (bind _door (Variables|Default|GetDoor))
  (Components|StaticMesh|SetStaticMesh _door (Utilities|Array|Get(acopy) (Variables|Default|GetDoorMeshes) (Variables|Controllers|GetDoorMeshSelector)))
  (Rendering|Material|SetMaterial _door 0 (Utilities|Array|Get(acopy) (Variables|Default|GetDoorMaterials) (Variables|Controllers|GetDoorMaterialSelector)))
  ;[1 1 1] Set 1
  (Utilities|InstancedWallMacro (Variables|Controllers|GetWall_Copies_Rt) (Variables|/Script/Engine.SceneComponent|GetRelativeLocation (Variables|Default|GetDoor)) 0.0 (Variables|ControllersLine1|GetY_Offset) 0.0 (Variables|ControllersLine1|GetRepeatingWidth) 0.0)
  (Utilities|InstancedWallMacro (Variables|Controllers|GetWall_Copies_Lt) (Variables|/Script/Engine.SceneComponent|GetRelativeLocation (Variables|Default|GetDoor)) 0.0 (* (* (+ (Variables|Controllers|GetWall_Copies_Lt) 1) (Variables|ControllersLine1|GetRepeatingWidth)) -1.0) 0.0 (Variables|ControllersLine1|GetRepeatingWidth) 1.8e+02))

(fn FetchArrowsfromVehicles
  (params (Seat :type E_VehicleSeat%20Enum :default "NewEnumerator0"))
  (return "0, 0, 0" "0, 0, 0"))

(fn GetVehicleNameandLoc
  (return "NewEnumerator0" "0, 0, 0"))

(fn ObtainTrunkArrowsPickup
  (params (Seat%281-6%29 :type Integer))
  (return "0, 0, 0" "0, 0, 0"))

(fn PlayerDependentLight?
  (return false))