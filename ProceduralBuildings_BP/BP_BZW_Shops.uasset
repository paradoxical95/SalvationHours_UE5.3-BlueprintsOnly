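; Procedural shop building Blueprint that shows a selectable shop mesh with a toggleable point light.
; The construction script and BeginPlay set the mesh from an array by ShopSelector, and BeginPlay also applies one of three materials at random.
; ToggleLighting shows or hides the light after a short random delay.
; The remaining functions, mostly vehicle queries, are stubs returning default values.
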(event EventBeginPlay
  (bind _mesh (Variables|Default|GetMesh))
  (Components|StaticMesh|SetStaticMesh _mesh (Utilities|Array|Get(acopy) (Variables|Default|GetMeshArray) (Variables|Default|GetShopSelector)))
  (Rendering|Material|SetMaterial _mesh 0 (Utilities|Array|Get(acopy) (Variables|Default|GetMaterialArray) (Math|Random|RandomIntegerinRange 0 2))))

(event EventToggleLighting
  (params (Enable? :type Boolean))
  ;[1 1 1] New Code
  (if Enable?
    (Utilities|FlowControl|Delay (Math|Random|RandomFloatinRange 0.5 2.5))
    (Rendering|SetVisibility (Variables|Default|GetPointLight) true false)
    (else
      (Utilities|FlowControl|Delay (Math|Random|RandomFloatinRange 0.5 2.5))
      (Rendering|SetVisibility (Variables|Default|GetPointLight) false false))))

(fn ConstructionScript
  (Components|StaticMesh|SetStaticMesh (Variables|Default|GetMesh) (Utilities|Array|Get(acopy) (Variables|Default|GetMeshArray) (Variables|Default|GetShopSelector))))

(fn FetchArrowsfromVehicles
  (params (Seat :type E_VehicleSeat%20Enum :default "NewEnumerator0"))
  (return "0, 0, 0" "0, 0, 0"))

(fn GetVehicleNameandLoc
  (return "NewEnumerator0" "0, 0, 0" "0, 0, 0"))

(fn IsVehicleMoving?
  (return false))

(fn ObtainTrunkArrowsPickup
  (params (Seat%281-6%29 :type Integer))
  (return "0, 0, 0" "0, 0, 0"))

(fn PlayerDependentLight?
  (return false))