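; BP_BuidlingsSetup is a procedural building actor that sets up a house mesh with a signboard in its construction script.
; It applies the selected mesh and a random material from HouseMat, targeting slot 1 for House2 and slot 0 otherwise.
; The signboard takes its visibility and transform from variables and randomly gets a clothing or store material.
; Randomization is unseeded, so materials can change whenever construction reruns.
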(event EventBeginPlay)

(fn ConstructionScript
  (bind _mainmesh (Variables|Default|GetMainMesh))
  (bind _housemesh (Variables|Default|GetHouseMesh))
  (bind _signboard (Variables|Default|GetSignBoard))
  (Components|StaticMesh|SetStaticMesh _mainmesh _housemesh)
  (Rendering|Material|CreateDynamicMaterialInstance _mainmesh (select (== _housemesh "/Game/_Main/Assets/BenghaziBuildings/House2.House2") 1 0) (.OutItem (Utilities|Array|Random (Variables|Default|GetHouseMat))) "None" :!class /Script/Engine.PrimitiveComponent)
  (Rendering|SetVisibility _signboard (Variables|Default|GetSignBoardVisible?) false)
  (Rendering|Material|CreateDynamicMaterialInstance _signboard 0 (select (Math|Random|RandomBool) "/Game/_Main/Assets/BenghaziBuildings/Asset_Props/Mat/SignBoard2_Clothing_Mat.SignBoard2_Clothing_Mat" "/Game/_Main/Assets/BenghaziBuildings/Asset_Props/Mat/MI_SignBoard2_Store.MI_SignBoard2_Store") "None" :!class /Script/Engine.PrimitiveComponent)
  (Transformation|SetRelativeTransform _signboard (Variables|Default|GetSignBoardTransform) false false))