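; Small procedural house Blueprint that randomizes its look at BeginPlay, with an empty construction script.
; One random material is applied to material slot 0 of both floors, and Prop1 gets a random mesh.
; A weighted roll usually shows the second floor (HouseSmall) and its children, otherwise hides them.
; The Flip2ndFloor variable, not randomized here, turns that floor 180 degrees and offsets it along Y.
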(event EventBeginPlay
  (bind _house_small (Variables|Default|GetHouse_Small))
  (bind _house_small_2 (Variables|Default|GetHouse_Small))
  (bind _flip2ndfloor_ (Variables|Default|GetFlip2ndFloor?))
  (bind _house_small_3 (Variables|Default|GetHouse_Small))
  (bind _relativelocation (Variables|/Script/Engine.SceneComponent|GetRelativeLocation _house_small_3))
  (bind _relativerotation (Variables|/Script/Engine.SceneComponent|GetRelativeRotation _house_small))
  (Rendering|Material|SetMaterial (Variables|Default|GetHouse_GroundFloor) 0 (.OutItem (Utilities|Array|Random (Variables|Default|GetMaterials))))
  (Components|StaticMesh|SetStaticMesh (Variables|Default|GetProp1) (.OutItem (Utilities|Array|Random (Variables|Default|GetPropsMeshes))))
  (Variables|Default|Set2FloorHouse? (Math|Random|RandomBoolwithWeight 0.75))
  (Rendering|SetVisibility _house_small_2 (Variables|Default|Get2FloorHouse?) true)
  (Transformation|SetRelativeTransform _house_small_2 (Math|Transform|MakeTransform (select _flip2ndfloor_ (+ _relativelocation "0,170.000000,0") _relativelocation) (select _flip2ndfloor_ (Math|Rotator|CombineRotators _relativerotation "0,180.000000, 0") _relativerotation)) false false))

(fn ConstructionScript)