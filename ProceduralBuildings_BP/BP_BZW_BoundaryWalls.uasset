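; Procedural boundary wall actor that builds a perimeter of repeated wall meshes around a door, with a lamp and light.
; The construction script applies the selected door and chains Box markers to place four instanced-mesh wall runs, sized by copy count and repeat width.
; BeginPlay re-randomizes the door mesh and material and shows one of two lamps.
; ToggleLighting switches the point light and lamp emissive after a random delay.
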(event EventBeginPlay
  (bind _door (Variables|Default|GetDoor))
  (Components|StaticMesh|SetStaticMesh _door (.OutItem (Utilities|Array|Random (Variables|Default|GetDoorMeshes))))
  (Rendering|Material|SetMaterial _door 0 (.OutItem (Utilities|Array|Random (Variables|Default|GetDoorMaterials))))
  (if (Math|Random|RandomBoolwithWeight 0.55)
    (Rendering|SetVisibility (Variables|Default|GetLamp_1) true false)
    (Rendering|SetVisibility (Variables|Default|GetLamp_2) false false)
    (else
      (Rendering|SetVisibility (Variables|Default|GetLamp_1) false false)
      (Rendering|SetVisibility (Variables|Default|GetLamp_2) true false))))

(event EventToggleLighting
  (params (Enable? :type Boolean))
  ;[1 1 1] New Code
  (if Enable?
    (Utilities|FlowControl|Delay (Math|Random|RandomFloatinRange 0.5 2.5))
    (Rendering|SetVisibility (Variables|Default|GetPointLight) true false)
    (bind _returnvalue (Rendering|Material|CreateDynamicMaterialInstance (Variables|Default|GetLamp_1) 0 "/Game/_Main/Assets/Props/OtherProps/Sketchfab/Mat/CeilingLamp_Classic.CeilingLamp_Classic" "None" :!class /Script/Engine.PrimitiveComponent))
    (Rendering|Material|SetScalarParameterValue _returnvalue "Emissive" 15.0 :!class /Script/Engine.MaterialInstanceDynamic)
    (bind _returnvalue_2 (Rendering|Material|CreateDynamicMaterialInstance (Variables|Default|GetLamp_2) 1 "/Game/_Main/Assets/Props/OtherProps/Custom/Mat/WallLamp_Emissive.WallLamp_Emissive" "None" :!class /Script/Engine.PrimitiveComponent))
    (Rendering|Material|SetScalarParameterValue _returnvalue_2 "Emissive" 15.0 :!class /Script/Engine.MaterialInstanceDynamic)
    (else
      (Utilities|FlowControl|Delay (Math|Random|RandomFloatinRange 0.5 2.5))
      (Rendering|SetVisibility (Variables|Default|GetPointLight) false false)
      (bind _returnvalue_3 (Rendering|Material|CreateDynamicMaterialInstance (Variables|Default|GetLamp_1) 0 "/Game/_Main/Assets/Props/OtherProps/Sketchfab/Mat/CeilingLamp_Classic.CeilingLamp_Classic" "None" :!class /Script/Engine.PrimitiveComponent))
      (Rendering|Material|SetScalarParameterValue _returnvalue_3 "Emissive" 0.5 :!class /Script/Engine.MaterialInstanceDynamic)
      (bind _returnvalue_4 (Rendering|Material|CreateDynamicMaterialInstance (Variables|Default|GetLamp_2) 1 "/Game/_Main/Assets/Props/OtherProps/Custom/Mat/WallLamp_Emissive.WallLamp_Emissive" "None" :!class /Script/Engine.PrimitiveComponent))
      (Rendering|Material|SetScalarParameterValue _returnvalue_4 "Emissive" 0.5 :!class /Script/Engine.MaterialInstanceDynamic))))

(fn ConstructionScript
  (bind _door (Variables|Default|GetDoor))
  (Components|StaticMesh|SetStaticMesh _door (Utilities|Array|Get(acopy) (Variables|Default|GetDoorMeshes) (Variables|Controllers|GetDoorMeshSelector)))
  (Rendering|Material|SetMaterial _door 0 (Utilities|Array|Get(acopy) (Variables|Default|GetDoorMaterials) (Variables|Controllers|GetDoorMaterialSelector)))
  ;[1 1 1] Set 1
  (Utilities|InstancedWallMacro (Variables|Controllers|GetWall_Copies) (Variables|/Script/Engine.SceneComponent|GetRelativeLocation (Variables|Default|GetDoor)) 0.0 (Variables|ControllersLine1|GetY_Offset) (Variables|ControllersLine1|GetRepeatingWidth) 0.0 0.0)
  ;[1 1 1] Set 2 3 4 5
  (Transformation|SetRelativeLocation (Variables|Default|GetBox1) (+ (Variables|/Script/Engine.SceneComponent|GetRelativeLocation (Variables|Default|GetDoor)) (Math|Vector|MakeVector 0.0 (+ (* (Variables|ControllersLine1|GetRepeatingWidth) (+ (Variables|Controllers|GetWall_Copies) 1)) (* (Variables|ControllersLine1|GetY_Offset) 0.5)) 0.0)) false false)
  (Utilities|InstancedWallMacro (Variables|Controllers|GetWall_Copies) (Variables|/Script/Engine.SceneComponent|GetRelativeLocation (Variables|Default|GetBox1)) -212.0 0.0 0.0 (* (Variables|ControllersLine1|GetRepeatingWidth) -1.0) 9e+01)
  (Transformation|SetRelativeLocation (Variables|Default|GetBox2) (+ (Variables|/Script/Engine.SceneComponent|GetRelativeLocation (Variables|Default|GetBox1)) (Math|Vector|MakeVector (* (* (Variables|ControllersLine1|GetRepeatingWidth) (+ (Variables|Controllers|GetWall_Copies) 1)) -1.0) 0.0 0.0)) false false)
  (Utilities|InstancedWallMacro (+ (Variables|Controllers|GetWall_Copies) 1) (Variables|/Script/Engine.SceneComponent|GetRelativeLocation (Variables|Default|GetBox2)) 0.0 -212.0 (* (Variables|ControllersLine1|GetRepeatingWidth) -1.0) 0.0 1.8e+02)
  (Transformation|SetRelativeLocation (Variables|Default|GetBox3) (+ (Variables|/Script/Engine.SceneComponent|GetRelativeLocation (Variables|Default|GetBox2)) (Math|Vector|MakeVector 0.0 (* (+ (* (Variables|ControllersLine1|GetRepeatingWidth) (+ (Variables|Controllers|GetWall_Copies) 1)) 515.0) -1.0) 0.0)) false false)
  (Utilities|InstancedWallMacro (Variables|Controllers|GetWall_Copies) (Variables|/Script/Engine.SceneComponent|GetRelativeLocation (Variables|Default|GetBox3)) 212.0 0.0 0.0 (Variables|ControllersLine1|GetRepeatingWidth) 9e+01)
  (Transformation|SetRelativeLocation (Variables|Default|GetExtraWall) (+ (Variables|/Script/Engine.SceneComponent|GetRelativeLocation (Variables|Default|GetDoor)) (Math|Vector|MakeVector (* (* (Variables|ControllersLine1|GetRepeatingWidth) (+ (Variables|Controllers|GetWall_Copies) 1)) -1.0) -6e+01 0.0)) false false))

(fn FetchArrowsfromVehicles
  (params (Seat :type E_VehicleSeat%20Enum :default "NewEnumerator0"))
  (return "0, 0, 0" "0, 0, 0"))

(fn GetVehicleNameandLoc
  (return "NewEnumerator0" "0, 0, 0"))

(fn ObtainTrunkArrowsPickup
  (params (Seat%281-6%29 :type Integer))
  (return "0, 0, 0" "0, 0, 0"))

(fn PlayerDependentLight?
  (return false))