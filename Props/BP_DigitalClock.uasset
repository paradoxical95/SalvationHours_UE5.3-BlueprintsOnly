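; Digital clock prop that shows a name label and the current time, shifted by its own hour and minute offsets.
; BeginPlay sets the label, and UpdateClockTiming, meant to be called by the Game Instance, stores the time and writes zero-padded hour and minute texts.
; Offsets are added without wraparound at 24 or 60.
; Vehicle seat, trunk, name and light functions are stubs returning defaults.
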(event EventBeginPlay
  (Rendering|Components|TextRender|SetText (Variables|Default|GetClockName) (Variables|Default|GetName)))

(event EventUpdateClockTiming
  (params (Hours :type Integer) (Minutes :type Integer))
  (Variables|Default|SetCurrentTimeHours Hours)
  (Variables|Default|SetCurrentTimeMinutes Minutes)
  (Rendering|Components|TextRender|SetText (Variables|Default|GetHours) (Utilities|Text|ToText(String) (select (< (+ (Variables|Default|GetCurrentTimeHours) (Variables|Default|GetOffsetHours)) 10) (Utilities|String|Append "0" (Utilities|String|ToString(Integer) (+ (Variables|Default|GetCurrentTimeHours) (Variables|Default|GetOffsetHours)))) (Utilities|String|ToString(Integer) (+ (Variables|Default|GetCurrentTimeHours) (Variables|Default|GetOffsetHours))))))
  (Rendering|Components|TextRender|SetText (Variables|Default|GetMinutes) (Utilities|Text|ToText(String) (select (< (+ (Variables|Default|GetCurrentTimeMinutes) (Variables|Default|GetOffsetMinutes)) 10) (Utilities|String|Append "0" (Utilities|String|ToString(Integer) (+ (Variables|Default|GetCurrentTimeMinutes) (Variables|Default|GetOffsetMinutes)))) (Utilities|String|ToString(Integer) (+ (Variables|Default|GetCurrentTimeMinutes) (Variables|Default|GetOffsetMinutes)))))))

(fn ConstructionScript)

(fn FetchArrowsfromVehicles
  (params (Seat :type E_VehicleSeat%20Enum :default "NewEnumerator0"))
  (return "0, 0, 0" "0, 0, 0"))

(fn GetVehicleNameandLoc
  (return "NewEnumerator0" "0, 0, 0"))

(fn ObtainTrunkArrowsPickup
  (params (Seat%281-6%29 :type Integer))
  (return "0, 0, 0" "0, 0, 0"))

(fn PlayerDependentLight?
  (return false))