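; Monitor and keyboard prop that randomizes whether its screen is on and what it displays.
; On BeginPlay the Screen component is shown if ScreenVisible is set, otherwise with a 75 percent chance.
; A visible screen gets a dynamic instance of MI_LCD_Screen with a ScreenTexture from PCScreenTextures.
; LCDSelector picks that texture when ScreenVisible is set; otherwise it is a random one of the first five.
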(event EventBeginPlay
  (bind _screen (Variables|Default|GetScreen))
  (Rendering|SetVisibility _screen (select (Variables|Default|GetScreenVisible?) true (Math|Random|RandomBoolwithWeight 0.75)) false)
  (if (Rendering|IsVisible _screen)
    (bind _returnvalue (Rendering|Material|CreateDynamicMaterialInstance (Variables|Default|GetScreen) 0 "/Game/_Main/Assets/Props/OtherProps/Basemesh/Mat/MI_LCD_Screen.MI_LCD_Screen" "None" :!class /Script/Engine.PrimitiveComponent))
    (Rendering|Material|SetTextureParameterValue _returnvalue "ScreenTexture" (Utilities|Array|Get(acopy) (Variables|Default|GetPCScreenTextures) (select (Variables|Default|GetScreenVisible?) (Variables|Default|GetLCD%20Selector) (Math|Random|RandomIntegerinRange 0 4))))))

(fn ConstructionScript)