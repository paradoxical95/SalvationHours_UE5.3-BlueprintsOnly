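; BP_Props_MonitorVertical is a vertical monitor prop that randomizes whether its screen is lit and what it shows.
; On BeginPlay the screen is forced visible or shown by weighted chance, then gets a dynamic LCD material with a chosen CCTV texture or random PC screen texture.
; A custom event for the Ch4Seg13 TOC entry swaps it to one of two command screen textures at random.
; The construction script's preview logic is disconnected.
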(event Custom|Event_SwitchToCMDScreen
  (bind _returnvalue (Rendering|Material|CreateDynamicMaterialInstance (Variables|Default|GetScreen) 0 "/Game/_Main/Assets/Props/OtherProps/Basemesh/Mat/MI_LCD_Screen.MI_LCD_Screen" "None" :!class /Script/Engine.PrimitiveComponent))
  (Rendering|Material|SetTextureParameterValue _returnvalue "ScreenTexture" (Utilities|Array|Get(acopy) (Variables|Default|GetPCScreenTextures) (select (Math|Random|RandomBoolwithWeight 0.45) 4 3))))

(event EventBeginPlay
  (bind _screen (Variables|Default|GetScreen))
  (bind _pcscreentextures (Variables|Default|GetPCScreenTextures))
  (if (Variables|Default|GetScreenVisible?)
    (Rendering|SetVisibility _screen true false)
    (else
      (Rendering|SetVisibility _screen (Math|Random|RandomBoolwithWeight 0.75) false)))
  (if (Rendering|IsVisible _screen)
    (bind _returnvalue (Rendering|Material|CreateDynamicMaterialInstance (Variables|Default|GetScreen) 0 "/Game/_Main/Assets/Props/OtherProps/Basemesh/Mat/MI_LCD_Screen.MI_LCD_Screen" "None" :!class /Script/Engine.PrimitiveComponent))
    (Rendering|Material|SetTextureParameterValue _returnvalue "ScreenTexture" (select (Variables|Default|GetSMC_CCTV?) (Utilities|Array|Get(acopy) (Variables|Default|GetCCTV_Textures) (Variables|Default|GetCCTV_Number)) (Utilities|Array|Get(acopy) _pcscreentextures (Math|Random|RandomIntegerinRange 0 (- (Utilities|Array|Length _pcscreentextures) 1)))))))

(fn ConstructionScript)