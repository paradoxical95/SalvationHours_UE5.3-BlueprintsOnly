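; Laptop prop Blueprint that dresses a scene with a randomized screen and an adjustable screen angle.
; The construction script sets the roll of the LaptopScreen component from the ScreenRotation variable.
; On BeginPlay the Screen is visible 95% of the time; when visible, it gets a dynamic LCD material instance with a random texture from PCScreenTextures.
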(event EventBeginPlay
  (bind _screen (Variables|Default|GetScreen))
  (Rendering|SetVisibility _screen (Math|Random|RandomBoolwithWeight 0.95) false)
  (if (Rendering|IsVisible _screen)
    (bind _returnvalue (Rendering|Material|CreateDynamicMaterialInstance (Variables|Default|GetScreen) 0 "/Game/_Main/Assets/Props/OtherProps/Basemesh/Mat/MI_LCD_Screen.MI_LCD_Screen" "None" :!class /Script/Engine.PrimitiveComponent))
    (Rendering|Material|SetTextureParameterValue _returnvalue "ScreenTexture" (Utilities|Array|Get(acopy) (Variables|Default|GetPCScreenTextures) (Math|Random|RandomIntegerinRange 0 4)))))

(fn ConstructionScript
  (Transformation|SetRelativeRotation (Variables|Default|GetLaptopScreen) (Math|Rotator|MakeRotator (Variables|Default|GetScreenRotation) 0.0 0.0) false false))