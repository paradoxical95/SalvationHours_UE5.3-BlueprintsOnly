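; Hard drive story pickup for Chapter 4, Segment 12, which can display as a wired or unwired disk, or as a laptop.
; BeginPlay applies the variant, and sphere overlaps toggle the interact prompt for the "Jack"-tagged actor during that segment.
; The pickup event checks only the chapter, notifies the GameInstance, hides the disk meshes, plays a sound and destroys the actor.
; Vehicle and light query functions are stubs returning defaults.
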(event OnComponentBeginOverlap(Sphere)
  (params (OverlappedComponent :type Primitive%20Component%20Object%20Reference) (OtherActor :type Actor%20Object%20Reference) (OtherComp :type Primitive%20Component%20Object%20Reference) (OtherBodyIndex :type Integer) (bFromSweep :type Boolean) (SweepResult :type Hit%20Result%20Structure%20%28by%20ref%29))
  (bind _chsegstruct (Class|BPIntGameInstance|GIFetchChapterSegment(Message) (Game|GetGameInstance)))
  (if (and (Utilities|Enum|Equal(Enum) (.CH4_Segment (Utilities|Struct|BreakS_ChapterSegmentData _chsegstruct)) "NewEnumerator12") (Utilities|Enum|Equal(Enum) (.ChapterNumber? (Utilities|Struct|BreakS_ChapterSegmentData _chsegstruct)) "NewEnumerator3"))
    (if (Actor|ActorHasTag OtherActor "Jack")
      (Class|BPIntJack|ToggleInteractPromptPlayer(Message) OtherActor true))))

(event OnComponentEndOverlap(Sphere)
  (params (OverlappedComponent :type Primitive%20Component%20Object%20Reference) (OtherActor :type Actor%20Object%20Reference) (OtherComp :type Primitive%20Component%20Object%20Reference) (OtherBodyIndex :type Integer))
  (bind _chsegstruct (Class|BPIntGameInstance|GIFetchChapterSegment(Message) (Game|GetGameInstance)))
  (if (and (Utilities|Enum|Equal(Enum) (.CH4_Segment (Utilities|Struct|BreakS_ChapterSegmentData _chsegstruct)) "NewEnumerator12") (Utilities|Enum|Equal(Enum) (.ChapterNumber? (Utilities|Struct|BreakS_ChapterSegmentData _chsegstruct)) "NewEnumerator3"))
    (if (Actor|ActorHasTag OtherActor "Jack")
      (Class|BPIntJack|ToggleInteractPromptPlayer(Message) OtherActor false))))

(event EventBeginPlay
  (bind _switchtolaptop (Variables|Default|GetSwitchToLaptop))
  (Components|StaticMesh|SetStaticMesh (Variables|Default|GetHardDriveMesh) (select (Variables|Default|GetWiredHDD?) "/Game/_Main/Assets/Props/OtherProps/Sketchfab/HardDisk_Wired.HardDisk_Wired" "/Game/_Main/Assets/Props/OtherProps/Sketchfab/HardDisk.HardDisk"))
  (Rendering|SetVisibility (Variables|Default|GetLaptop) _switchtolaptop false)
  (Rendering|SetVisibility (Variables|Default|GetHardDisk) (not _switchtolaptop) false))

(event EventPickUpPropCh4Seg12
  (bind _chsegstruct (Class|BPIntGameInstance|GIFetchChapterSegment(Message) (Game|GetGameInstance)))
  (if (Utilities|Enum|Equal(Enum) (Utilities|Struct|BreakS_ChapterSegmentData _chsegstruct) "NewEnumerator3")
    (Class|BPIntGameInstance|GICH4PickupHDD(Message) (Game|GetGameInstance) true)
    (Rendering|SetVisibility (Variables|Default|GetHardDriveMesh) false false)
    (Audio|PlaySound2D "/Game/MilitaryWeapDark/Sound/Shotgun/Shotgun_AmmoPickup_Cue.Shotgun_AmmoPickup_Cue" 0.5 1.0 0.0 0 0)
    (Utilities|FlowControl|Delay 0.2)
    (Actor|DestroyActor)))

(fn ConstructionScript)

(fn FetchArrowsfromVehicles
  (params (Seat :type E_VehicleSeat%20Enum :default "NewEnumerator0"))
  (return "0, 0, 0" "0, 0, 0"))

(fn GetVehicleNameandLoc
  (return "NewEnumerator0" "0, 0, 0"))

(fn IsVehicleMoving?
  (return false))

(fn ObtainTrunkArrowsPickup
  (params (Seat%281-6%29 :type Integer))
  (return "0, 0, 0" "0, 0, 0"))

(fn PlayerDependentLight?
  (return false))