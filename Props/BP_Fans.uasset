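; BP_Fans is a spinning fan prop with selectable variants, each with its own mesh, spin speed and looping or ambient sound.
; The construction script applies the selected mesh and sets the RotatingMovement yaw rate from the RotationRate variable.
; On BeginPlay, SelectMesh again picks the mesh, replaces that rate with a hardcoded per-variant speed, and starts the matching air conditioner or table fan audio.
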(event EventBeginPlay
  (bind _audio (Variables|Default|GetAudio))
  (Components|StaticMesh|SetStaticMesh (Variables|Default|GetFan) (Utilities|Array|Get(acopy) (Variables|Default|GetFanMesh) (Variables|Default|GetSelectMesh)))
  (Variables|/Script/Engine.RotatingMovementComponent|SetRotationRate (Variables|Default|GetRotatingMovement) (Math|Rotator|MakeRotator 0.0 (Utilities|Select :Index (Variables|Default|GetSelectMesh) :Option%200 1e+03 :Option%201 7.5e+02) 0.0))
  (Audio|Components|Audio|SetSound _audio (Utilities|Select :Index (Variables|Default|GetSelectMesh) :Option%200 "/Game/_Main/Sounds/Props/AirConditioner.AirConditioner" :Option%201 "/Game/_Main/Sounds/Props/TableFan.TableFan"))
  (Components|Activation|Activate _audio false)
  (Audio|Components|Audio|Play _audio 0.0))

(fn ConstructionScript
  (Components|StaticMesh|SetStaticMesh (Variables|Default|GetFan) (Utilities|Array|Get(acopy) (Variables|Default|GetFanMesh) (Variables|Default|GetSelectMesh)))
  (Variables|/Script/Engine.RotatingMovementComponent|SetRotationRate (Variables|Default|GetRotatingMovement) (Math|Rotator|MakeRotator 0.0 (Variables|Default|GetRotation%20Rate) 0.0)))