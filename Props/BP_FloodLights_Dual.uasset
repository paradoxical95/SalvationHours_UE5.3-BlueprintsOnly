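; Dual floodlight prop that switches on and off, follows day and night events, and can be permanently broken when shot.
; Each switch sets emissive on two planes through dynamic material instances and toggles visibility of spotlights on separately referenced AttachedLights actors.
; ToggleLighting adds switch and hum audio, with a per-instance random delay staggering changes.
; DestroyLighting darkens it, removes collision, plays a break sound and notifies the GameInstance.
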(event Custom|ToggleLights
  (if (Variables|Default|GetLightDisabled?)
    (Development|PrintString "Light Turned off")
    (Utilities|Time|ClearandInvalidateTimerbyHandle (Variables|Default|GetTimer))))

(event Custom|Event_DayTime
  (CallFunction|SetEmissiveValue (Variables|Default|GetPlane) 0.05)
  (CallFunction|SetEmissiveValue (Variables|Default|GetPlane1) 0.05)
  (CallFunction|TurnOffLights false))

(event Custom|Event_NightTime
  (Utilities|FlowControl|Delay (Variables|Default|GetRandomDelay))
  (CallFunction|SetEmissiveValue (Variables|Default|GetPlane) 8.0)
  (CallFunction|SetEmissiveValue (Variables|Default|GetPlane1) 8.0)
  (CallFunction|TurnOffLights true) ; Controlling Lights from this BP
)

(event EventBeginPlay
  (Variables|Default|SetRandomDelay (Math|Random|RandomFloatinRange 0.5 3.0)))

(event EventToggleLighting
  (params (Enable? :type Boolean))
  (bind _audio (Variables|Default|GetAudio))
  (bind _audio_2 (Variables|Default|GetAudio))
  (bind _audio_3 (Variables|Default|GetAudio))
  (bind _randomdelay (Variables|Default|GetRandomDelay))
  ;[1 1 1] New Code
  (if Enable?
    (if (not (Variables|Default|GetLightDisabled?))
      (Utilities|FlowControl|Delay _randomdelay)
      (CallFunction|SetEmissiveValue (Variables|Default|GetPlane) 8.0)
      (CallFunction|SetEmissiveValue (Variables|Default|GetPlane1) 8.0)
      (CallFunction|TurnOffLights true) ; Controlling Lights from this BP
      (Components|Tick|SetComponentTickEnabled (Variables|Default|GetAudio) true)
      (Audio|Components|Audio|SetSound _audio_3 "/Game/_Main/Sounds/Props/Floodlights_On.Floodlights_On")
      (Components|Activation|Activate _audio_3 false)
      (Audio|Components|Audio|FadeIn _audio_3 0.0 1.0 0.0 "Linear" :!class /Script/Engine.AudioComponent)
      (Utilities|FlowControl|Delay 0.85)
      (Audio|Components|Audio|SetSound _audio "/Game/_Main/Sounds/Props/Floodlights_Humm.Floodlights_Humm")
      (Audio|Components|Audio|FadeIn _audio 1.0 1.0 0.0 "Linear" :!class /Script/Engine.AudioComponent))
    (else
      (Utilities|FlowControl|Delay _randomdelay)
      (CallFunction|SetEmissiveValue (Variables|Default|GetPlane) 0.05)
      (CallFunction|SetEmissiveValue (Variables|Default|GetPlane1) 0.05)
      (CallFunction|TurnOffLights false)
      (Audio|Components|Audio|SetSound _audio_2 "/Game/_Main/Sounds/Props/Floodlights_On.Floodlights_On")
      (Audio|Components|Audio|Play _audio_2 0.0)
      (Utilities|FlowControl|Delay 0.85)
      (Components|Activation|Deactivate _audio_2)
      (Components|Tick|SetComponentTickEnabled (Variables|Default|GetAudio) false))))

(event EventDestroyLighting
  (bind _audio (Variables|Default|GetAudio))
  ;[1 1 1] If player shoots it
  (if (not (Variables|Default|GetLightDisabled?))
    (Variables|Default|SetLightDisabled? true)
    (CallFunction|SetEmissiveValue (Variables|Default|GetPlane) 0.05)
    (CallFunction|SetEmissiveValue (Variables|Default|GetPlane1) 0.05)
    (CallFunction|TurnOffLights false)
    (Class|BPIntGameInstance|GITrackDestroyedAnnexLights(Message) (Game|GetGameInstance))
    (Collision|SetCollisionEnabled (Variables|Default|GetMesh) "NoCollision")
    (Components|Activation|Activate _audio false)
    (Audio|Components|Audio|SetSound _audio "/Game/_Main/Sounds/Props/Floodlights_Break.Floodlights_Break")
    (Audio|Components|Audio|FadeIn _audio 0.0 1.0 0.0 "Linear" :!class /Script/Engine.AudioComponent)
    (Utilities|FlowControl|Delay 0.8)
    (Components|Activation|Deactivate _audio)
    (Components|Tick|SetComponentTickEnabled (Variables|Default|GetAudio) false)))

(fn ConstructionScript)

(fn GetTime
  (params (Hours :type Integer))
  (Variables|Default|SetTimeInHours Hours))

(fn SetEmissiveValue
  (params (Mesh :type Primitive%20Component%20Object%20Reference) (Value :type Float%20%28single-precision%29))
  (bind _returnvalue (Rendering|Material|CreateDynamicMaterialInstance Mesh 0 "/Game/_Main/Assets/Props/OtherProps/Custom/Mat/FloodLights_Inst.FloodLights_Inst" "None" :!class /Script/Engine.PrimitiveComponent))
  (Rendering|Material|SetScalarParameterValue _returnvalue "Emissive" Value :!class /Script/Engine.MaterialInstanceDynamic))

(fn TurnOffLights
  (params (Enable%20Lights? :type Boolean))
  (if Enable%20Lights?
    (for _array_element (Variables|Default|GetAttachedLights)
      (Utilities|IsValid _array_element
        (:Is%20Valid
          (Rendering|SetVisibility (Variables|/Script/Engine.SpotLight|GetSpotLightComponent _array_element) true false))))
    (else
      (for _array_element_2 (Variables|Default|GetAttachedLights)
        (Utilities|IsValid _array_element_2
          (:Is%20Valid
            (Rendering|SetVisibility (Variables|/Script/Engine.SpotLight|GetSpotLightComponent _array_element_2) false false)))))))

(fn FetchArrowsfromVehicles
  (params (Seat :type E_VehicleSeat%20Enum :default "NewEnumerator0"))
  (return "0, 0, 0" "0, 0, 0"))

(fn GetVehicleNameandLoc
  (return "NewEnumerator0" "0, 0, 0"))

(fn ObtainTrunkArrowsPickup
  (params (Seat%281-6%29 :type Integer))
  (return "0, 0, 0" "0, 0, 0"))

(fn PlayerDependentLight?
  (return (Variables|Default|GetPlayerDependent?)))