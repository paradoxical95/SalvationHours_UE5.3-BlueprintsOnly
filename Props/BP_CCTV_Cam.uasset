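; BP_CCTV_Cam is a CCTV camera prop that can be aimed through two rotation variables.
; On BeginPlay it sets the relative yaw of its Rotator component from ZRotation and the pitch of CCTVBody from YRotation, with the other axes zeroed.
; The same calls sit disconnected in the Construction Script, so only BeginPlay applies the angles.
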(event EventBeginPlay
  (Transformation|SetRelativeRotation (Variables|Default|GetRotator) (Math|Rotator|MakeRotator 0.0 0.0 (Variables|Default|GetZ%20Rotation)) false false)
  (Transformation|SetRelativeRotation (Variables|Default|GetCCTV_Body) (Math|Rotator|MakeRotator 0.0 (Variables|Default|GetY%20Rotation) 0.0) false false))

(fn ConstructionScript)