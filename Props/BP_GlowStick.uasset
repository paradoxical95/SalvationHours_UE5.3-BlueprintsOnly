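; Glow stick prop that glows green or red, with an optional attached point light actor in the matching colour.
; BeginPlay sets the colour on a dynamic emissive material and on the light.
; ToggleLighting, when the light is valid, switches its visibility, intensity and mesh emissive, creating a fresh material instance each time without reapplying the colour.
; Vehicle seat, trunk and player-dependent light functions return only default values.
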(event EventBeginPlay
  (bind _attachedpointlight (Variables|Default|GetAttachedPointLight))
  (bind _glowcolorgreen (Variables|Default|GetGlowColorGreen))
  (bind _returnvalue (select _glowcolorgreen "(R=0.115812,G=1.000000,B=0.000000,A=1.000000)" "(R=1.000000,G=0.000000,B=0.010000,A=1.000000)"))
  (bind _returnvalue_2 (Rendering|Material|CreateDynamicMaterialInstance (Variables|Default|GetMesh) 1 "/Game/_Main/Assets/Props/OtherProps/Custom/Mat/GlowStick_Emissive_Mat.GlowStick_Emissive_Mat" "None" :!class /Script/Engine.PrimitiveComponent))
  (Rendering|Material|SetVectorParameterValue _returnvalue_2 "Color" _returnvalue :!class /Script/Engine.MaterialInstanceDynamic)
  (Utilities|IsValid _attachedpointlight
    (:Is%20Valid
      (Rendering|Components|Light|SetLightColor (Variables|/Script/Engine.PointLight|GetPointLightComponent _attachedpointlight) _returnvalue true))))

(event EventToggleLighting
  (params (Enable? :type Boolean))
  (bind _attachedpointlight (Variables|Default|GetAttachedPointLight))
  (bind _pointlightcomponent (Variables|/Script/Engine.PointLight|GetPointLightComponent _attachedpointlight))
  ;[1 1 1] New Code
  (if Enable?
    (Utilities|IsValid _attachedpointlight
      (:Is%20Valid
        (Rendering|SetVisibility _pointlightcomponent true false)
        (Rendering|Components|Light|SetIntensity _pointlightcomponent 1e+01)
        (bind _returnvalue (Rendering|Material|CreateDynamicMaterialInstance (Variables|Default|GetMesh) 1 "/Game/_Main/Assets/Props/OtherProps/Custom/Mat/GlowStick_Emissive_Mat.GlowStick_Emissive_Mat" "None" :!class /Script/Engine.PrimitiveComponent))
        (Rendering|Material|SetScalarParameterValue _returnvalue "Emissive" 2e+01 :!class /Script/Engine.MaterialInstanceDynamic)))
    (else
      (Utilities|IsValid _attachedpointlight
        (:Is%20Valid
          (Rendering|SetVisibility _pointlightcomponent false false)
          (Rendering|Components|Light|SetIntensity _pointlightcomponent 0.0)
          (bind _returnvalue_2 (Rendering|Material|CreateDynamicMaterialInstance (Variables|Default|GetMesh) 1 "/Game/_Main/Assets/Props/OtherProps/Custom/Mat/GlowStick_Emissive_Mat.GlowStick_Emissive_Mat" "None" :!class /Script/Engine.PrimitiveComponent))
          (Rendering|Material|SetScalarParameterValue _returnvalue_2 "Emissive" 0.5 :!class /Script/Engine.MaterialInstanceDynamic))))))

(fn ConstructionScript)

(fn FetchArrowsfromVehicles
  (params (Seat :type E_VehicleSeat%20Enum :default "NewEnumerator0"))
  (return "0, 0, 0" "0, 0, 0"))

(fn GetVehicleNameandLoc
  (return "NewEnumerator0" "0, 0, 0"))

(fn ObtainTrunkArrowsPickup
  (params (Seat%281-6%29 :type Integer))
  (return "0, 0, 0" "0, 0, 0"))

(fn PlayerDependentLight?
  (return false))