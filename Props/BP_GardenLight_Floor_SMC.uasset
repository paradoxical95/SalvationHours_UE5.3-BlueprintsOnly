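; Floor garden light prop that toggles its emissive plane and an optional attached light actor on or off.
; ToggleLighting creates a dynamic material instance on each call to set the glow, then shows or hides the attached light's root component.
; A random delay picked at BeginPlay staggers switch-on, while switch-off is immediate.
; Other functions store the time, set light intensity or return placeholder values, including unused vehicle queries.
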(event EventBeginPlay
  (Variables|Default|SetRandomDelay (Math|Random|RandomFloatinRange 1.0 6.0)))

(event EventToggleLighting
  (params (Enable? :type Boolean))
  (bind _plane (Variables|Default|GetPlane))
  (bind _attachedlight (Variables|Default|GetAttachedLight))
  (bind _attachedlight_2 (Variables|Default|GetAttachedLight))
  ;[1 1 1] New code
  (if Enable?
    (Utilities|FlowControl|Delay (Variables|Default|GetRandomDelay))
    ;[1 1 1] Emissive Plane
    (bind _returnvalue (Rendering|Material|CreateDynamicMaterialInstance _plane 0 "/Game/_Main/Assets/Props/OtherProps/Custom/Mat/ExtraLights_Emissive_Inst.ExtraLights_Emissive_Inst" "None" :!class /Script/Engine.PrimitiveComponent))
    (Rendering|Material|SetScalarParameterValue _returnvalue "Emissive" 8.5 :!class /Script/Engine.MaterialInstanceDynamic)
    ;[1 1 1] Light Toggle
    (Utilities|IsValid _attachedlight_2
      (:Is%20Valid
        (Rendering|SetVisibility (Variables|/Script/Engine.Actor|GetRootComponent _attachedlight_2) true false)))
    (else
      (bind _returnvalue_2 (Rendering|Material|CreateDynamicMaterialInstance _plane 0 "/Game/_Main/Assets/Props/OtherProps/Custom/Mat/ExtraLights_Emissive_Inst.ExtraLights_Emissive_Inst" "None" :!class /Script/Engine.PrimitiveComponent))
      (Rendering|Material|SetScalarParameterValue _returnvalue_2 "Emissive" 0.05 :!class /Script/Engine.MaterialInstanceDynamic)
      (Utilities|IsValid _attachedlight
        (:Is%20Valid
          (Rendering|SetVisibility (Variables|/Script/Engine.Actor|GetRootComponent _attachedlight) false false))))))

(fn ConstructionScript)

(fn GetTime
  (params (Hours :type Integer))
  (Variables|Default|SetTimeInHours Hours))

(fn LightIntensity
  (params (Target :type Light%20Component%20Object%20Reference) (Intensity :type Float%20%28single-precision%29))
  (Rendering|Components|Light|SetIntensity Target Intensity))

(fn FetchArrowsfromVehicles
  (params (Seat :type E_VehicleSeat%20Enum :default "NewEnumerator0"))
  (return "0, 0, 0" "0, 0, 0"))

(fn GetVehicleNameandLoc
  (return "NewEnumerator0" "0, 0, 0"))

(fn ObtainTrunkArrowsPickup
  (params (Seat%281-6%29 :type Integer))
  (return "0, 0, 0" "0, 0, 0"))

(fn PlayerDependentLight?
  (return false))