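; BP_Rpt_Props_HDD is a repeating prop Blueprint that builds rows of instanced meshes in the construction script, similar to an array modifier.
; Each RepeatingAsset entry gets its own instanced static mesh component with the entry's mesh and a dynamic instance of its material.
; Instances start at the entry's transform and step by RepeatWidth along X, Y or both, per the axis flags, with the count driven by Copies.
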(event EventBeginPlay)

(event Collision|EventActorBeginOverlap
  (params (OtherActor :type Actor%20Object%20Reference)))

(event EventTick
  (params (DeltaSeconds :type Float%20%28single-precision%29)))

(fn ConstructionScript
  (for _array_element (Variables|Default|GetRepeatingAsset)
    (bind _returnvalue (AddComponent|AddInstancedStaticMeshComponent false)) ; INSTANCED SM not standard SM
    (Components|StaticMesh|SetStaticMesh _returnvalue (.Mesh (Utilities|Struct|BreakS_RepeatingAssets _array_element))) ; will set that as the SM for this BP
    (bind _returnvalue_2 (Rendering|Material|CreateDynamicMaterialInstance _returnvalue 0 (.Material (Utilities|Struct|BreakS_RepeatingAssets _array_element)) "None" :!class /Script/Engine.PrimitiveComponent)) ; Create a dynamic Mat
    (Rendering|Material|SetMaterial _returnvalue 0 _returnvalue_2)
    (for _index (range 0 (Variables|Default|GetCopies))
      (Components|InstancedStaticMesh|AddInstance _returnvalue (Math|Transform|MakeTransform (Math|Vector|MakeVector (select (Variables|Default|GetX%20Axis?) (+ (* _index (Variables|Default|GetRepeatWidth)) (.x (.Location (Math|Transform|BreakTransform (.Transform (Utilities|Struct|BreakS_RepeatingAssets _array_element)))))) (.x (.Location (Math|Transform|BreakTransform (.Transform (Utilities|Struct|BreakS_RepeatingAssets _array_element)))))) (select (Variables|Default|GetY%20Axis?) (+ (* _index (Variables|Default|GetRepeatWidth)) (.y (.Location (Math|Transform|BreakTransform (.Transform (Utilities|Struct|BreakS_RepeatingAssets _array_element)))))) (.y (.Location (Math|Transform|BreakTransform (.Transform (Utilities|Struct|BreakS_RepeatingAssets _array_element)))))) (.z (.Location (Math|Transform|BreakTransform (.Transform (Utilities|Struct|BreakS_RepeatingAssets _array_element)))))) (.Rotation (Math|Transform|BreakTransform (.Transform (Utilities|Struct|BreakS_RepeatingAssets _array_element)))) (.Scale (Math|Transform|BreakTransform (.Transform (Utilities|Struct|BreakS_RepeatingAssets _array_element))))) false) ; modification on instance
    )))