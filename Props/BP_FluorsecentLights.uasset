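; Fluorescent light prop that offers a big and a small lamp variant in one actor.
; The construction script uses SelectMesh to show either LampBig or LampSmall, propagating visibility to child components.
; Nodes for intensity, turning lights off, attenuation radius, temperature and color are present but unconnected, so those settings are never applied.
; The event graph holds only disabled default events, so the Blueprint has no runtime logic.
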(event EventBeginPlay)

(event Collision|EventActorBeginOverlap
  (params (OtherActor :type Actor%20Object%20Reference)))

(event EventTick
  (params (DeltaSeconds :type Float%20%28single-precision%29)))

(fn ConstructionScript
  (bind _selectmesh (Variables|Default|GetSelectMesh))
  (Rendering|SetVisibility (Variables|Default|GetLamp_Small) (Utilities|Select :Index _selectmesh :Option%200 false :Option%201 true) true)
  (Rendering|SetVisibility (Variables|Default|GetLamp_Big) (Utilities|Select :Index _selectmesh :Option%200 true :Option%201 false) true))