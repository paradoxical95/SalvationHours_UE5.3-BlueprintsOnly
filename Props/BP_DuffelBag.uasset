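; BP_DuffelBag is a duffel bag prop that the player picks up during chapter 4, segment 12.
; A Sphere overlap toggles the interact prompt on the actor tagged Jack as it enters and leaves range.
; The PickUpPropCh4Seg12 event hides the Bag component, notifies the game instance of the pickup and plays a cloth swipe sound.
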(event OnComponentBeginOverlap(Sphere)
  (params (OverlappedComponent :type Primitive%20Component%20Object%20Reference) (OtherActor :type Actor%20Object%20Reference) (OtherComp :type Primitive%20Component%20Object%20Reference) (OtherBodyIndex :type Integer) (bFromSweep :type Boolean) (SweepResult :type Hit%20Result%20Structure%20%28by%20ref%29))
  (if (Actor|ActorHasTag OtherActor "Jack")
    (Class|BPIntJack|ToggleInteractPromptPlayer(Message) OtherActor true)))

(event OnComponentEndOverlap(Sphere)
  (params (OverlappedComponent :type Primitive%20Component%20Object%20Reference) (OtherActor :type Actor%20Object%20Reference) (OtherComp :type Primitive%20Component%20Object%20Reference) (OtherBodyIndex :type Integer))
  (if (Actor|ActorHasTag OtherActor "Jack")
    (Class|BPIntJack|ToggleInteractPromptPlayer(Message) OtherActor false)))

(event EventBeginPlay)

(event Collision|EventActorBeginOverlap
  (params (OtherActor :type Actor%20Object%20Reference)))

(event EventTick
  (params (DeltaSeconds :type Float%20%28single-precision%29)))

(event EventPickUpPropCh4Seg12
  (Rendering|SetVisibility (Variables|Default|GetBag) false false)
  (Class|BPIntGameInstance|GICH4PickupBag(Message) (Game|GetGameInstance) true)
  (Audio|PlaySound2D "/Game/Sounds/Foley/SCue_Foley_SwipeCloth.SCue_Foley_SwipeCloth" 0.5 1.0 0.0 0 0))

(fn ConstructionScript)