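; Wardrobe prop whose two doors swing open automatically when an actor tagged "Jack" enters its Box trigger and close when it leaves.
; Overlap begin plays the OpenCloseDoor timeline from the start, lerping the relative yaw of the Right and Left components in opposite directions to slightly different angles.
; Overlap end reverses the timeline from its end, so an interrupted swing snaps to an endpoint before animating.
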(event OnComponentBeginOverlap(Box)
  (params (OverlappedComponent :type Primitive%20Component%20Object%20Reference) (OtherActor :type Actor%20Object%20Reference) (OtherComp :type Primitive%20Component%20Object%20Reference) (OtherBodyIndex :type Integer) (bFromSweep :type Boolean) (SweepResult :type Hit%20Result%20Structure%20%28by%20ref%29))
  (if (Actor|ActorHasTag OtherActor "Jack")
    (bind _float (Timeline|OpenCloseDoor PlayFromStart)
      (:Update
        (Transformation|SetRelativeRotation (Variables|Default|GetRight) (Math|Rotator|MakeRotator 0.0 0.0 (Math|Float|Lerp 0.0 -8e+01 _float)) false false)
        (Transformation|SetRelativeRotation (Variables|Default|GetLeft) (Math|Rotator|MakeRotator 0.0 0.0 (Math|Float|Lerp 0.0 75.0 _float)) false false)))))

(event OnComponentEndOverlap(Box)
  (params (OverlappedComponent :type Primitive%20Component%20Object%20Reference) (OtherActor :type Actor%20Object%20Reference) (OtherComp :type Primitive%20Component%20Object%20Reference) (OtherBodyIndex :type Integer))
  (if (Actor|ActorHasTag OtherActor "Jack")
    (bind _float (Timeline|OpenCloseDoor ReverseFromEnd)
      (:Update
        (Transformation|SetRelativeRotation (Variables|Default|GetRight) (Math|Rotator|MakeRotator 0.0 0.0 (Math|Float|Lerp 0.0 -8e+01 _float)) false false)
        (Transformation|SetRelativeRotation (Variables|Default|GetLeft) (Math|Rotator|MakeRotator 0.0 0.0 (Math|Float|Lerp 0.0 75.0 _float)) false false)))))

(event EventBeginPlay)

(event Collision|EventActorBeginOverlap
  (params (OtherActor :type Actor%20Object%20Reference)))

(event EventTick
  (params (DeltaSeconds :type Float%20%28single-precision%29)))

(fn ConstructionScript)