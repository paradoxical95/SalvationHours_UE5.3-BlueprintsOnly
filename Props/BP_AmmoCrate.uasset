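; BP_AmmoCrate is an ammo crate prop that lets the player refill ammo while standing within its collision volume.
; Overlaps by an actor tagged "Jack" toggle that actor's refill permission and interact prompt via messages, along with the crate's text visibility.
; One timeline tilts the lid and raises the text on entry, reversing from its end on exit.
; The lid's initial rotation is saved on BeginPlay but never read here.
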(event OnComponentBeginOverlap(Collision)
  (params (OverlappedComponent :type Primitive%20Component%20Object%20Reference) (OtherActor :type Actor%20Object%20Reference) (OtherComp :type Primitive%20Component%20Object%20Reference) (OtherBodyIndex :type Integer) (bFromSweep :type Boolean) (SweepResult :type Hit%20Result%20Structure%20%28by%20ref%29))
  (if (Actor|ActorHasTag OtherActor "Jack")
    (Class|BPIntJack|AmmoRefillAllowed?(Message) OtherActor true)
    (Class|BPIntJack|ToggleInteractPromptPlayer(Message) OtherActor true)
    (Rendering|SetVisibility (Variables|Default|GetTextRender) true false)
    (bind _float (Timeline|LidRotation PlayFromStart)
      (:Update
        (Transformation|SetRelativeRotation (Variables|Default|GetLid) (Math|Rotator|Lerp(Rotator) "0, 0, 0" "0, 0,-11.000000" _float) false false)
        (Transformation|SetRelativeLocation (Variables|Default|GetTextRender) (Math|Vector|MakeVector -5e+01 -58.0 (Math|Float|Lerp -24.0 6e+01 _float)) false false)))))

(event OnComponentEndOverlap(Collision)
  (params (OverlappedComponent :type Primitive%20Component%20Object%20Reference) (OtherActor :type Actor%20Object%20Reference) (OtherComp :type Primitive%20Component%20Object%20Reference) (OtherBodyIndex :type Integer))
  (if (Actor|ActorHasTag OtherActor "Jack")
    (Class|BPIntJack|AmmoRefillAllowed?(Message) OtherActor false)
    (Class|BPIntJack|ToggleInteractPromptPlayer(Message) OtherActor false)
    (Rendering|SetVisibility (Variables|Default|GetTextRender) false false)
    (bind _float (Timeline|LidRotation ReverseFromEnd)
      (:Update
        (Transformation|SetRelativeRotation (Variables|Default|GetLid) (Math|Rotator|Lerp(Rotator) "0, 0, 0" "0, 0,-11.000000" _float) false false)
        (Transformation|SetRelativeLocation (Variables|Default|GetTextRender) (Math|Vector|MakeVector -5e+01 -58.0 (Math|Float|Lerp -24.0 6e+01 _float)) false false)))))

(event EventBeginPlay
  (Variables|Default|SetOriginalLidRotation (Variables|/Script/Engine.SceneComponent|GetRelativeRotation (Variables|Default|GetLid))))

(fn ConstructionScript)