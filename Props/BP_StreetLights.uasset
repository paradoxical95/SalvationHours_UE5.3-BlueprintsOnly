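; Street lamp prop that switches its spotlights on or off through the ToggleLighting event.
; At BeginPlay the DualLight flag selects the single or dual lamp mesh, and a random delay of a few seconds is rolled.
; Switching on waits for that delay, staggering lamps, while switching off is immediate; the second spotlight follows only on dual lamps.
; Helpers store the hour and set light intensity, while vehicle-related functions are empty stubs.
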(event EventBeginPlay
  (Components|StaticMesh|SetStaticMesh (Variables|Default|GetStaticMesh) (select (Variables|Default|GetDualLight?) "/Game/_Main/Assets/Props/OtherProps/Custom/StreetLamp_Dual.StreetLamp_Dual" "/Game/_Main/Assets/Props/OtherProps/Custom/StreetLamp_Single.StreetLamp_Single"))
  (Variables|Default|SetRandomDelay (Math|Random|RandomFloatinRange 1.0 6.0)))

(event EventToggleLighting
  (params (Enable? :type Boolean))
  ;[1 1 1] Light Toggle
  (if Enable?
    (Utilities|FlowControl|Delay (Variables|Default|GetRandomDelay))
    (Rendering|SetVisibility (Variables|Default|GetSpotLight_1) true false)
    (if (Variables|Default|GetDualLight?)
      (Rendering|SetVisibility (Variables|Default|GetSpotLight_2) true false))
    (else
      (Rendering|SetVisibility (Variables|Default|GetSpotLight_1) false false)
      (if (Variables|Default|GetDualLight?)
        (Rendering|SetVisibility (Variables|Default|GetSpotLight_2) false false)))))

(fn ConstructionScript)

(fn GetTime
  (params (Hours :type Integer))
  (Variables|Default|SetTimeInHours Hours))

(fn LightIntensity
  (params (Target :type Light%20Component%20Object%20Reference) (Intensity :type Float%20%28single-precision%29))
  (Rendering|Components|Light|SetIntensity Target Intensity))

(fn FetchArrowsfromVehicles
  (params (Seat :type E_VehicleSeat%20Enum :default "NewEnumerator0"))
  (return "0, 0, 0" "0, 0, 0"))

(fn GetVehicleNameandLoc
  (return "NewEnumerator0" "0, 0, 0"))

(fn ObtainTrunkArrowsPickup
  (params (Seat%281-6%29 :type Integer))
  (return "0, 0, 0" "0, 0, 0"))

(fn PlayerDependentLight?
  (return false))