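; Pickup prop for Jack's belongings in Chapter 6, showing a mesh chosen from an array by Selector at BeginPlay.
; When picking is allowed, the overlap sphere toggles the interact prompt for the Jack-tagged actor and tracks range.
; Pickup also requires the army bag flag, then hides the mesh, notifies the GameInstance, plays a cloth sound and destroys the actor after a delay.
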(event OnComponentBeginOverlap(Sphere)
  (params (OverlappedComponent :type Primitive%20Component%20Object%20Reference) (OtherActor :type Actor%20Object%20Reference) (OtherComp :type Primitive%20Component%20Object%20Reference) (OtherBodyIndex :type Integer) (bFromSweep :type Boolean) (SweepResult :type Hit%20Result%20Structure%20%28by%20ref%29))
  (if (Variables|Default|GetAllowedToPick?)
    (if (Actor|ActorHasTag OtherActor "Jack")
      (Class|BPIntJack|ToggleInteractPromptPlayer(Message) OtherActor true)
      (Variables|Default|SetInRange? true))))

(event OnComponentEndOverlap(Sphere)
  (params (OverlappedComponent :type Primitive%20Component%20Object%20Reference) (OtherActor :type Actor%20Object%20Reference) (OtherComp :type Primitive%20Component%20Object%20Reference) (OtherBodyIndex :type Integer))
  (if (Actor|ActorHasTag OtherActor "Jack")
    (Class|BPIntJack|ToggleInteractPromptPlayer(Message) OtherActor false)
    (Variables|Default|SetInRange? false)))

(event EventBeginPlay
  (Components|StaticMesh|SetStaticMesh (Variables|Default|GetStaticMesh) (Utilities|Array|Get(acopy) (Variables|Default|GetMesh) (Variables|Default|GetSelector))))

(event EventBelongingsAllowedtoPick?
  (params (Allowed? :type Boolean))
  (Variables|Default|SetAllowedToPick? Allowed?))

(event EventPickupBelongingsCH6
  (if (and (Variables|Default|GetInRange?) (Variables|Default|GetArmyBagPicked?)) ; Need to be In Range + Army Bag picked
    (Rendering|SetVisibility (Variables|Default|GetStaticMesh) false false)
    (Class|BPIntGameInstance|GIPickupBelongingsCH6(Message) (Game|GetGameInstance))
    (Audio|PlaySound2D "/Game/Sounds/Foley/SCue_Foley_SwipeCloth.SCue_Foley_SwipeCloth" 0.5 1.0 0.0 0 0)
    (Utilities|FlowControl|Delay 1e+01)
    (Actor|DestroyActor)))

(event EventBelongingsPrimed?
  (params (IsArmyBagPicked? :type Boolean))
  (Variables|Default|SetArmyBagPicked? IsArmyBagPicked?))

(fn ConstructionScript)

(fn PlayerDependentLight?
  (return false))