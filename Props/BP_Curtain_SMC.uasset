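; BP_Curtain_SMC is a configurable curtain prop with two optional attachment pieces.
; Its construction script scales the curtain in width and height from variables, with fixed depth, and slides it along its local X axis.
; Each attachment gets its own visibility, X position, pitch and a flip toggle that switches its yaw to face the opposite way, with mirrored defaults between the two.
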(fn ConstructionScript
  (bind _curtain (Variables|Default|GetCurtain))
  (bind _attachment (Variables|Default|GetAttachment))
  (bind _attachment2 (Variables|Default|GetAttachment2))
  (Transformation|SetWorldScale3D _curtain (Math|Vector|MakeVector (Variables|Default|GetCurtain_X_Scale) 1.1 (Variables|Default|GetCurtain_Z_Scale)))
  (Transformation|SetRelativeLocation _curtain (Math|Vector|MakeVector (Variables|Default|GetCurtain_Movement) 0.0 0.0) false false)
  (Transformation|SetRelativeLocation _attachment (Math|Vector|MakeVector (Variables|Default|GetAttachmentLocation) 0.0 0.0) false false)
  (Transformation|SetRelativeRotation _attachment (Math|Rotator|MakeRotator 0.0 (Variables|Default|GetPitchRotationAttachment_1) (select (Variables|Default|GetFlipAttachment_1?) -9e+01 9e+01)) false false)
  (Rendering|SetVisibility (Variables|Default|GetAttachment2) (Variables|Default|GetAttachment_2_Visible?) false)
  (Transformation|SetRelativeRotation _attachment2 (Math|Rotator|MakeRotator 0.0 (Variables|Default|GetPitchRotationAttachment_2) (select (Variables|Default|GetFlipAttachment_2?) 9e+01 -9e+01)) false false)
  (Transformation|SetRelativeLocation _attachment2 (Math|Vector|MakeVector (Variables|Default|GetAttachment_2_Location) 0.0 0.0) false false)
  (Rendering|SetVisibility (Variables|Default|GetAttachment) (Variables|Default|GetAttachment_1_Visible?) false))