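; BP_Stretcher is a stretcher prop with logic for spline travel and a swappable belt mesh, though neither is wired up.
; Its events and construction script are empty.
; The disconnected graphs would use a timeline, timed by TimeToTravel, to move the actor along SplineRef's spline with a yaw offset, and switch the belt between curved and flat meshes via Flip.
; PlayerDependentLight always returns false.
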(event Custom|Event_SplineMovt_Stretcher)

(event EventBeginPlay)

(event EventChangeBeltStretcher
  (params (Flip? :type Boolean)))

(fn ConstructionScript)

(fn PlayerDependentLight?
  (return false))