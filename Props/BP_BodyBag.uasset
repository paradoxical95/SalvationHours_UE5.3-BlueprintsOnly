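; Body bag prop Blueprint with logic meant to move the actor along a referenced spline.
; A timeline, rate-scaled by the inverse of TimeToTravel, maps its alpha to spline distance and sets world location and yaw plus an offset.
; That movement chain is disconnected and never runs: Event_SplineMovt_BodyBag, BeginPlay and the construction script are all empty.
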(event Custom|Event_SplineMovt_BodyBag)

(event EventBeginPlay)

(fn ConstructionScript)