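; BP_WallLamp is a wall lamp prop with a configurable point light.
; Its construction script copies Blueprint variables for intensity, attenuation radius, falloff exponent and visibility onto the PointLight component.
; The event graph holds only disabled placeholder events, so the lamp runs no gameplay logic of its own.
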(event EventBeginPlay)

(event Collision|EventActorBeginOverlap
  (params (OtherActor :type Actor%20Object%20Reference)))

(event EventTick
  (params (DeltaSeconds :type Float%20%28single-precision%29)))

(fn ConstructionScript
  (Rendering|Components|Light|SetIntensity (Variables|Default|GetPointLight) (Variables|Default|GetIntensity))
  (Rendering|Lighting|SetAttenuationRadius (Variables|Default|GetPointLight) (Variables|Default|GetAttn%20Radius))
  (Class|PointLightComponent|SetLightFalloffExponent (Variables|Default|GetPointLight) (Variables|Default|GetLightFalloffExponent))
  (Rendering|SetVisibility (Variables|Default|GetPointLight) (Variables|Default|GetLight%20Visible?) false))