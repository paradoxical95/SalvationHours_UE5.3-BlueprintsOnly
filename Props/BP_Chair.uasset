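; BP_Chair is a chair prop that seats and releases an actor through its AttachtoChair event.
; Sitting snaps the actor to the mesh's Attach socket, or Typing socket when CaseOfficerTyping is set; detaching moves it to ExitLocation.
; Both paths send SitOnChairNPCMessage to update the actor's sitting state, with the typing flag passed when seating.
; The vehicle arrow and light query functions are stubs returning default values.
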(event EventAttachtoChair
  (params (Detach? :type Boolean) (ActorRef :type Actor%20Object%20Reference))
  (bind _chairmesh (Variables|Default|GetChairMesh))
  (bind _caseofficertyping_ (Variables|Default|GetCaseOfficerTyping?))
  (bind _exit_location (Variables|Default|GetExit%20Location))
  (bind _returnvalue (Transformation|GetWorldTransform _exit_location))
  (bind _returnvalue_2 (select _caseofficertyping_ "Typing" "Attach"))
  (bind _returnvalue_3 (Transformation|GetSocketTransform _chairmesh _returnvalue_2 "RTS_World"))
  (if Detach?
    (Utilities|IsValid ActorRef
      (:Is%20Valid
        (Transformation|DetachFromActor ActorRef "KeepRelative" "KeepRelative" "KeepRelative")
        (Transformation|SetActorTransform ActorRef (Math|Transform|MakeTransform (.location _returnvalue) (.rotation _returnvalue) "1.000000,1.000000,1.000000")) ; Leave the chair and stand right next to it
        (Class|BPIntNPC|SitonChairNPC(Message) ActorRef false false false)))
    (else
      (Transformation|AttachComponentToComponent ActorRef _chairmesh _returnvalue_2 "SnapToTarget" "SnapToTarget" "SnapToTarget" true)
      (Transformation|SetActorTransform ActorRef (Math|Transform|MakeTransform (.location _returnvalue_3) (.rotation _returnvalue_3) "1.000000,1.000000,1.000000")) ; Setting the Actor's Loc and Rot, the same as chair
      (Class|BPIntNPC|SitonChairNPC(Message) ActorRef true false (Variables|Default|GetCaseOfficerTyping?)))))

(fn ConstructionScript)

(fn FetchArrowsfromVehicles
  (params (Seat :type E_VehicleSeat%20Enum :default "NewEnumerator0"))
  (return "0, 0, 0" "0, 0, 0"))

(fn GetVehicleNameandLoc
  (return "NewEnumerator0" "0, 0, 0"))

(fn ObtainTrunkArrowsPickup
  (params (Seat%281-6%29 :type Integer))
  (return "0, 0, 0" "0, 0, 0"))

(fn PlayerDependentLight?
  (return false))