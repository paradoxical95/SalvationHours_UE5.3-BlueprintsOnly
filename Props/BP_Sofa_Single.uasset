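; BP_Sofa_Single is a single sofa prop that NPCs can be seated on and removed from.
; Its AttachtoChair event snaps the given actor to the SofaMesh "Attach" socket, matches that socket's transform, and sends SitOnChairNPCMessage to start sofa sitting.
; When detaching, it releases the valid actor, places it beside the sofa at a fixed world-space Y offset, and sends the same message to end sitting.
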(event EventAttachtoChair
  (params (Detach? :type Boolean) (ActorRef :type Actor%20Object%20Reference))
  (bind _sofamesh (Variables|Default|GetSofaMesh))
  (bind _sofamesh_2 (Variables|Default|GetSofaMesh))
  (bind _returnvalue (Transformation|GetSocketTransform _sofamesh_2 "Attach" "RTS_World"))
  (bind _returnvalue_2 (Transformation|GetWorldTransform _sofamesh))
  (if Detach?
    (Utilities|IsValid ActorRef
      (:Is%20Valid
        (Transformation|DetachFromActor ActorRef "KeepRelative" "KeepRelative" "KeepRelative")
        (Transformation|SetActorTransform ActorRef (Math|Transform|MakeTransform (+ (.location _returnvalue_2) "0,80.000000,0") (.rotation _returnvalue_2) "1.000000,1.000000,1.000000")) ; Leave the chair and stand right next to it
        (Class|BPIntNPC|SitonChairNPC(Message) ActorRef false false)))
    (else
      (Transformation|AttachComponentToComponent ActorRef _sofamesh_2 "Attach" "SnapToTarget" "SnapToTarget" "SnapToTarget" true)
      (Transformation|SetActorTransform ActorRef (Math|Transform|MakeTransform (.location _returnvalue) (.rotation _returnvalue) "1.000000,1.000000,1.000000")) ; Setting the Actor's Loc and Rot, the same as chair
      (Class|BPIntNPC|SitonChairNPC(Message) ActorRef true true))))

(fn ConstructionScript)