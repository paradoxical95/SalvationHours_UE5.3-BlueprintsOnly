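; Floor floodlight prop that switches an attached light and emissive plane on and off, and can be shot out permanently.
; Toggle and day/night events set light visibility and a dynamic material's emissive value, with a random per-instance delay staggering switch-on.
; Toggling also plays switch and hum audio, while destruction plays a break sound and blocks later switch-on.
; Remaining functions are mostly stubs returning defaults.
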(event Custom|Event_NightTime
  (bind _attachedlight (Variables|Default|GetAttachedLight))
  (if (not (Variables|Default|GetLightDisabled?))
    (Utilities|FlowControl|Delay (Variables|Default|GetRandomDelay))
    (bind _returnvalue (Rendering|Material|CreateDynamicMaterialInstance (Variables|Default|GetPlane) 0 "/Game/_Main/Assets/Props/OtherProps/Custom/Mat/FloodLights_Inst.FloodLights_Inst" "None" :!class /Script/Engine.PrimitiveComponent))
    (Rendering|Material|SetScalarParameterValue _returnvalue "Emissive" 8.5 :!class /Script/Engine.MaterialInstanceDynamic)
    ;[1 1 1] Light
    (Utilities|IsValid _attachedlight
      (:Is%20Valid
        (Rendering|SetVisibility (Variables|/Script/Engine.Actor|GetRootComponent _attachedlight) true false)))))

(event Custom|Event_DayTime
  (bind _attachedlight (Variables|Default|GetAttachedLight))
  (bind _returnvalue (Rendering|Material|CreateDynamicMaterialInstance (Variables|Default|GetPlane) 0 "/Game/_Main/Assets/Props/OtherProps/Custom/Mat/FloodLights_Inst.FloodLights_Inst" "None" :!class /Script/Engine.PrimitiveComponent))
  (Rendering|Material|SetScalarParameterValue _returnvalue "Emissive" 0.1 :!class /Script/Engine.MaterialInstanceDynamic)
  ;[1 1 1] Light
  (Utilities|IsValid _attachedlight
    (:Is%20Valid
      (Rendering|SetVisibility (Variables|/Script/Engine.Actor|GetRootComponent _attachedlight) false false))))

(event EventBeginPlay
  (Variables|Default|SetRandomDelay (Math|Random|RandomFloatinRange 0.5 4.0)))

(event EventToggleLighting
  (params (Enable? :type Boolean))
  (bind _plane (Variables|Default|GetPlane))
  (bind _attachedlight (Variables|Default|GetAttachedLight))
  (bind _audio (Variables|Default|GetAudio))
  (bind _audio_2 (Variables|Default|GetAudio))
  (bind _audio_3 (Variables|Default|GetAudio))
  (bind _attachedlight_2 (Variables|Default|GetAttachedLight))
  ;[1 1 1] New Code
  (if Enable?
    (if (not (Variables|Default|GetLightDisabled?))
      (Utilities|FlowControl|Delay (Variables|Default|GetRandomDelay))
      (bind _returnvalue (Rendering|Material|CreateDynamicMaterialInstance _plane 0 "/Game/_Main/Assets/Props/OtherProps/Custom/Mat/FloodLights_Inst.FloodLights_Inst" "None" :!class /Script/Engine.PrimitiveComponent))
      (Rendering|Material|SetScalarParameterValue _returnvalue "Emissive" 8.5 :!class /Script/Engine.MaterialInstanceDynamic)
      (Utilities|IsValid _attachedlight_2
        (:Is%20Valid
          (Rendering|SetVisibility (Variables|/Script/Engine.Actor|GetRootComponent _attachedlight_2) true false)
          (Components|Tick|SetComponentTickEnabled _audio_3 true)
          (Audio|Components|Audio|SetSound _audio_3 "/Game/_Main/Sounds/Props/Floodlights_On_2.Floodlights_On_2")
          (Components|Activation|Activate _audio_3 false)
          (Audio|Components|Audio|FadeIn _audio_3 0.0 1.0 0.0 "Linear" :!class /Script/Engine.AudioComponent)
          (Utilities|FlowControl|Delay 0.85)
          (Audio|Components|Audio|SetSound _audio "/Game/_Main/Sounds/Props/Floodlights_Humm.Floodlights_Humm")
          (Audio|Components|Audio|FadeIn _audio 1.0 1.0 0.0 "Linear" :!class /Script/Engine.AudioComponent))))
    (else
      (bind _returnvalue_2 (Rendering|Material|CreateDynamicMaterialInstance _plane 0 "/Game/_Main/Assets/Props/OtherProps/Custom/Mat/FloodLights_Inst.FloodLights_Inst" "None" :!class /Script/Engine.PrimitiveComponent))
      (Rendering|Material|SetScalarParameterValue _returnvalue_2 "Emissive" 0.0 :!class /Script/Engine.MaterialInstanceDynamic)
      (Utilities|IsValid _attachedlight
        (:Is%20Valid
          (Rendering|SetVisibility (Variables|/Script/Engine.Actor|GetRootComponent _attachedlight) false false)
          (Audio|Components|Audio|SetSound _audio_2 "/Game/_Main/Sounds/Props/Floodlights_On_2.Floodlights_On_2")
          (Audio|Components|Audio|Play _audio_2 0.0)
          (Utilities|FlowControl|Delay 0.85)
          (Components|Activation|Deactivate _audio_2)
          (Components|Tick|SetComponentTickEnabled (Variables|Default|GetAudio) false))))))

(event EventDestroyLighting
  (bind _attachedlight (Variables|Default|GetAttachedLight))
  (bind _audio (Variables|Default|GetAudio))
  ;[1 1 1] Deactivate light if player shoots it
  (Utilities|IsValid _attachedlight
    (:Is%20Valid
      (Rendering|SetVisibility (Variables|/Script/Engine.SpotLight|GetSpotLightComponent _attachedlight) false false)
      (bind _returnvalue (Rendering|Material|CreateDynamicMaterialInstance (Variables|Default|GetPlane) 0 "/Game/_Main/Assets/Props/OtherProps/Custom/Mat/FloodLights_Inst.FloodLights_Inst" "None" :!class /Script/Engine.PrimitiveComponent))
      (Rendering|Material|SetScalarParameterValue _returnvalue "Emissive" 0.0 :!class /Script/Engine.MaterialInstanceDynamic)
      (Variables|Default|SetLightDisabled? true)
      (Components|Activation|Activate _audio false)
      (Audio|Components|Audio|SetSound _audio "/Game/_Main/Sounds/Props/Floodlights_Break.Floodlights_Break")
      (Audio|Components|Audio|FadeIn _audio 0.0 1.0 0.0 "Linear" :!class /Script/Engine.AudioComponent)
      (Utilities|FlowControl|Delay 0.8)
      (Components|Activation|Deactivate _audio)
      (Components|Tick|SetComponentTickEnabled (Variables|Default|GetAudio) false))))

(fn ConstructionScript)

(fn GetTime
  (params (Hours :type Integer))
  (Variables|Default|SetTimeInHours Hours))

(fn LightIntensity
  (params (Target :type Light%20Component%20Object%20Reference) (Intensity :type Float%20%28single-precision%29))
  (Rendering|Components|Light|SetIntensity Target Intensity))

(fn FetchArrowsfromVehicles
  (params (Seat :type E_VehicleSeat%20Enum :default "NewEnumerator0"))
  (return "0, 0, 0" "0, 0, 0"))

(fn GetVehicleNameandLoc
  (return "NewEnumerator0" "0, 0, 0"))

(fn ObtainTrunkArrowsPickup
  (params (Seat%281-6%29 :type Integer))
  (return "0, 0, 0" "0, 0, 0"))

(fn PlayerDependentLight?
  (return false))