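; BP_Curtain is an interactable curtain prop with two adjustable attachments, laid out by the Construction Script.
; InteractwithActor forwards to InteractWithCurtain, where a FlipFlop alternately plays and reverses the OpenClose timeline.
; Timeline updates lerp Y scale and Y position toward fixed targets, narrowing and sliding the curtain.
; Each lerp overwrites its own start value, so reversing does not restore the original shape.
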(event Custom|InteractWithCurtain
  (bind _curtain (Variables|Default|GetCurtain))
  (Utilities|FlowControl|FlipFlop
    (:A
      (bind _floatvalue (Timeline|OpenClose PlayFromStart)
        (:Update
          (Variables|Default|SetCurtain_Y_Scale (Math|Float|Lerp (Variables|Default|GetCurtain_Y_Scale) 0.25 _floatvalue))
          (Variables|Default|SetCurtain_Movement (Math|Float|Lerp (Variables|Default|GetCurtain_Movement) 85.0 _floatvalue))
          (Transformation|SetWorldScale3D _curtain (Math|Vector|MakeVector 1.0 (Variables|Default|GetCurtain_Y_Scale) (Variables|Default|GetCurtain_Z_Scale)))
          (Transformation|SetRelativeLocation _curtain (Math|Vector|MakeVector 0.0 (Variables|Default|GetCurtain_Movement) 0.0) false false))))
    (:B
      (Timeline|OpenClose ReverseFromEnd))))

(event EventInteractwithActor
  (CallFunction|InteractwithCurtain))

(fn ConstructionScript
  (bind _curtain (Variables|Default|GetCurtain))
  (bind _attachment (Variables|Default|GetAttachment))
  (bind _attachment2 (Variables|Default|GetAttachment2))
  (Transformation|SetWorldScale3D _curtain (Math|Vector|MakeVector 1.0 (Variables|Default|GetCurtain_Y_Scale) (Variables|Default|GetCurtain_Z_Scale)))
  (Transformation|SetRelativeLocation _curtain (Math|Vector|MakeVector 0.0 (Variables|Default|GetCurtain_Movement) 0.0) false false)
  (Transformation|SetRelativeLocation _attachment (Math|Vector|MakeVector 0.0 (Variables|Default|GetAttachmentLocation) 0.0) false false)
  (Transformation|SetRelativeRotation _attachment (Math|Rotator|MakeRotator 0.0 (Variables|Default|GetPitchRotationAttachment) (select (Variables|Default|GetFlipAttachment?) 1.8e+02 0.0)) false false)
  (Rendering|SetVisibility (Variables|Default|GetAttachment2) (Variables|Default|GetAttachment_2_Visible?) false)
  (Transformation|SetRelativeRotation _attachment2 (Math|Rotator|MakeRotator 0.0 (Variables|Default|GetPitchRotationAttachment_2) (select (Variables|Default|GetFlipAttachment_2?) 1.8e+02 0.0)) false false)
  (Transformation|SetRelativeLocation _attachment2 (Math|Vector|MakeVector 0.0 (Variables|Default|GetAttachment_2_Location) 0.0) false false))