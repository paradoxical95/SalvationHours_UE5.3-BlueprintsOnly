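; Pin board prop that shows a chosen material on each of its four pinned paper components.
; On BeginPlay, each paper's second material slot is set from a shared Materials array, using that paper's own Selector index.
; The Construction Script holds an unconnected copy of the same logic, so it applies none of these materials.
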(event EventBeginPlay
  (Rendering|Material|SetMaterial (Variables|Default|GetPinupPaper1) 1 (Utilities|Array|Get(acopy) (Variables|Default|GetMaterials) (Variables|Default|GetSelector)))
  (Rendering|Material|SetMaterial (Variables|Default|GetPinupPaper2) 1 (Utilities|Array|Get(acopy) (Variables|Default|GetMaterials) (Variables|Default|GetSelector2)))
  (Rendering|Material|SetMaterial (Variables|Default|GetPinupPaper3) 1 (Utilities|Array|Get(acopy) (Variables|Default|GetMaterials) (Variables|Default|GetSelector3)))
  (Rendering|Material|SetMaterial (Variables|Default|GetPinupPaper) 1 (Utilities|Array|Get(acopy) (Variables|Default|GetMaterials) (Variables|Default|GetSelector4))))

(fn ConstructionScript)