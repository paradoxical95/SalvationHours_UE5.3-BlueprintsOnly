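; BP_Props_Lamp is a configurable lamp prop that can appear as either a desk lamp or a table lamp.
; Its construction script applies visibility and intensity variables to two spot lights and uses a selector to show one lamp component and hide the other.
; The event graph holds only disabled stub events, so the graphs add no runtime behaviour.
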(event EventBeginPlay)

(event Collision|EventActorBeginOverlap
  (params (OtherActor :type Actor%20Object%20Reference)))

(event EventTick
  (params (DeltaSeconds :type Float%20%28single-precision%29)))

(fn ConstructionScript
  (bind _spotlight (Variables|Default|GetSpotLight))
  (Rendering|SetVisibility _spotlight (Variables|Default|GetLightVisible) true)
  (Rendering|Components|Light|SetIntensity _spotlight (Variables|Default|GetLightIntensity))
  (Rendering|SetVisibility (Variables|Default|GetDeskLamp) (Utilities|Select :Index (Variables|Default|GetSelector) :Option%200 true :Option%201 false) true)
  (Rendering|SetVisibility (Variables|Default|GetTableLamp) (Utilities|Select :Index (Variables|Default|GetSelector) :Option%200 false :Option%201 true) true))