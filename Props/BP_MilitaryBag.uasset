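; Military bag pickup prop, named for CH6, that the player tagged Jack can collect once an external event allows picking.
; Sphere overlap toggles Jack's interact prompt and the in-range flag.
; The pickup event, when in range, hides the bag, notifies the GameInstance, plays a cloth sound and destroys the actor after a delay.
; The vehicle and light functions are stubs returning defaults.
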(event OnComponentBeginOverlap(Sphere)
  (params (OverlappedComponent :type Primitive%20Component%20Object%20Reference) (OtherActor :type Actor%20Object%20Reference) (OtherComp :type Primitive%20Component%20Object%20Reference) (OtherBodyIndex :type Integer) (bFromSweep :type Boolean) (SweepResult :type Hit%20Result%20Structure%20%28by%20ref%29))
  (if (Variables|Default|GetAllowedToPick?)
    (if (Actor|ActorHasTag OtherActor "Jack")
      (Class|BPIntJack|ToggleInteractPromptPlayer(Message) OtherActor true)
      (Variables|Default|SetInRange? true))))

(event OnComponentEndOverlap(Sphere)
  (params (OverlappedComponent :type Primitive%20Component%20Object%20Reference) (OtherActor :type Actor%20Object%20Reference) (OtherComp :type Primitive%20Component%20Object%20Reference) (OtherBodyIndex :type Integer))
  (if (Actor|ActorHasTag OtherActor "Jack")
    (Class|BPIntJack|ToggleInteractPromptPlayer(Message) OtherActor false)
    (Variables|Default|SetInRange? false)))

(event EventBelongingsAllowedtoPick?
  (params (Allowed? :type Boolean))
  (Variables|Default|SetAllowedToPick? Allowed?))

(event EventPickupMilitaryBagCH6
  (if (Variables|Default|GetInRange?)
    (Rendering|SetVisibility (Variables|Default|GetBag) false false)
    (Class|BPIntGameInstance|GIPickupMilitaryBagCH6(Message) (Game|GetGameInstance))
    (Audio|PlaySound2D "/Game/Sounds/Foley/SCue_Foley_SwipeCloth.SCue_Foley_SwipeCloth" 0.5 1.0 0.0 0 0)
    (Utilities|FlowControl|Delay 1e+01)
    (Actor|DestroyActor)))

(fn ConstructionScript)

(fn FetchArrowsfromVehicles
  (params (Seat :type E_VehicleSeat%20Enum :default "NewEnumerator0"))
  (return "0, 0, 0" "0, 0, 0"))

(fn GetVehicleNameandLoc
  (return "NewEnumerator0" "0, 0, 0" "0, 0, 0"))

(fn IsVehicleMoving?
  (return false))

(fn ObtainTrunkArrowsPickup
  (params (Seat%281-6%29 :type Integer))
  (return "0, 0, 0" "0, 0, 0"))

(fn PlayerDependentLight?
  (return false))