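; Hatchback vehicle Blueprint that registers with the GameInstance, sets its body paint colour and travels along splines on request.
; A timeline scaled to TimeToTravel moves it along the spline, while a timer triggers the braking stop shortly before arrival.
; Front doors open and auto-close, arrow components supply front-seat transforms, and a macro handles door and engine sounds.
; Interaction and segment-check events are empty, and occupant rotation code is unconnected.
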(event Custom|StopDrivingSlowly
  ;[1 1 1] Spline Movement
  ;;[0.3438 0.04946 0.0392] Start Vehicle
  (Variables|Default|SetStartVehicle? false)
  (Utilities|MVehicleSound "NewEnumerator4"))

(event Custom|StartMovementVehicle
  (bind _splineref (Variables|Default|GetSplineRef))
  (bind _spline (Variables|/Game/_Main/Blueprints/Vehicles/BP_Spline_Vehicle.BP_Spline_Vehicle_C|GetSpline _splineref))
  ;[1 1 1] Spline Movement
  (if (not (Variables|Default|GetTravelFinished?))
    (Utilities|MVehicleSound "NewEnumerator2")
    ;;[0.3438 0.04946 0.0392] Start Vehicle
    (Variables|Default|SetStartVehicle? true)
    (bind _returnvalue (Utilities|Time|SetTimerbyEvent (delegate Custom|StopDrivingSlowly) (- (Variables|Default|GetTimeToTravel) 3.0)))
    (Variables|Default|SetTimerHandle _returnvalue)
    (Components|Timeline|SetPlayRate (Variables|Default|GetTimelineMoveVehicle) (/ 1.0 (Variables|Default|GetTimeToTravel))) ; How fast
    (Utilities|MVehicleSound "NewEnumerator3")
    (bind _float (Timeline|TimelineMoveVehicle PlayFromStart)
      (:Update
        (Transformation|SetActorTransform (Math|Transform|MakeTransform (Spline|GetLocationatDistanceAlongSpline _spline (Math|Float|Lerp 0.0 (Spline|GetSplineLength (Variables|/Game/_Main/Blueprints/Vehicles/BP_Spline_Vehicle.BP_Spline_Vehicle_C|GetSpline (Variables|Default|GetSplineRef))) _float) "World") (Math|Rotator|MakeRotator (.roll (Spline|GetRotationatDistanceAlongSpline _spline (Math|Float|Lerp 0.0 (Spline|GetSplineLength (Variables|/Game/_Main/Blueprints/Vehicles/BP_Spline_Vehicle.BP_Spline_Vehicle_C|GetSpline (Variables|Default|GetSplineRef))) _float) "Local")) (.pitch (Spline|GetRotationatDistanceAlongSpline _spline (Math|Float|Lerp 0.0 (Spline|GetSplineLength (Variables|/Game/_Main/Blueprints/Vehicles/BP_Spline_Vehicle.BP_Spline_Vehicle_C|GetSpline (Variables|Default|GetSplineRef))) _float) "Local")) (+ (.yaw (Spline|GetRotationatDistanceAlongSpline _spline (Math|Float|Lerp 0.0 (Spline|GetSplineLength (Variables|/Game/_Main/Blueprints/Vehicles/BP_Spline_Vehicle.BP_Spline_Vehicle_C|GetSpline (Variables|Default|GetSplineRef))) _float) "Local")) (Variables|Default|GetOffset_Z_RotationSpline))) "1.000000,1.000000,1.000000")))
      (:Finished
        (Variables|Default|SetTravelFinished? true)
        (Utilities|Time|ClearandInvalidateTimerbyHandle (Variables|Default|GetTimerHandle))))))

(event Custom|Event_CheckForVehicleMovement
  (params (ChapterSegmentData :type S%20Chapter%20Segment%20Data%20Structure)))

(event EventBeginPlay
  (Class|BPIntGameInstance|GetVehicleRef(Message) (Game|GetGameInstance) self (Variables|Default|GetVehicleName))
  (bind _returnvalue (Rendering|Material|CreateDynamicMaterialInstance (Variables|Default|GetMesh) 1 "/Game/_Main/Assets/Vehicles/Golf_Hatchback/Mat/Golf_BodyPaint_MI.Golf_BodyPaint_MI" "None" :!class /Script/Engine.PrimitiveComponent))
  (Rendering|Material|SetVectorParameterValue _returnvalue "Color" (Utilities|Array|Get(acopy) (Variables|Default|GetColor_Hatchback) (Math|Integer|Clamp(Integer) (select (Variables|Default|GetRandomColor?) (Math|Random|RandomIntegerinRange 0 4) (Variables|Default|GetColorSwitcher)) 0 4)) :!class /Script/Engine.MaterialInstanceDynamic))

(event EventInteractwithVehicle
  (params (CharacterRef :type Character%20Object%20Reference) (InteractingManually? :type Boolean))
  ;[1 1 1] Sit _REWORK NEEDED
)

(event EventFollowSplinePathVehicle
  (params (SplineRef :type BP%20Spline%20Vehicle%20Object%20Reference))
  ;[1 1 1] Spline Movement
  (Variables|Default|SetSplineRef SplineRef)
  (Variables|Default|SetTravelFinished? false)
  (CallFunction|StartMovementVehicle))

(event EventUpdateChapterSegment
  (params (Struct_Ch_Seg_Data :type S%20Chapter%20Segment%20Data%20Structure))
  (bind _output_get (Variables|Default|SetChapterSegmentData Struct_Ch_Seg_Data))
  (CallFunction|EventCheckforVehicleMovement _output_get))

(event EventToggleVehicleDoors
  (params (Seat :type E_VehicleSeat%20Enum :default "NewEnumerator0"))
  ;[1 1 1] Doors
  (switch Utilities|FlowControl|Switch|SwitchonE_VehicleSeat Seat
    (:NewEnumerator0
      (Utilities|MVehicleSound "NewEnumerator0")
      (Variables|Default|SetDoor_FL_Open? true)
      (Utilities|FlowControl|Delay 4.0)
      (Variables|Default|SetDoor_FL_Open? false)
      (Utilities|MVehicleSound "NewEnumerator1"))
    (:NewEnumerator1
      (Utilities|MVehicleSound "NewEnumerator0")
      (Variables|Default|SetDoor_FR_Open? true)
      (Utilities|FlowControl|Delay 4.0)
      (Variables|Default|SetDoor_FR_Open? false)
      (Utilities|MVehicleSound "NewEnumerator1"))))

(fn ConstructionScript)

(fn ObtainArrowsTransform
  (params (Seat :type E_VehicleSeat%20Enum :default "NewEnumerator0"))
  (bind _arrow_driver (Variables|Default|GetArrow_Driver))
  (bind _arrow_passenger (Variables|Default|GetArrow_Passenger))
  (bind _returnvalue (Utilities|Select :Index Seat :NewEnumerator0 _arrow_driver :NewEnumerator1 _arrow_passenger :NewEnumerator2 0 :NewEnumerator3 0 :NewEnumerator4 0 :NewEnumerator5 0 :NewEnumerator6 0))
  (bind _returnvalue_2 (Transformation|GetWorldTransform _returnvalue))
  (return (.location _returnvalue_2) (.rotation _returnvalue_2)))

(fn FetchArrowsfromVehicles
  (params (Seat :type E_VehicleSeat%20Enum :default "NewEnumerator0"))
  (bind (_arrowlocation _arrowrotation) (CallFunction|ObtainArrowsTransform Seat))
  (return _arrowlocation _arrowrotation))

(fn GetVehicleNameandLoc
  (return "NewEnumerator0" "0, 0, 0"))

(fn ObtainTrunkArrowsPickup
  (params (Seat%281-6%29 :type Integer))
  (return "0, 0, 0" "0, 0, 0"))

(fn PlayerDependentLight?
  (return false))