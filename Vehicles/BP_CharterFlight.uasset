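; Charter flight vehicle that flies along a supplied spline with a take-off sound, then hides itself.
; A timeline, rate-scaled by TimeToTravel, moves the actor by distance along the spline.
; Rotation ignores the spline, blending pitch from level to -45 degrees with fixed yaw and roll.
; The other vehicle query functions, for seat arrows, name, location and lighting, are stubs returning default values.
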(event EventFollowSplinePathVehicle
  (params (SplineRef :type BP%20Spline%20Vehicle%20Object%20Reference))
  (bind _audio (Variables|Default|GetAudio))
  (Variables|Default|SetSplineRef SplineRef)
  (Components|Timeline|SetPlayRate (Variables|Default|GetTimelineSplineTravel) (/ 1.0 (Variables|Default|GetTimeToTravel))) ; How fast
  (Audio|Components|Audio|SetSound _audio "/Game/_Main/Sounds/Airport/CharterFlight_TakeOff_Full.CharterFlight_TakeOff_Full")
  (Audio|Components|Audio|FadeIn _audio 2.0 1.0 0.0 "Linear" :!class /Script/Engine.AudioComponent)
  (bind _float (Timeline|TimelineSplineTravel PlayFromStart)
    (:Update
      (Transformation|SetActorTransform (Math|Transform|MakeTransform (.location (Spline|GetTransformatDistanceAlongSpline (Variables|/Game/_Main/Blueprints/Vehicles/BP_Spline_Vehicle.BP_Spline_Vehicle_C|GetSpline (Variables|Default|GetSplineRef)) (Math|Float|Lerp 0.0 (Spline|GetSplineLength (Variables|/Game/_Main/Blueprints/Vehicles/BP_Spline_Vehicle.BP_Spline_Vehicle_C|GetSpline (Variables|Default|GetSplineRef))) _float) "World" false)) (Math|Rotator|MakeRotator 0.0 (Math|Float|Lerp 0.0 -45.0 _float) 0.0) "1.000000,1.000000,1.000000")))
    (:Finished
      (Rendering|SetActorHiddenInGame true))))

(fn ConstructionScript)

(fn FetchArrowsfromVehicles
  (params (Seat :type E_VehicleSeat%20Enum :default "NewEnumerator0"))
  (return "0, 0, 0" "0, 0, 0"))

(fn GetVehicleNameandLoc
  (return "NewEnumerator0" "0, 0, 0"))

(fn ObtainTrunkArrowsPickup
  (params (Seat%281-6%29 :type Integer))
  (return "0, 0, 0" "0, 0, 0"))

(fn PlayerDependentLight?
  (return false))