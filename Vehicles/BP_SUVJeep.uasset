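; Drivable-looking SUV jeep for story chapters that carries the player and NPCs along scripted spline paths.
; A timeline moves it along the given spline over a chapter-set travel time, updating the seated player's camera, while a timer triggers braking shortly before arrival.
; Interaction seats the player via per-seat arrows and timed door toggles.
; It registers with the GameInstance, tints its paint and picks interior or exterior engine audio.
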(event Custom|StopDrivingSlowly
  ;[1 1 1] Spline Movement
  ;;[0.3438 0.04946 0.0392] Start Vehicle
  (Variables|Default|SetStartVehicle? false)
  (Class|BPIntNPC|NPCVehicleMovementStarted(Message) (Variables|Default|GetDriverNPC_Ref) false)
  (Utilities|MVehicleSound "NewEnumerator4"))

(event Custom|StartMovementVehicle
  (bind _splineref (Variables|Default|GetSplineRef))
  (bind _playerref (Variables|Default|GetPlayerRef))
  (bind _spline (Variables|/Game/_Main/Blueprints/Vehicles/BP_Spline_Vehicle.BP_Spline_Vehicle_C|GetSpline _splineref))
  ;[1 1 1] Spline Movement
  (if (not (Variables|Default|GetTravelFinished?))
    (Utilities|MVehicleSound "NewEnumerator2")
    ;;[0.3438 0.04946 0.0392] Start Vehicle
    (Variables|Default|SetStartVehicle? true)
    (Class|BPIntNPC|NPCVehicleMovementStarted(Message) (Variables|Default|GetDriverNPC_Ref) true)
    (bind _returnvalue (Utilities|Time|SetTimerbyEvent (delegate Custom|StopDrivingSlowly) (- (Variables|Default|GetTimeToTravel) 3.0)))
    (Variables|Default|SetTimerHandle _returnvalue)
    (Components|Timeline|SetPlayRate (Variables|Default|GetTimeline_Move_Vehicle) (/ 1.0 (Variables|Default|GetTimeToTravel))) ; How fast
    (Utilities|MVehicleSound "NewEnumerator3")
    (bind _float (Timeline|Timeline_Move_Vehicle PlayFromStart)
      (:Update
        (Transformation|SetActorTransform (Math|Transform|MakeTransform (.location (Spline|GetTransformatDistanceAlongSpline _spline (Math|Float|Lerp 0.0 (Spline|GetSplineLength _spline) _float) "World" false)) (Math|Rotator|MakeRotator (.Roll (Math|Rotator|BreakRotator (Spline|GetRotationatDistanceAlongSpline _spline (Math|Float|Lerp 0.0 (Spline|GetSplineLength _spline) _float) "Local"))) (.Pitch (Math|Rotator|BreakRotator (Spline|GetRotationatDistanceAlongSpline _spline (Math|Float|Lerp 0.0 (Spline|GetSplineLength _spline) _float) "Local"))) (+ (.Yaw (Math|Rotator|BreakRotator (Spline|GetRotationatDistanceAlongSpline _spline (Math|Float|Lerp 0.0 (Spline|GetSplineLength _spline) _float) "Local"))) (Variables|Default|GetOffset_Z_RotationSpline))) "1.000000,1.000000,1.000000"))
        (Utilities|IsValid _playerref
          (:Is%20Valid
            (Class|BPIntJack|UpdateCamerainVehicle(Message) _playerref (+ (.Yaw (Math|Rotator|BreakRotator (Math|Rotator|MakeRotator (.Roll (Math|Rotator|BreakRotator (Spline|GetRotationatDistanceAlongSpline _spline (Math|Float|Lerp 0.0 (Spline|GetSplineLength _spline) _float) "Local"))) (.Pitch (Math|Rotator|BreakRotator (Spline|GetRotationatDistanceAlongSpline _spline (Math|Float|Lerp 0.0 (Spline|GetSplineLength _spline) _float) "Local"))) (+ (.Yaw (Math|Rotator|BreakRotator (Spline|GetRotationatDistanceAlongSpline _spline (Math|Float|Lerp 0.0 (Spline|GetSplineLength _spline) _float) "Local"))) (Variables|Default|GetOffset_Z_RotationSpline))))) (+ (Variables|Default|GetCharacterRotationOffset) -11.0)) (+ (.Yaw (Math|Rotator|BreakRotator (Math|Rotator|MakeRotator (.Roll (Math|Rotator|BreakRotator (Spline|GetRotationatDistanceAlongSpline _spline (Math|Float|Lerp 0.0 (Spline|GetSplineLength _spline) _float) "Local"))) (.Pitch (Math|Rotator|BreakRotator (Spline|GetRotationatDistanceAlongSpline _spline (Math|Float|Lerp 0.0 (Spline|GetSplineLength _spline) _float) "Local"))) (+ (.Yaw (Math|Rotator|BreakRotator (Spline|GetRotationatDistanceAlongSpline _spline (Math|Float|Lerp 0.0 (Spline|GetSplineLength _spline) _float) "Local"))) (Variables|Default|GetOffset_Z_RotationSpline))))) (Variables|Default|GetCharacterRotationOffset)) "0, 0, 0"))))
      (:Finished
        ;;[0.59 0.814 1] When Travel Finished
        (Variables|Default|SetTravelFinished? true)
        (Utilities|Time|ClearandInvalidateTimerbyHandle (Variables|Default|GetTimerHandle))
        (Variables|Default|SetPlayerInside?%20 false)))))

(event Custom|Event_CheckForVehicleMovement
  (params (ChapterSegmentData :type S%20Chapter%20Segment%20Data%20Structure))
  (bind (_ch1_segment _ch2_segment _ch3_segment _ch4_segment _ch5_segment _ch6_segment _chapternumber_) (Utilities|Struct|BreakS_ChapterSegmentData ChapterSegmentData))
  (switch Utilities|FlowControl|Switch|SwitchonE_ChapterNumber _chapternumber_
    (:NewEnumerator2
      (switch Utilities|FlowControl|Switch|SwitchonE_Chapter3_Segments _ch3_segment
        (:NewEnumerator2
          (Variables|Default|SetTimeToTravel 4e+01))))))

(event Custom|Event_OpenJeepTrunk
  (params (Toggle? :type Boolean))
  ;[1 1 1] Trunk
  (Variables|Default|SetJeepTrunkOpen? Toggle?))

(event EventBeginPlay
  (Class|BPIntGameInstance|GetVehicleRef(Message) (Game|GetGameInstance) self (Variables|Default|GetVehicleName))
  (bind _returnvalue (Rendering|Material|CreateDynamicMaterialInstance (Variables|Default|GetMesh) 21 "/Game/_Main/Assets/Vehicles/Jeep_SUV/Mat/BodyPaint_Jeep_MI.BodyPaint_Jeep_MI" "None" :!class /Script/Engine.PrimitiveComponent))
  (Rendering|Material|SetVectorParameterValue _returnvalue "Color" (Variables|Default|GetJeepColor) :!class /Script/Engine.MaterialInstanceDynamic))

(event EventInteractwithVehicle
  (params (CharacterRef :type Character%20Object%20Reference) (InteractingManually? :type Boolean))
  (bind (_arrowlocation _arrowrotation) (CallFunction|ObtainArrowsTransform "NewEnumerator1"))
  ;[1 1 1] Sit
  (Variables|Default|SetPlayerRef CharacterRef)
  (if InteractingManually? ; TRUE if interacting manually\nSo it attaches as well\nEg: Ch1Seg1\nFALSE when attached without interacting
    (Class|BPIntJack|JackEnterVehicle(Message) (Variables|Default|GetPlayerRef) (Variables|Default|GetVehicleName) self _arrowlocation _arrowrotation)
    (CallFunction|ToggleVehicleDoors "NewEnumerator1")
    (Variables|Default|SetPlayerInside?%20 true)))

(event EventToggleVehicleDoors
  (params (Seat :type E_VehicleSeat%20Enum :default "NewEnumerator0"))
  ;[1 1 1] Doors
  (switch Utilities|FlowControl|Switch|SwitchonE_VehicleSeat Seat
    (:NewEnumerator0
      (Utilities|MVehicleSound "NewEnumerator0")
      (Variables|Default|SetDoor_FL_Open? true)
      (Utilities|FlowControl|Delay 4.0)
      (Variables|Default|SetDoor_FL_Open? false)
      (Utilities|MVehicleSound "NewEnumerator1"))
    (:NewEnumerator1
      (Utilities|MVehicleSound "NewEnumerator0")
      (Variables|Default|SetDoor_FR_Open? true)
      (Utilities|FlowControl|Delay 4.0)
      (Variables|Default|SetDoor_FR_Open? false)
      (Utilities|MVehicleSound "NewEnumerator1"))
    (:NewEnumerator2
      (Utilities|MVehicleSound "NewEnumerator0")
      (Variables|Default|SetDoor_RL_Open? true :!label _label)
      (Utilities|FlowControl|Delay 4.0)
      (Variables|Default|SetDoor_RL_Open? false)
      (Utilities|MVehicleSound "NewEnumerator1"))
    (:NewEnumerator3
      (Utilities|FlowControl|Delay (Math|Random|RandomFloatinRange 0.05 0.1))
      (Utilities|MVehicleSound "NewEnumerator0")
      (Variables|Default|SetDoor_RR_Open? true)
      (Utilities|FlowControl|Delay 4.0)
      (Variables|Default|SetDoor_RR_Open? false)
      (Utilities|MVehicleSound "NewEnumerator1"))
    (:NewEnumerator4
      (Utilities|FlowControl|Delay (Math|Random|RandomFloatinRange 0.05 0.1))
      (Utilities|MVehicleSound "NewEnumerator0")
      (goto _label))))

(event EventFollowSplinePathVehicle
  (params (SplineRef :type BP%20Spline%20Vehicle%20Object%20Reference))
  ;[1 1 1] Spline Movement
  (Variables|Default|SetSplineRef SplineRef)
  (Variables|Default|SetTravelFinished? false)
  (CallFunction|StartMovementVehicle))

(event EventUpdateChapterSegment
  (params (Struct_Ch_Seg_Data :type S%20Chapter%20Segment%20Data%20Structure))
  (bind _output_get (Variables|Default|SetChapterSegmentData Struct_Ch_Seg_Data))
  (CallFunction|EventCheckforVehicleMovement _output_get))

(event EventGetDriverRefforCars
  (params (Driver_NPC :type Actor%20Object%20Reference) (IsTheDriver? :type Boolean))
  ;[1 1 1] Driver Ref
  (if IsTheDriver?
    (Variables|Default|SetDriverNPC_Ref Driver_NPC)))

(event EventFetchJackRefforVehicles
  (params (JackRef :type Character%20Object%20Reference))
  ;[1 1 1] Sit
  (Variables|Default|SetPlayerRef JackRef)
  (Variables|Default|SetPlayerInside?%20 true))

(fn ConstructionScript)

(fn ObtainArrowsTransform
  (params (Seat :type E_VehicleSeat%20Enum :default "NewEnumerator0"))
  (bind _passenger_r_l_arrow (Variables|Default|GetPassenger_R_L_Arrow))
  (bind _passenger_r_r_arrow (Variables|Default|GetPassenger_R_R_Arrow))
  (bind _driver_arrow (Variables|Default|GetDriver_Arrow))
  (bind _passenger_front_arrow (Variables|Default|GetPassenger_Front_Arrow))
  (bind _passenger_r_m_arrow (Variables|Default|GetPassenger_R_M_Arrow))
  (bind _returnvalue (Utilities|Select :Index Seat :NewEnumerator0 _driver_arrow :NewEnumerator1 _passenger_front_arrow :NewEnumerator2 _passenger_r_l_arrow :NewEnumerator3 _passenger_r_r_arrow :NewEnumerator4 _passenger_r_m_arrow :NewEnumerator5 0 :NewEnumerator6 0))
  (bind _returnvalue_2 (Transformation|GetWorldTransform _returnvalue))
  (return (.location _returnvalue_2) (.rotation _returnvalue_2)))

(fn FetchArrowsfromVehicles
  (params (Seat :type E_VehicleSeat%20Enum :default "NewEnumerator0"))
  (bind (_arrowlocation _arrowrotation) (CallFunction|ObtainArrowsTransform Seat))
  (return _arrowlocation _arrowrotation))

(fn GetVehicleNameandLoc
  (return (Variables|Default|GetVehicleName) (Transformation|GetActorLocation) (Transformation|GetActorRotation)))

(fn IsVehicleMoving?
  (return false))

(fn ObtainTrunkArrowsPickup
  (params (Seat%281-6%29 :type Integer))
  (return "0, 0, 0" "0, 0, 0"))

(fn PlayerDependentLight?
  (return false))