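; Prop car actor that dresses itself at BeginPlay as one of four vehicles: sedan, hatchback, Golf or pickup.
; RandomMesh chooses between a random pick and MeshSelector, then the chosen static mesh is async-loaded and applied, with a height offset for the Golf.
; A dynamic material on that model's paint slot gets a color from a seven-entry palette, indexed by the sum of two random rolls.
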(event EventBeginPlay
  (bind _mesh (Variables|Default|GetMesh))
  (bind _mesh_2 (Variables|Default|GetMesh))
  (bind _relativelocation (Variables|/Script/Engine.SceneComponent|GetRelativeLocation _mesh))
  (Variables|Default|SetRandomInteger (Math|Integer|Clamp(Integer) (Math|Random|RandomIntegerinRange 0 3) 0 3))
  (if (Variables|Default|GetRandomMesh?)
    (bind _object (Utilities|AsyncLoadAsset (Utilities|Select :Index (Variables|Default|GetRandomInteger) :Option%200 "/Game/_Main/Assets/WorldBased/Sedan_Old.Sedan_Old" :Option%201 "/Game/_Main/Assets/WorldBased/Hatchback_Compact.Hatchback_Compact" :Option%202 "/Game/_Main/Assets/Vehicles/Golf_Hatchback/Golf_Hatch_SM.Golf_Hatch_SM" :Option%203 "/Game/_Main/Assets/Vehicles/PickupTruck/PickupTruck_SM.PickupTruck_SM"))
      (:Completed
        (bind _asstatic_mesh (Utilities|Casting|CastToStaticMesh _object))
        (Utilities|IsValid _asstatic_mesh
          (:Is%20Valid
            (Components|StaticMesh|SetStaticMesh (Variables|Default|GetMesh) _asstatic_mesh)
            (Transformation|SetRelativeLocation _mesh_2 (select (== (select (Variables|Default|GetRandomMesh?) (Variables|Default|GetRandomInteger) (Variables|Default|GetMeshSelector)) 2) (+ _relativelocation "0.000000,0.000000,83.000000") _relativelocation) false false :!label _label)
            (bind _returnvalue (Rendering|Material|CreateDynamicMaterialInstance _mesh_2 (Utilities|Select :Index (select (Variables|Default|GetRandomMesh?) (Variables|Default|GetRandomInteger) (Variables|Default|GetMeshSelector)) :Option%200 0 :Option%201 0 :Option%202 1 :Option%203 2) (Utilities|Select :Index (select (Variables|Default|GetRandomMesh?) (Variables|Default|GetRandomInteger) (Variables|Default|GetMeshSelector)) :Option%200 "/Game/_Main/Assets/WorldBased/Mat/Sedan_Old_Mat.Sedan_Old_Mat" :Option%201 "/Game/_Main/Assets/WorldBased/Mat/Hatchback_Compact_BodyColor_Mat.Hatchback_Compact_BodyColor_Mat" :Option%202 "/Game/_Main/Assets/Vehicles/Golf_Hatchback/Mat/Golf_BodyPaint.Golf_BodyPaint" :Option%203 "/Game/_Main/Assets/Vehicles/PickupTruck/Mat/Pickup_Paint.Pickup_Paint") "None" :!class /Script/Engine.PrimitiveComponent))
            (Rendering|Material|SetVectorParameterValue _returnvalue "Color" (Utilities|Select :Index (+ (Variables|Default|GetRandomInteger) (Math|Random|RandomIntegerinRange 0 3)) :Option%200 "(R=0.019608,G=0.019608,B=0.019608,A=1.000000)" :Option%201 "(R=0.274510,G=0.015686,B=0.015686,A=1.000000)" :Option%202 "(R=0.400000,G=0.392157,B=0.384314,A=1.000000)" :Option%203 "(R=0.105882,G=0.172549,B=0.066667,A=1.000000)" :Option%204 "(R=0.007843,G=0.062745,B=0.168627,A=1.000000)" :Option%205 "(R=0.614583,G=0.321260,B=0.000000,A=1.000000)" :Option%206 "(R=0.023529,G=0.121569,B=0.109804,A=1.000000)") :!class /Script/Engine.MaterialInstanceDynamic))
          (:Is%20Not%20Valid
            (bind _returnvalue_2 (Rendering|Material|CreateDynamicMaterialInstance (Variables|Default|GetMesh) 0 "/Game/_Main/Assets/WorldBased/Mat/Sedan_Old_Mat.Sedan_Old_Mat" "None" :!class /Script/Engine.PrimitiveComponent :!label _label_2))
            (Rendering|Material|SetVectorParameterValue _returnvalue_2 "Color" (Utilities|Select :Index (+ (Variables|Default|GetRandomInteger) (Math|Random|RandomIntegerinRange 0 3)) :Option%200 "(R=0.019608,G=0.019608,B=0.019608,A=1.000000)" :Option%201 "(R=0.274510,G=0.015686,B=0.015686,A=1.000000)" :Option%202 "(R=0.400000,G=0.392157,B=0.384314,A=1.000000)" :Option%203 "(R=0.105882,G=0.172549,B=0.066667,A=1.000000)" :Option%204 "(R=0.007843,G=0.062745,B=0.168627,A=1.000000)" :Option%205 "(R=0.192157,G=0.109804,B=0.019608,A=1.000000)" :Option%206 "(R=0.023529,G=0.121569,B=0.109804,A=1.000000)") :!class /Script/Engine.MaterialInstanceDynamic)))))
    (else
      (bind _object_2 (Utilities|AsyncLoadAsset (Utilities|Select :Index (Variables|Default|GetMeshSelector) :Option%200 "/Game/_Main/Assets/WorldBased/Sedan_Old.Sedan_Old" :Option%201 "/Game/_Main/Assets/WorldBased/Hatchback_Compact.Hatchback_Compact" :Option%202 "/Game/_Main/Assets/Vehicles/Golf_Hatchback/Golf_Hatch_SM.Golf_Hatch_SM" :Option%203 "/Game/_Main/Assets/Vehicles/PickupTruck/PickupTruck_SM.PickupTruck_SM"))
        (:Completed
          (bind _asstatic_mesh_2 (Utilities|Casting|CastToStaticMesh _object_2))
          (Utilities|IsValid _asstatic_mesh_2
            (:Is%20Valid
              (Components|StaticMesh|SetStaticMesh _mesh_2 _asstatic_mesh_2)
              (goto _label))
            (:Is%20Not%20Valid
              (goto _label_2))))))))

(fn ConstructionScript)