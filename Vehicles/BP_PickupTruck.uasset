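; Scripted pickup truck for chapter-based story segments, with a color-switchable paint material and an optional "Technical" variant, plus toggleable cargo props.
; A timeline moves it along a supplied spline over TimeToTravel, which chapter data can override, with engine audio and a brake timer before arrival.
; Events set timed door and trunk flags, and functions return seat arrow transforms.
; Player seating and camera-follow logic is disconnected, leaving InteractwithVehicle empty.
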(event Custom|StopDrivingSlowly
  ;[1 1 1] Spline Movement
  ;;[0.3438 0.04946 0.0392] Start Vehicle
  (Variables|Default|SetStartVehicle? false)
  (Utilities|MVehicleSound "NewEnumerator4"))

(event Custom|StartMovementVehicle
  (bind _endsplinepoint (Variables|Default|GetEndSplinePoint))
  (bind _splineref (Variables|Default|GetSplineRef))
  (bind _spline (Variables|/Game/_Main/Blueprints/Vehicles/BP_Spline_Vehicle.BP_Spline_Vehicle_C|GetSpline _splineref))
  (bind _returnvalue (Spline|GetNumberOfSplinePoints _spline))
  ;[1 1 1] Spline Movement
  (if (not (Variables|Default|GetTravelFinished?))
    (Utilities|MVehicleSound "NewEnumerator2")
    ;;[0.3438 0.04946 0.0392] Start Vehicle
    (Variables|Default|SetStartVehicle? true)
    (bind _returnvalue_2 (Utilities|Time|SetTimerbyEvent (delegate Custom|StopDrivingSlowly) (- (Variables|Default|GetTimeToTravel) 3.0)))
    (Variables|Default|SetTimerHandle _returnvalue_2)
    (Components|Timeline|SetPlayRate (Variables|Default|GetTimeline_Move_Vehicle) (/ 1.0 (Variables|Default|GetTimeToTravel))) ; How fast
    (Utilities|MVehicleSound "NewEnumerator3")
    (bind _float (Timeline|Timeline_Move_Vehicle PlayFromStart)
      (:Update
        (Transformation|SetActorTransform (Math|Transform|MakeTransform (.location (Spline|GetTransformatDistanceAlongSpline _spline (Math|Float|Lerp 0.0 (Spline|GetDistanceAlongSplineatSplinePoint _spline (Math|Integer|Clamp(Integer) (select (== _endsplinepoint 0) _returnvalue _endsplinepoint) 0 _returnvalue)) _float) "World" false)) (Math|Rotator|MakeRotator 0.0 0.0 (+ (.Yaw (Math|Rotator|BreakRotator (Spline|GetRotationatDistanceAlongSpline _spline (Math|Float|Lerp 0.0 (Spline|GetDistanceAlongSplineatSplinePoint _spline (Math|Integer|Clamp(Integer) (select (== _endsplinepoint 0) _returnvalue _endsplinepoint) 0 _returnvalue)) _float) "Local"))) (Variables|Default|GetOffset_Z_RotationSpline))) "1.000000,1.000000,1.000000")))
      (:Finished
        (Variables|Default|SetTravelFinished? true)
        (Utilities|Time|ClearandInvalidateTimerbyHandle (Variables|Default|GetTimerHandle))))))

(event Custom|Event_CheckForVehicleMovement
  (params (ChapterSegmentData :type S%20Chapter%20Segment%20Data%20Structure))
  (bind (_ch1_segment _ch2_segment _ch3_segment _ch4_segment _ch5_segment _ch6_segment _chapternumber_) (Utilities|Struct|BreakS_ChapterSegmentData ChapterSegmentData))
  (switch Utilities|FlowControl|Switch|SwitchonE_ChapterNumber _chapternumber_
    (:NewEnumerator2
      (switch Utilities|FlowControl|Switch|SwitchonE_Chapter3_Segments _ch3_segment
        (:NewEnumerator2
          (Variables|Default|SetTimeToTravel 4e+01))))))

(event EventBeginPlay
  (Rendering|SetVisibility (Variables|Default|GetLMG) (Variables|Default|GetTechnical?) false)
  (bind _returnvalue (Rendering|Material|CreateDynamicMaterialInstance (Variables|Default|GetSkeletalMesh) 2 "/Game/_Main/Assets/Vehicles/PickupTruck/Mat/Pickup_Paint_MI.Pickup_Paint_MI" "None" :!class /Script/Engine.PrimitiveComponent))
  (Rendering|Material|SetVectorParameterValue _returnvalue "Color" (Utilities|Array|Get(acopy) (Variables|Default|GetPickupColor) (Variables|Default|GetColorSwitcher)) :!class /Script/Engine.MaterialInstanceDynamic)
  (Rendering|SetVisibility (Variables|Default|GetSM_LibyanTechnical) (Variables|Default|GetTechnical?) false))

(event EventInteractwithVehicle
  (params (CharacterRef :type Character%20Object%20Reference) (InteractingManually? :type Boolean))
  ;[1 1 1] Sit  - Player
)

(event EventToggleVehicleDoors
  (params (Seat :type E_VehicleSeat%20Enum :default "NewEnumerator0"))
  ;[1 1 1] Doors
  (switch Utilities|FlowControl|Switch|SwitchonE_VehicleSeat Seat
    (:NewEnumerator0
      (Utilities|MVehicleSound "NewEnumerator0")
      (Variables|Default|SetDoor_FL_Open? true)
      (Utilities|FlowControl|Delay 4.0)
      (Variables|Default|SetDoor_FL_Open? false)
      (Utilities|MVehicleSound "NewEnumerator1"))
    (:NewEnumerator1
      (Utilities|MVehicleSound "NewEnumerator0")
      (Variables|Default|SetDoor_FR_Open? true)
      (Utilities|FlowControl|Delay 4.0)
      (Variables|Default|SetDoor_FR_Open? false)
      (Utilities|MVehicleSound "NewEnumerator1"))))

(event EventPickupTruckShowBoxes
  (params (ToggleBoxes? :type Boolean))
  ;[1 1 1] Boxes and BodyBags and Stretcher
  (Rendering|SetVisibility (Variables|Default|GetBoxes) ToggleBoxes? true))

(event EventUpdateChapterSegment
  (params (Struct_Ch_Seg_Data :type S%20Chapter%20Segment%20Data%20Structure))
  (bind _output_get (Variables|Default|SetChapterSegmentData Struct_Ch_Seg_Data))
  (CallFunction|EventCheckforVehicleMovement _output_get))

(event EventShowBodyBagsonPickupTruck
  (params (ToggleVisibility? :type Boolean) (BagLocation%281%20or%202%29 :type Integer))
  ;[1 1 1] Boxes and BodyBags and Stretcher
  (Rendering|SetVisibility (Utilities|Select :Index (Math|Integer|Clamp(Integer) BagLocation%281%20or%202%29 1 2) :Option%200 0 :Option%201 (Variables|Default|GetBodyBag_1) :Option%202 (Variables|Default|GetBodyBag_2)) ToggleVisibility? false))

(event EventTogglePickupTruckSoldier
  (params (Toggle :type Boolean))
  (Rendering|SetVisibility (Variables|Default|GetSM_LibyanTechnical) Toggle false))

(event EventFollowSplinePathVehicle
  (params (SplineRef :type BP%20Spline%20Vehicle%20Object%20Reference))
  ;[1 1 1] Spline Movement
  (Variables|Default|SetSplineRef SplineRef)
  (Variables|Default|SetTravelFinished? false)
  (CallFunction|StartMovementVehicle)
  (Development|PrintString "Pickup Truck Spline Movement"))

(event EventTogglePickupTrunk
  (params (Toggle? :type Boolean))
  ;[1 1 1] Trunk
  (Variables|Default|SetTrunkOpen? Toggle?))

(fn ConstructionScript)

(fn ObtainArrowsTransform
  (params (Seat%20Number :type Integer))
  (bind _seat_5 (Variables|Default|GetSeat_5))
  (bind _seat_2 (Variables|Default|GetSeat_2))
  (bind _seat_1 (Variables|Default|GetSeat_1))
  (bind _seat_6 (Variables|Default|GetSeat_6))
  (bind _seat_3 (Variables|Default|GetSeat_3))
  (bind _seat_4 (Variables|Default|GetSeat_4))
  (bind _returnvalue (Utilities|Select :Index Seat%20Number :Option%200 0 :Option%201 _seat_1 :Option%202 _seat_2 :Option%203 _seat_3 :Option%204 _seat_4 :Option%205 _seat_5 :Option%206 _seat_6))
  (bind _returnvalue_2 (Transformation|GetWorldTransform _returnvalue))
  (return (.location _returnvalue_2) (.rotation _returnvalue_2)))

(fn FetchArrowsfromVehicles
  (params (Seat :type E_VehicleSeat%20Enum :default "NewEnumerator0"))
  (bind _seat_passenger (Variables|Default|GetSeat_Passenger))
  (bind _seat_driver (Variables|Default|GetSeat_Driver))
  (bind _seat_trunk (Variables|Default|GetSeat_Trunk))
  (bind _returnvalue (Transformation|GetWorldTransform _seat_driver))
  (bind _returnvalue_2 (Transformation|GetWorldTransform _seat_trunk))
  (bind _returnvalue_3 (Transformation|GetWorldTransform _seat_passenger))
  (return (Utilities|Select :Index Seat :NewEnumerator0 (.location _returnvalue) :NewEnumerator1 (.location _returnvalue_3) :NewEnumerator2 "0, 0, 0" :NewEnumerator3 "0, 0, 0" :NewEnumerator4 "0, 0, 0" :NewEnumerator5 "0, 0, 0" :NewEnumerator6 (.location _returnvalue_2)) (Utilities|Select :Index Seat :NewEnumerator0 (.rotation _returnvalue) :NewEnumerator1 (.rotation _returnvalue_3) :NewEnumerator2 "0, 0, 0" :NewEnumerator3 "0, 0, 0" :NewEnumerator4 "0, 0, 0" :NewEnumerator5 "0, 0, 0" :NewEnumerator6 (.rotation _returnvalue_2))))

(fn GetVehicleNameandLoc
  (return "NewEnumerator6" (Transformation|GetActorLocation) (Transformation|GetActorRotation)))

(fn IsVehicleMoving?
  (return false))

(fn ObtainTrunkArrowsPickup
  (params (Seat%281-6%29 :type Integer))
  (bind (_arrowlocation _arrowrotation) (CallFunction|ObtainArrowsTransform Seat%281-6%29))
  (return _arrowlocation _arrowrotation))

(fn PlayerDependentLight?
  (return false))