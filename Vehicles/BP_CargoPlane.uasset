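; Cargo plane vehicle actor that travels along a given spline, plays flight audio and opens or closes its cargo bay.
; A timeline timed by TimeToTravel drives position and offset yaw from the spline, with pitch either following it or ramping during takeoff.
; Audio switches from landing to idle on arrival, with a separate timed interior takeoff sound.
; A second timeline animates bay doors and tray, while the vehicle query functions return only defaults.
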(event Custom|ToggleCargoBay
  (params (Toggle? :type Boolean))
  (Audio|PlaySoundatLocation "/Game/_Main/Sounds/Airport/CargoDoor_OpenClose.CargoDoor_OpenClose" (Transformation|GetWorldLocation (Variables|Default|GetCargoBay_Bottom)) "0, 0, 0" 0.75 1.0 0.0 "/Game/_Main/Blueprints/Vehicles/VehicleAttenuation.VehicleAttenuation" 0 self 0)
  (if Toggle?
    (bind _float (Timeline|Timeline_CargoBay PlayFromStart) ; 8s
      (:Update
        (Transformation|SetRelativeLocation (Variables|Default|GetCargoBay_Tray) (Math|Vector|MakeVector 0.0 (Math|Float|Lerp -5.1e+02 -704.0 _float) (Math|Float|Lerp 86.0 1.2e+02 _float)) false false)
        (Transformation|SetRelativeRotation (Variables|Default|GetCargoBay_Bottom) (Math|Rotator|MakeRotator (Math|Float|Lerp 0.0 -25.0 _float) 0.0 0.0) false false)
        (Transformation|SetRelativeRotation (Variables|Default|GetCargoBay_Top) (Math|Rotator|MakeRotator (Math|Float|Lerp 0.0 -29.0 _float) 0.0 0.0) false false)))
    (else
      (Timeline|Timeline_CargoBay ReverseFromEnd))))

(event Custom|Event_CargoPlaneTakeOffSound
  (bind _audio (Variables|Default|GetAudio))
  (Audio|Components|Audio|SetSound _audio "/Game/_Main/Sounds/Airport/CargoPlane_TakeOff_Interior.CargoPlane_TakeOff_Interior")
  (Audio|Components|Audio|FadeIn _audio 1.0 1.0 0.0 "Linear" :!class /Script/Engine.AudioComponent)
  (Utilities|FlowControl|Delay 23.0)
  (Audio|Components|Audio|FadeOut _audio 2.0 0.0 "Linear" :!class /Script/Engine.AudioComponent))

(event EventFollowSplinePathVehicle
  (params (SplineRef :type BP%20Spline%20Vehicle%20Object%20Reference))
  (bind _audio (Variables|Default|GetAudio))
  (bind _audio_2 (Variables|Default|GetAudio))
  (Variables|Default|SetSplineRef SplineRef)
  (Components|Timeline|SetPlayRate (Variables|Default|GetTimelineSplineTravel) (/ 1.0 (Variables|Default|GetTimeToTravel))) ; How fast
  (Audio|Components|Audio|SetSound _audio_2 "/Game/_Main/Sounds/Airport/CargoBob_Landing_Ch6.CargoBob_Landing_Ch6")
  (Audio|Components|Audio|FadeIn _audio_2 1.0 1.0 0.0 "Linear" :!class /Script/Engine.AudioComponent)
  (bind _float (Timeline|TimelineSplineTravel PlayFromStart)
    (:Update
      (Transformation|SetActorTransform (Math|Transform|MakeTransform (.location (Spline|GetTransformatDistanceAlongSpline (Variables|/Game/_Main/Blueprints/Vehicles/BP_Spline_Vehicle.BP_Spline_Vehicle_C|GetSpline (Variables|Default|GetSplineRef)) (Math|Float|Lerp 0.0 (Spline|GetSplineLength (Variables|/Game/_Main/Blueprints/Vehicles/BP_Spline_Vehicle.BP_Spline_Vehicle_C|GetSpline (Variables|Default|GetSplineRef))) _float) "World" false)) (select (Variables|Default|GetTakeOff?) (Math|Rotator|MakeRotator 0.0 (Math|Float|Lerp 0.0 -35.0 _float) (+ (.Yaw (Math|Rotator|BreakRotator (Spline|GetRotationatDistanceAlongSpline (Variables|/Game/_Main/Blueprints/Vehicles/BP_Spline_Vehicle.BP_Spline_Vehicle_C|GetSpline (Variables|Default|GetSplineRef)) (Math|Float|Lerp 0.0 (Spline|GetSplineLength (Variables|/Game/_Main/Blueprints/Vehicles/BP_Spline_Vehicle.BP_Spline_Vehicle_C|GetSpline (Variables|Default|GetSplineRef))) _float) "Local"))) (Variables|Default|GetOffset_Z_RotationSpline))) (Math|Rotator|MakeRotator (.Roll (Math|Rotator|BreakRotator (Spline|GetRotationatDistanceAlongSpline (Variables|/Game/_Main/Blueprints/Vehicles/BP_Spline_Vehicle.BP_Spline_Vehicle_C|GetSpline (Variables|Default|GetSplineRef)) (Math|Float|Lerp 0.0 (Spline|GetSplineLength (Variables|/Game/_Main/Blueprints/Vehicles/BP_Spline_Vehicle.BP_Spline_Vehicle_C|GetSpline (Variables|Default|GetSplineRef))) _float) "Local"))) (.Pitch (Math|Rotator|BreakRotator (Spline|GetRotationatDistanceAlongSpline (Variables|/Game/_Main/Blueprints/Vehicles/BP_Spline_Vehicle.BP_Spline_Vehicle_C|GetSpline (Variables|Default|GetSplineRef)) (Math|Float|Lerp 0.0 (Spline|GetSplineLength (Variables|/Game/_Main/Blueprints/Vehicles/BP_Spline_Vehicle.BP_Spline_Vehicle_C|GetSpline (Variables|Default|GetSplineRef))) _float) "Local"))) (+ (.Yaw (Math|Rotator|BreakRotator (Spline|GetRotationatDistanceAlongSpline (Variables|/Game/_Main/Blueprints/Vehicles/BP_Spline_Vehicle.BP_Spline_Vehicle_C|GetSpline (Variables|Default|GetSplineRef)) (Math|Float|Lerp 0.0 (Spline|GetSplineLength (Variables|/Game/_Main/Blueprints/Vehicles/BP_Spline_Vehicle.BP_Spline_Vehicle_C|GetSpline (Variables|Default|GetSplineRef))) _float) "Local"))) (Variables|Default|GetOffset_Z_RotationSpline)))) "1.000000,1.000000,1.000000")))
    (:Finished
      (Audio|Components|Audio|SetSound _audio "/Game/_Main/Sounds/Airport/CargoPlane_Idle.CargoPlane_Idle")
      (Audio|Components|Audio|FadeIn _audio 2.0 1.0 0.0 "Linear" :!class /Script/Engine.AudioComponent))))

(fn ConstructionScript)

(fn FetchArrowsfromVehicles
  (params (Seat :type E_VehicleSeat%20Enum :default "NewEnumerator0"))
  (return "0, 0, 0" "0, 0, 0"))

(fn GetVehicleNameandLoc
  (return "NewEnumerator0" "0, 0, 0" "0, 0, 0"))

(fn IsVehicleMoving?
  (return false))

(fn ObtainTrunkArrowsPickup
  (params (Seat%281-6%29 :type Integer))
  (return "0, 0, 0" "0, 0, 0"))

(fn PlayerDependentLight?
  (return false))