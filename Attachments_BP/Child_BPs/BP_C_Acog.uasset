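; ACOG scope attachment Blueprint, a child class that sets how the optic looks when the player aims down sights.
; ScopeInOut switches on the scope-in mode and handles only Standard in this file.
; In that mode ADS hides the Lens and squashes AttachmentMesh along X, both restored on exit, while the RTLens stays hidden.
; BeginPlay and construction just call the parent.
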(event EventBeginPlay
  (|CallParentFunction))

(event Collision|EventActorBeginOverlap
  (params (OtherActor :type Actor%20Object%20Reference))
  (|CallParentFunction OtherActor) ; This node is disabled and will not be called.\nDrag off pins to build functionality.
)

(event EventTick
  (params (DeltaSeconds :type Float%20%28single-precision%29))
  (|CallParentFunction DeltaSeconds) ; This node is disabled and will not be called.\nDrag off pins to build functionality.
)

(fn ConstructionScript
  (|CallParentFunction))

(fn ScopeinOut
  (params (IsInADS? :type Boolean) (ScopeInMode :type E_ScopeInMode%20Enum :default "NewEnumerator0"))
  (switch Utilities|FlowControl|Switch|SwitchonE_ScopeInMode ScopeInMode
    (:NewEnumerator0
      (Rendering|SetVisibility (Variables|Default|GetLens) (not IsInADS?) false)
      (Rendering|SetVisibility (Variables|Default|GetRTLens) false false)
      (Transformation|SetRelativeScale3D (Variables|Default|GetAttachmentMesh) (Math|Vector|MakeVector (select IsInADS? 0.15 1.0) 1.0 1.0)))))