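; Leupold 6x scope attachment, a child Blueprint that changes the scope's visuals when entering or leaving ADS.
; ScopeInOut branches on scope mode, hiding the regular lens during ADS in both Standard and Picture in Picture.
; Standard also swaps the trim mesh for a cut mesh flattened along X, with RTLens hidden.
; Picture in Picture instead shows RTLens while aiming and leaves the mesh untouched.
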(event EventBeginPlay
  (|CallParentFunction) ; This node is disabled and will not be called.\nDrag off pins to build functionality.
)

(event Collision|EventActorBeginOverlap
  (params (OtherActor :type Actor%20Object%20Reference))
  (|CallParentFunction OtherActor) ; This node is disabled and will not be called.\nDrag off pins to build functionality.
)

(event EventTick
  (params (DeltaSeconds :type Float%20%28single-precision%29))
  (|CallParentFunction DeltaSeconds) ; This node is disabled and will not be called.\nDrag off pins to build functionality.
)

(fn ConstructionScript
  (|CallParentFunction))

(fn ScopeinOut
  (params (IsInADS? :type Boolean) (ScopeInMode :type E_ScopeInMode%20Enum :default "NewEnumerator0"))
  (bind _returnvalue (not IsInADS?))
  (bind _attachmentmesh (Variables|Default|GetAttachmentMesh))
  (switch Utilities|FlowControl|Switch|SwitchonE_ScopeInMode ScopeInMode
    (:NewEnumerator0
      (Rendering|SetVisibility (Variables|Default|GetLens) _returnvalue false)
      (Rendering|SetVisibility (Variables|Default|GetRTLens) false false)
      (if IsInADS?
        (Components|StaticMesh|SetStaticMesh _attachmentmesh "/Game/_Main/Weapons/Attachments/Leupold6x_Cut.Leupold6x_Cut")
        (Transformation|SetRelativeScale3D (Variables|Default|GetAttachmentMesh) "0.150000,1.000000,1.000000")
        (else
          (Components|StaticMesh|SetStaticMesh _attachmentmesh "/Game/_Main/Weapons/Attachments/Leupold6x_Trim.Leupold6x_Trim")
          (Transformation|SetRelativeScale3D (Variables|Default|GetAttachmentMesh) "1.000000,1.000000,1.000000"))))
    (:NewEnumerator1
      (Rendering|SetVisibility (Variables|Default|GetRTLens) IsInADS? false)
      (Rendering|SetVisibility (Variables|Default|GetLens) _returnvalue false))))