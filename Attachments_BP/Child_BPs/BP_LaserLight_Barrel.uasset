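; BP_LaserLight_Barrel is a barrel attachment Blueprint that provides a toggleable laser sight with a dot decal where it hits.
; ToggleLaser shows or hides the laser mesh and starts or clears a fast looping timer, hiding the decal when switched off.
; Each tick of that timer line traces forward from the mesh, placing the decal aligned to the impact normal or hiding it when nothing is hit.
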(event Custom|ToggleLaser
  (params (Visibility :type Boolean))
  (Rendering|SetVisibility (Variables|Default|GetLaserMesh) Visibility false)
  (if Visibility
    (bind _returnvalue (Utilities|Time|SetTimerbyEvent (delegate Custom|LaserLineTrace) 0.05 true))
    (Variables|Default|SetLaserTimer _returnvalue)
    (else
      (Utilities|Time|ClearandInvalidateTimerbyHandle (Variables|Default|GetLaserTimer))
      (Rendering|SetVisibility (Variables|Default|GetLaserDecal) false false))))

(event Custom|LaserLineTrace
  (bind _lasermesh (Variables|Default|GetLaserMesh))
  (bind _laserdecal (Variables|Default|GetLaserDecal))
  (bind _returnvalue (Transformation|GetWorldLocation _lasermesh))
  (bind _outhit (Collision|LineTraceByChannel _returnvalue (+ _returnvalue (* (Math|Vector|GetForwardVector _lasermesh) (Variables|Default|GetLaserDistance))) "TraceTypeQuery1" true 0 "None" true "(R=1.000000,G=0.000000,B=0.000000,A=1.000000)" "(R=0.000000,G=1.000000,B=0.000000,A=1.000000)" 0.05))
  (if (.bBlockingHit (Collision|BreakHitResult _outhit))
    (Transformation|SetWorldLocationAndRotation _laserdecal (.Location (Collision|BreakHitResult _outhit)) (Math|Rotator|MakeRotfromX (.ImpactNormal (Collision|BreakHitResult _outhit))) false false)
    (Rendering|SetVisibility _laserdecal true false)
    (else
      (Rendering|SetVisibility _laserdecal false false))))

(fn ConstructionScript)