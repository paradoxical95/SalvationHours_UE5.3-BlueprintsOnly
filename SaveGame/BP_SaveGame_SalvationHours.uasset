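; SaveGame object for Salvation Hours that stores player settings and campaign progress.
; Paired save and get functions copy grouped values in and out: controls, audio, visuals, upscalers, FPS toggle, player transform, time and combat state, and weapon attachments.
; It also keeps chapter segment states with active map, save point and task, plus named location data for four NPC groups and the vehicles.
; Only the chapter save prints a debug string.
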(fn SaveVisualStuff
  (params (SoftwareRT? :type Boolean))
  (Variables|VisualStuff|SetSoftwareLumen? SoftwareRT?))

(fn SaveControlStuff
  (params (GameDifficulty :type E_GameDifficulty%20Enum :default "NewEnumerator0") (X_Invert? :type Boolean) (Y_Invert? :type Boolean) (X_Sens_Multiplier :type Float%20%28double-precision%29) (Y_Sens_Multiplier :type Float%20%28double-precision%29) (FOV_Value :type Float%20%28double-precision%29) (ACOG_Sens :type Float%20%28double-precision%29) (Gamepad_Sens_Horz :type Float%20%28single-precision%29) (Gamepad_Sens_Vert :type Float%20%28single-precision%29) (Gamepad_Vert_Invert? :type Boolean) (WereThumbsticksFlipped? :type Boolean))
  (Variables|PlayerControls|SetGameDifficulty GameDifficulty)
  (Variables|PlayerControls|SetMouseX_Invert? X_Invert?)
  (Variables|PlayerControls|SetMouseY_Invert? Y_Invert?)
  (Variables|PlayerControls|SetMouseX_Sens_Multiplier X_Sens_Multiplier) ; make sure the range is proper
  (Variables|PlayerControls|SetMouseY_Sens_Multiplier Y_Sens_Multiplier)
  (Variables|PlayerControls|SetFOV%20Value FOV_Value)
  (Variables|PlayerControls|SetACOG_Sens ACOG_Sens)
  (Variables|PlayerControls|SetGamepad_Sens_Horz Gamepad_Sens_Horz)
  (Variables|PlayerControls|SetGamepad_Sens_Vert Gamepad_Sens_Vert)
  (Variables|PlayerControls|SetGamepad_Vert_Invert? Gamepad_Vert_Invert?)
  (Variables|PlayerControls|SetWereThumbsticksFlipped? WereThumbsticksFlipped?))

(fn SaveAudioStuff
  (params (AmbientVol :type Float%20%28double-precision%29) (EffectsVol :type Float%20%28double-precision%29) (MusicVol :type Float%20%28double-precision%29) (DialogueVol :type Float%20%28double-precision%29))
  (Variables|AudioStuff|SetAmbientVol AmbientVol)
  (Variables|AudioStuff|SetEffectsVol EffectsVol)
  (Variables|AudioStuff|SetMusicVol MusicVol)
  (Variables|AudioStuff|SetDialogueVol DialogueVol))

(fn SavePlayerData
  (params (PlayerTransform :type Transform) (TimeInHours :type Integer) (TimeInMinutes :type Integer) (PlayerCombatState :type E_CombatStates%20Enum :default "NewEnumerator0"))
  (Variables|PlayerGeneralData|SetPlayerTransform PlayerTransform)
  (Variables|PlayerGeneralData|SetTimeInHours TimeInHours)
  (Variables|PlayerGeneralData|SetTimeInMinutes TimeInMinutes)
  (Variables|PlayerGeneralData|SetPlayer%20Combat%20State PlayerCombatState))

(fn SaveWeaponData
  (params (OpticName :type E_Optics%20Enum :default "NewEnumerator0") (CantedAttached? :type Boolean) (SuppressorAttached?%20 :type Boolean) (VerticalGripAttached? :type Boolean) (FlashlightAttached? :type Boolean) (LaserLightAttached? :type Boolean) (PistolActive? :type Boolean))
  (Variables|WeaponData|SetOptic%20Name OpticName)
  (Variables|WeaponData|SetCanted%20Attached? CantedAttached?)
  (Variables|WeaponData|SetSuppressor%20Attached? SuppressorAttached?%20)
  (Variables|WeaponData|SetVertical%20Grip%20Attached? VerticalGripAttached?)
  (Variables|WeaponData|SetFlashlightAttached? FlashlightAttached?)
  (Variables|WeaponData|SetLaserLightAttached? LaserLightAttached?)
  (Variables|WeaponData|SetPistol%20Active? PistolActive?))

(fn GetSavedControlStuff
  (return (Variables|PlayerControls|GetGameDifficulty) (Variables|PlayerControls|GetMouseX_Invert?) (Variables|PlayerControls|GetMouseY_Invert?) (Variables|PlayerControls|GetMouseX_Sens_Multiplier) (Variables|PlayerControls|GetMouseY_Sens_Multiplier) (Variables|PlayerControls|GetFOV%20Value) (Variables|PlayerControls|GetACOG_Sens) (Variables|PlayerControls|GetGamepad_Sens_Horz) (Variables|PlayerControls|GetGamepad_Sens_Vert) (Variables|PlayerControls|GetGamepad_Vert_Invert?) (Variables|PlayerControls|GetWereThumbsticksFlipped?)))

(fn GetSavedVisualStuff
  (return (Variables|VisualStuff|GetSoftwareLumen?)))

(fn GetSavedPlayerData
  (return (Variables|PlayerGeneralData|GetPlayerTransform) (Variables|PlayerGeneralData|GetTimeInHours) (Variables|PlayerGeneralData|GetTimeInMinutes) (Variables|PlayerGeneralData|GetPlayer%20Combat%20State)))

(fn SaveToggleFPS
  (params (ToggleFPS? :type Boolean))
  (Variables|VisualStuff|SetToggleFPS? ToggleFPS?))

(fn GetSavedToggleFPS
  (return (Variables|VisualStuff|GetToggleFPS?)))

(fn GetSavedNPCLocDataTripoli
  (return (Variables|LocDataNPC|GetLoc%20Data%20Jim) (Variables|LocDataNPC|GetLoc%20Data%20Delta%20A) (Variables|LocDataNPC|GetLoc%20Data%20Delta%20B) (Variables|LocDataNPC|GetLoc%20Data%20Delta%20C0) (Variables|LocDataNPC|GetLoc%20Data%20Delta%20C1) (Variables|LocDataNPC|GetLoc%20Data%20Country%20TL)))

(fn GetSavedWeaponData
  (return (Variables|WeaponData|GetOptic%20Name) (Variables|WeaponData|GetCanted%20Attached?) (Variables|WeaponData|GetSuppressor%20Attached?) (Variables|WeaponData|GetVertical%20Grip%20Attached?) (Variables|WeaponData|GetFlashlightAttached?) (Variables|WeaponData|GetLaserLightAttached?) (Variables|WeaponData|GetPistol%20Active?)))

(fn SaveChapterStates
  (params (ChapterNumber :type E_ChapterNumber%20Enum :default "NewEnumerator0") (CH1_Segments :type E_Chapter1_Segments%20Enum :default "NewEnumerator0") (CH2_Segments :type E_Chapter2_Segments%20Enum :default "NewEnumerator6") (CH3_Segments :type E_Chapter3_Segments%20Enum :default "NewEnumerator6") (CH4_Segments :type E_Chapter4_Segments%20Enum :default "NewEnumerator15") (CH5_Segments :type E_Chapter5_Segments%20Enum :default "NewEnumerator15") (CH6_Segments :type E_Chapter6_Segments%20Enum :default "NewEnumerator15") (ActiveLevelMap :type E_LevelMap%20Enum :default "NewEnumerator0") (SavePoint :type E_SavePoints%20Enum :default "NewEnumerator0") (ActiveTask :type Integer))
  (bind _output_get (Variables|ChapterStates|SetChapterNumber ChapterNumber))
  (Variables|ChapterStates|SetCH1_Segments CH1_Segments)
  (Variables|ChapterStates|SetCH2_Segments CH2_Segments)
  (Variables|ChapterStates|SetCH3_Segments CH3_Segments)
  (Variables|ChapterStates|SetCH4_Segments CH4_Segments)
  (Variables|ChapterStates|SetCH5_Segments CH5_Segments)
  (Variables|ChapterStates|SetCH6_Segments CH6_Segments)
  (bind _output_get_2 (Variables|Default|SetActiveMap ActiveLevelMap))
  (bind _output_get_3 (Variables|Default|SetSavePoint SavePoint))
  (Variables|ChapterStates|SetActiveTaskNumber ActiveTask)
  (Development|PrintString 0 (Utilities|String|Append "SaveGameBP  : 
Active Map - " (Utilities|String|EnumtoString _output_get_2) " 
Save Point - " (Utilities|String|EnumtoString _output_get_3) " 
Chapter Number - " (Utilities|String|EnumtoString _output_get)) true true "(R=0.000000,G=0.148287,B=1.000000,A=1.000000)" 3.0))

(fn GetSavedChapterStates
  (return (Variables|ChapterStates|GetChapterNumber) (Variables|ChapterStates|GetCH1_Segments) (Variables|ChapterStates|GetCH2_Segments) (Variables|ChapterStates|GetCH3_Segments) (Variables|ChapterStates|GetCH4_Segments) (Variables|ChapterStates|GetCH5_Segments) (Variables|ChapterStates|GetCH6_Segments) (Variables|Default|GetActiveMap) (Variables|Default|GetSavePoint) (Variables|ChapterStates|GetActiveTaskNumber)))

(fn SaveNPCLocDataGRS
  (params (LocDataDrew :type S%20NPC%20Transform%20Structure) (LocDataRob :type S%20NPC%20Transform%20Structure) (LocDataRic :type S%20NPC%20Transform%20Structure) (LocDataDC :type S%20NPC%20Transform%20Structure) (LocDataMat :type S%20NPC%20Transform%20Structure))
  (Variables|LocDataNPC|SetLoc%20Data%20Drew LocDataDrew)
  (Variables|LocDataNPC|SetLoc%20Data%20Rob LocDataRob)
  (Variables|LocDataNPC|SetLoc%20Data%20Ric LocDataRic)
  (Variables|LocDataNPC|SetLoc%20Data%20DC LocDataDC)
  (Variables|LocDataNPC|SetLoc%20Data%20Mat LocDataMat))

(fn SaveNPCLocDataDS
  (params (LocDataAmbo :type S%20NPC%20Transform%20Structure) (LocDataMarcus :type S%20NPC%20Transform%20Structure) (LocDataFred :type S%20NPC%20Transform%20Structure) (LocDataCody :type S%20NPC%20Transform%20Structure) (LocDataAlex :type S%20NPC%20Transform%20Structure) (LocDataCarlos :type S%20NPC%20Transform%20Structure) (LocDataFloyd :type S%20NPC%20Transform%20Structure))
  (Variables|LocDataNPC|SetLoc%20Data%20Ambo LocDataAmbo)
  (Variables|LocDataNPC|SetLoc%20Data%20Marcus LocDataMarcus)
  (Variables|LocDataNPC|SetLoc%20Data%20Fred LocDataFred)
  (Variables|LocDataNPC|SetLoc%20Data%20Cody LocDataCody)
  (Variables|LocDataNPC|SetLoc%20Data%20Alex LocDataAlex)
  (Variables|LocDataNPC|SetLoc%20Data%20Carlos LocDataCarlos)
  (Variables|LocDataNPC|SetLoc%20Data%20Floyd LocDataFloyd))

(fn SaveNPCLocDataAnnex
  (params (LocDataWalker :type S%20NPC%20Transform%20Structure) (LocDataJeff :type S%20NPC%20Transform%20Structure) (LocDataPhillip :type S%20NPC%20Transform%20Structure) (LocDataNancy :type S%20NPC%20Transform%20Structure) (LocDataChester :type S%20NPC%20Transform%20Structure) (LocDataMike :type S%20NPC%20Transform%20Structure))
  (Variables|LocDataNPC|SetLoc%20Data%20Walker LocDataWalker)
  (Variables|LocDataNPC|SetLoc%20Data%20Jeff LocDataJeff)
  (Variables|LocDataNPC|SetLoc%20Data%20Phillip LocDataPhillip)
  (Variables|LocDataNPC|SetLoc%20Data%20Nancy LocDataNancy)
  (Variables|LocDataNPC|SetLoc%20Data%20Chester LocDataChester)
  (Variables|LocDataNPC|SetLoc%20Data%20Mike LocDataMike))

(fn SaveNPCLocDataTripoli
  (params (LocDataJim :type S%20NPC%20Transform%20Structure) (LocDataDeltaA :type S%20NPC%20Transform%20Structure) (LocDataDeltaB :type S%20NPC%20Transform%20Structure) (LocDataDeltaC0 :type S%20NPC%20Transform%20Structure) (LocDataDeltaC1 :type S%20NPC%20Transform%20Structure) (LocDataCountryTL :type S%20NPC%20Transform%20Structure))
  (Variables|LocDataNPC|SetLoc%20Data%20Jim LocDataJim)
  (Variables|LocDataNPC|SetLoc%20Data%20Delta%20A LocDataDeltaA)
  (Variables|LocDataNPC|SetLoc%20Data%20Delta%20B LocDataDeltaB)
  (Variables|LocDataNPC|SetLoc%20Data%20Delta%20C0 LocDataDeltaC0)
  (Variables|LocDataNPC|SetLoc%20Data%20Delta%20C1 LocDataDeltaC1)
  (Variables|LocDataNPC|SetLoc%20Data%20Country%20TL LocDataCountryTL))

(fn GetSavedNPCLocDataGRS
  (return (Variables|LocDataNPC|GetLoc%20Data%20Drew) (Variables|LocDataNPC|GetLoc%20Data%20Rob) (Variables|LocDataNPC|GetLoc%20Data%20Ric) (Variables|LocDataNPC|GetLoc%20Data%20DC) (Variables|LocDataNPC|GetLoc%20Data%20Mat)))

(fn GetSavedNPCLocDataDS
  (return (Variables|LocDataNPC|GetLoc%20Data%20Ambo) (Variables|LocDataNPC|GetLoc%20Data%20Marcus) (Variables|LocDataNPC|GetLoc%20Data%20Fred) (Variables|LocDataNPC|GetLoc%20Data%20Cody) (Variables|LocDataNPC|GetLoc%20Data%20Alex) (Variables|LocDataNPC|GetLoc%20Data%20Carlos) (Variables|LocDataNPC|GetLoc%20Data%20Floyd)))

(fn GetSavedNPCLocDataAnnex
  (return (Variables|LocDataNPC|GetLoc%20Data%20Walker) (Variables|LocDataNPC|GetLoc%20Data%20Jeff) (Variables|LocDataNPC|GetLoc%20Data%20Phillip) (Variables|LocDataNPC|GetLoc%20Data%20Nancy) (Variables|LocDataNPC|GetLoc%20Data%20Chester) (Variables|LocDataNPC|GetLoc%20Data%20Mike)))

(fn SaveVehicleLocations
  (params (LocData_EClass :type S%20Vehicle%20Transform%20Structure) (LocData_BMW :type S%20Vehicle%20Transform%20Structure) (LocData_Jeep_SMC :type S%20Vehicle%20Transform%20Structure) (LocData_Jeep_Delta :type S%20Vehicle%20Transform%20Structure) (LocData_GWagon :type S%20Vehicle%20Transform%20Structure))
  (Variables|VehicleLocData|SetLocData_EClass LocData_EClass)
  (Variables|VehicleLocData|SetLocData_BMW LocData_BMW)
  (Variables|VehicleLocData|SetLocData_Jeep_SMC LocData_Jeep_SMC)
  (Variables|VehicleLocData|SetLocData_Jeep_Delta LocData_Jeep_Delta)
  (Variables|VehicleLocData|SetLocData_GWagon LocData_GWagon))

(fn GetSavedVehicleLocData
  (return (Variables|VehicleLocData|GetLocData_EClass) (Variables|VehicleLocData|GetLocData_BMW) (Variables|VehicleLocData|GetLocData_Jeep_SMC) (Variables|VehicleLocData|GetLocData_Jeep_Delta) (Variables|VehicleLocData|GetLocData_GWagon)))

(fn GetSavedAudioData
  (return (Variables|AudioStuff|GetAmbientVol) (Variables|AudioStuff|GetEffectsVol) (Variables|AudioStuff|GetMusicVol) (Variables|AudioStuff|GetDialogueVol)))

(fn SaveUpscalerData
  (params (UpscalersData :type S%20Upscaler%20Data%20Total%20Structure))
  (Variables|VisualStuff|SetUpscalersData UpscalersData))

(fn GetSavedUpscalerData
  (return (Variables|VisualStuff|GetUpscalersData)))