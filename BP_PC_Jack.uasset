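; Player controller for Jack that acts as the central hub for the player's UI.
; BeginPlay creates the main widgets and adds the Enhanced Input context, while events relay gameplay updates to HUD and subtitle widgets.
; Pause, attachments, death and friendly-fire screens switch input mode and cursor, with death quotes drawn randomly from an async-loaded DataTable.
; It also handles pausing on input device connection changes, FOV updates and FSR3 re-application after unpausing.
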(event Custom|Event_CheckAndSet_FSR3
  ;[1 0.02526 0] FSR3 CRASH HANDLE CODE
  (if (Variables|Default|GetDidPlayerSwitchToFSR?)
    (Development|ExecuteConsoleCommand "r.FidelityFX.FSR3.Enabled 1" 0)
    (Development|ExecuteConsoleCommand (Utilities|String|BuildString(Integer) "" "r.FidelityFX.FSR3.QualityMode " (Variables|Default|GetFSR_Preset_Value)) 0)))

(event Custom|Event_OnInputDeviceConnectionChange
  (params (NewConnectionState :type EInputDeviceConnectionState%20Enum :default "Invalid") (PlatformUserId :type Platform%20User%20Id%20Structure) (InputDeviceId :type Input%20Device%20Id%20Structure))
  ;[0.4262 0.9701 1] Gamepad Connect/Disconnect
  (if (not (Variables|Default|GetIsGamePaused?))
    (CallFunction|CECreatePauseMenuGamepadConnection)))

(event Custom|CE_CreatePauseMenu_GamepadConnection
  ;[0.2917 0.1868 0.1456] Pause Menu
  (CallFunction|CreatePauseMenuWidget true))

(event EventBeginPlay
  (bind _returnvalue (PlayerController|LocalPlayerSubsystems|GetEnhancedInputLocalPlayerSubsystem))
  (bind _returnvalue_2 (Class|EnhancedInputSubsystemInterface|GetUserSettings _returnvalue))
  (bind _returnvalue_3 (UserInterface|CreateWidget "/Game/_Main/Blueprints/UserInterface/WBP_FPS_Counter.WBP_FPS_Counter_C"))
  (bind _output_get (Variables|Default|SetFPS_Widget _returnvalue_3))
  (UserInterface|Viewport|AddtoViewport _output_get 2)
  (bind _returnvalue_4 (UserInterface|CreateWidget "/Game/_Main/Blueprints/UserInterface/WBP_Subtitles.WBP_Subtitles_C" self))
  (bind _output_get_2 (Variables|Default|SetSubtitleWidget _returnvalue_4))
  (UserInterface|Viewport|AddtoViewport _output_get_2 2)
  (bind _returnvalue_5 (UserInterface|CreateWidget "/Game/_Main/Blueprints/UserInterface/WBP_HUD.WBP_HUD_C" self))
  (bind _output_get_3 (Variables|Default|SetHUD_Widget _returnvalue_5))
  (UserInterface|Viewport|AddtoViewport _output_get_3 0)
  (bind _returnvalue_6 (UserInterface|CreateWidget "/Game/_Main/Blueprints/UserInterface/PauseMenu/PauseMenu_Main.PauseMenu_Main_C" self))
  (Variables|Default|SetPauseMenu_Widget _returnvalue_6)
  (bind _returnvalue_7 (UserInterface|CreateWidget "/Game/_Main/Blueprints/UserInterface/WBP_Fade.WBP_Fade_C" self))
  (Variables|Default|SetFadeWidget _returnvalue_7)
  (bind _returnvalue_8 (UserInterface|CreateWidget "/Game/_Main/Blueprints/UserInterface/WBP_DayDateTime.WBP_DayDateTime_C" self))
  (Variables|Default|SetDayDateTimeWidget_Ref _returnvalue_8)
  (bind _returnvalue_9 (UserInterface|CreateWidget "/Game/_Main/Blueprints/UserInterface/WBP_FriendlyFire.WBP_FriendlyFire_C" self))
  (Variables|Default|SetFriendlyFireWidget _returnvalue_9)
  ;[1 1 1] Enhanced Input
  (Utilities|IsValid _returnvalue
    (:Is%20Valid
      (Input|AddMappingContext _returnvalue "/Game/_Main/Blueprints/EnhancedInput/IMC_SalvationHours.IMC_SalvationHours" 0 "(bIgnoreAllPressedKeysUntilRelease=True,bForceImmediately=False,bNotifyUserSettings=False)")
      (if (not (Class|EnhancedInputUserSettings|IsMappingContextRegistered _returnvalue_2 "/Game/_Main/Blueprints/EnhancedInput/IMC_SalvationHours.IMC_SalvationHours"))
        (Class|EnhancedInputUserSettings|RegisterInputMappingContext _returnvalue_2 "/Game/_Main/Blueprints/EnhancedInput/IMC_SalvationHours.IMC_SalvationHours")
        ;[0.4262 0.9701 1] Gamepad Connect/Disconnect
        (EventDispatchers|BindEventtoOnInputDeviceConnectionChange (Game|GetGameInstance) (delegate Custom|Event_OnInputDeviceConnectionChange))))))

(event EventGetPlayerFiringMode
  (params (Mode? :type E_FireMode%20Enum :default "NewEnumerator2"))
  ;[1 1 1] HUD Related
  (Default|GetFiringMode (Variables|Default|GetHUD_Widget) Mode?))

(event EventToggleSubtitleVisibility
  (params (Visible? :type Boolean))
  ;[1 1 1] Subtitle Widget
)

(event EventToggleNPCNameWidget
  (params (Toggle? :type Boolean) (NPC_Name :type E_CharacterNames%20Enum :default "NewEnumerator0"))
  ;[1 1 1 1 14] NPC Name Widget part
  (Default|ShowandUpdateNameNPC (Variables|Default|GetHUD_Widget) Toggle? NPC_Name))

(event EventToggleTaskWidget
  (params (Toggle? :type Boolean) (TaskText :type Text))
  ;[1 1 1] Task Widget
  (Default|ShowandUpdateTask (Variables|Default|GetHUD_Widget) Toggle? TaskText))

(event EventFadetoBlackWidget
  (params (Forwards? :type Boolean))
  (bind _fadewidget (Variables|Default|GetFadeWidget))
  ;[1 1 1] FadeToBlackWidget
  (if Forwards?
    (UserInterface|Viewport|AddtoViewport _fadewidget 0)
    (Default|FadetoBlack _fadewidget true)
    (else
      (if (UserInterface|Viewport|IsinViewport _fadewidget)
        _
        (else
          (UserInterface|Viewport|AddtoViewport _fadewidget 0)))
      (Default|FadetoBlack _fadewidget false)
      (Utilities|FlowControl|Delay 3.0)
      (Widget|RemovefromParent _fadewidget))))

(event EventHideAmmoWidget
  (params (Hide? :type Boolean))
  ;[1 1 1] Hiding Ammo Widget
  (Default|EventHideAmmoWidget (Variables|Default|GetHUD_Widget) Hide?))

(event EventPlayHealWidget
  ;[1 1 1] Damage, Hitmarker and Heal Widgets
  (Default|HealingAnimFX (Variables|Default|GetHUD_Widget)))

(event EventShowDamageWidgetOnce
  ;[1 1 1] Damage, Hitmarker and Heal Widgets
  (Default|TakeDamageFX (Variables|Default|GetHUD_Widget)))

(event EventShowHitMarkerWidget
  (params (ShowInRed? :type Boolean))
  ;[1 1 1] Damage, Hitmarker and Heal Widgets
  (Default|ShowHitMarker (Variables|Default|GetHUD_Widget) ShowInRed?))

(event EventChangeHitMarkerPos
  (params (M4_Optic :type E_Optics%20Enum :default "NewEnumerator0") (PistolActive? :type Boolean) (CantedActive? :type Boolean))
  ;[1 1 1] Damage, Hitmarker and Heal Widgets
  (Default|AdjustHitMarkerPosition (Variables|Default|GetHUD_Widget) M4_Optic CantedActive? PistolActive?))

(event EventChangeHitMarkeronLean
  (params (LeanState :type E_LeanStates%20Enum :default "NewEnumerator0") (Leaning? :type Boolean))
  ;[1 1 1] Damage, Hitmarker and Heal Widgets
  (Default|AdjustHitMarkerLean (Variables|Default|GetHUD_Widget) LeanState Leaning?))

(event EventDayDateTimeWidget
  (params (Visible? :type Boolean) (TimeIn24HrsFormat :type Text) (HoursSinceAttack :type Text) (DateInDigits :type Text) (ShowTimeSinceAttk? :type Boolean))
  (bind _daydatetimewidget_ref (Variables|Default|GetDayDateTimeWidget_Ref))
  ;[1 1 1] Day Date Time Widget
  (if Visible?
    (UserInterface|Viewport|AddtoViewport _daydatetimewidget_ref 0)
    (Default|ShowDateandTime _daydatetimewidget_ref true TimeIn24HrsFormat HoursSinceAttack DateInDigits ShowTimeSinceAttk?)
    (else
      (Widget|RemovefromParent _daydatetimewidget_ref))))

(event EventUpdateHealthWidget
  (params (Health :type Float%20%28double-precision%29))
  ;[1 1 1] Health Widget
  (Default|UpdateHealth (Variables|Default|GetHUD_Widget) Health))

(event EventShowDeathScreen
  ;[1 1 1] Death Screen Widget
  (bind _object (Utilities|AsyncLoadAsset (Variables|Default|GetQuotes_DT))
    (:Completed
      (bind _asdata_table (Utilities|Casting|CastToDataTable _object))
      (bind _returnvalue (Utilities|GetDataTableRow _asdata_table (.OutItem (Utilities|Array|Random (Variables|Default|GetRowNames_DT))))
        (:then
          (Variables|Default|SetDeathQuoteText (Utilities|Struct|BreakS_DeathQuotes _returnvalue)))
        (:RowNotFound
          (Variables|Default|SetDeathQuoteText "\"You are the architect of your own doom\"")))
      (bind _returnvalue_2 (UserInterface|CreateWidget "/Game/_Main/Blueprints/UserInterface/WBP_DeathScreen.WBP_DeathScreen_C" self))
      (bind _output_get (Variables|Default|SetDeathScreen_Widget _returnvalue_2))
      (UserInterface|Viewport|AddtoViewport _output_get 0)
      (Variables|Default|SetbShowMouseCursor true)
      (Input|SetInputModeUIOnly self _output_get "DoNotLock" false)
      (Default|ShowDeathScreen _output_get (Variables|Default|GetDeathQuoteText)))))

(event EventShowFriendlyFireWidget
  (params (Toggle? :type Boolean))
  (bind _friendlyfirewidget (Variables|Default|GetFriendlyFireWidget))
  ;[1 1 1] Friendly Fire Widget
  (if Toggle?
    (Class|BPIntJack|StopFiringExternally(Message) (Game|GetPlayerCharacter 0))
    (UserInterface|Viewport|AddtoViewport _friendlyfirewidget 0)
    (Default|EventFriendlyFireScreen _friendlyfirewidget)
    (Utilities|FlowControl|Delay 0.5)
    (Game|SetGamePaused true)
    (Input|SetInputModeUIOnly self (Variables|Default|GetFriendlyFireWidget) "DoNotLock" false)
    (Variables|Default|SetbShowMouseCursor true)
    (else
      (Utilities|FlowControl|Delay 1.0)
      (Widget|RemovefromParent (Variables|Default|GetFriendlyFireWidget))
      (Input|SetInputModeGameOnly self false)
      (Variables|Default|SetbShowMouseCursor false)
      (Game|SetGamePaused false))))

(event EventShowSavingAnim
  ;[1 1 1] Saving Checkpoint Anim
  (bind _returnvalue (UserInterface|CreateWidget "/Game/_Main/Blueprints/UserInterface/WBP_SavingCheckpoint.WBP_SavingCheckpoint_C" self))
  (UserInterface|Viewport|AddtoViewport _returnvalue 0)
  (Utilities|FlowControl|Delay 8.0)
  (Widget|RemovefromParent _returnvalue))

(event EventDisableSubtitlesforUser
  (params (EnableSubtitles? :type Boolean))
  ;[1 1 1] Subtitle Widget
  (Default|EventDisableSubtitles? (Variables|Default|GetSubtitleWidget) (not EnableSubtitles?)))

(event EventUpdateFOVonPlayer
  (params (NewFOV :type Float%20%28double-precision%29))
  ;[0.2274 0.4635 0.2109] Updating FOV
  (bind _asbp_camera_manager_jack (Utilities|Casting|CastToBP_CameraManager_Jack (Game|GetPlayerCameraManager 0)))
  (Default|UpdateCamFOV _asbp_camera_manager_jack NewFOV) ; clamps b/w 60 and 120
)

(event EventTick
  (params (DeltaSeconds :type Float%20%28single-precision%29))
  ;[1 1 1] Testing/Experimenting
)

(event EventControllerSwitchtoFSR
  (params (DidPlayerSwitch? :type Boolean) (QualityPresetInteger :type Integer))
  ;[1 0.02526 0] FSR3 CRASH HANDLE CODE
  (Variables|Default|SetDidPlayerSwitchToFSR? DidPlayerSwitch?)
  (Variables|Default|SetFSR_Preset_Value QualityPresetInteger))

(event EventControllerUpdateCompass
  ;[1 1 1] Compasss
  (Default|UpdateCompassRot (Variables|Default|GetHUD_Widget)) ; this in turns call the Compass Widget
)

(event EventControllerHideMinimap
  (params (Hide? :type Boolean))
  ;[1 1 1] Hide minimap
  (Default|EventHideMiniMap (Variables|Default|GetHUD_Widget) Hide?))

(event EventCreateInteractPrompt
  (params (Visible? :type Boolean) (InteractKeyImage :type Texture%202D%20Object%20Reference))
  ;[1 1 1] HUD Related
  (Default|ShowInteractMenu (Variables|Default|GetHUD_Widget) Visible? InteractKeyImage))

(event EventUpdateTimeWidget
  (params (Hours :type Integer) (Minutes :type Integer))
  ;[1 1 1] HUD Related
)

(event EventUpdateAmmoWidget
  (params (WidgetVisible? :type Boolean) (DifficultyLevel :type E_GameDifficulty%20Enum :default "NewEnumerator0") (MaxAmmo :type Integer) (CurrentAmmo :type Integer) (MagNumber :type E_MagazineSet%20Enum :default "NewEnumerator0") (Mag1Ammo :type Integer) (Mag2Ammo :type Integer) (Mag3Ammo :type Integer) (PistolActive? :type Boolean))
  ;[1 1 1] HUD Related
  (Default|ShowandUpdateAmmo (Variables|Default|GetHUD_Widget) WidgetVisible? DifficultyLevel MaxAmmo CurrentAmmo MagNumber Mag1Ammo Mag2Ammo Mag3Ammo PistolActive?))

(event EventToggleFPSCounter
  (params (Toggle? :type Boolean))
  ;[1 1 1] FPS Counter
  (Default|EventToggleFPS? (Variables|Default|GetFPS_Widget) (not Toggle?)))

(event EventCreateAttachmentsMenu
  (params (Toggle? :type Boolean) (PistolActive? :type Boolean))
  ;[0.1406 0.09073 0.1242] Create Attachments Menu
  (if Toggle?
    (Utilities|IsValid (Variables|Default|GetAttachments_Widget)
      (:Is%20Valid
        (Default|SetPistolActive (Variables|Default|GetAttachments_Widget) PistolActive?)
        (UserInterface|Viewport|AddtoViewport (Variables|Default|GetAttachments_Widget) 0))
      (:Is%20Not%20Valid
        (bind _returnvalue (UserInterface|CreateWidget "/Game/_Main/Blueprints/UserInterface/WBP_Attachments.WBP_Attachments_C"))
        (bind _output_get (Variables|Default|SetAttachments_Widget _returnvalue))
        (Default|SetPistolActive _output_get PistolActive?)
        (UserInterface|Viewport|AddtoViewport _output_get 0)))
    (Input|SetInputModeUIOnly self (Variables|Default|GetAttachments_Widget) "DoNotLock" false)
    (Variables|Default|SetbShowMouseCursor true)
    (else
      (Widget|RemovefromParent (Variables|Default|GetAttachments_Widget))
      (Input|SetInputModeGameOnly self false)
      (Variables|Default|SetbShowMouseCursor false))))

(event EventCreatePauseMenuWidget
  (params (Toggle? :type Boolean))
  (bind _pausemenu_widget (Variables|Default|GetPauseMenu_Widget))
  ;[0.2917 0.1868 0.1456] Pause Menu
  (bind _output_get (Variables|Default|SetIsGamePaused? Toggle?)) ; Placed here esp for Gamepad \nconnect-disconnect event below\nto prevent overlap
  (Default|EventHideSubtitles (Variables|Default|GetSubtitleWidget) _output_get) ; experimenting this here\ngiving control to PC direclty
  (if Toggle?
    (UserInterface|Viewport|AddtoViewport _pausemenu_widget 0)
    (Input|SetInputModeGameandUI self _pausemenu_widget "DoNotLock" false false)
    (bind _outactors (Actor|GetAllActorswithTag "Soundtrack"))
    (for _array_element _outactors
      (Class|BPIntActorProps|SoundtrackPlayerPauseMenu(Message) _array_element true))
    (Variables|Default|SetbShowMouseCursor true)
    (Utilities|FlowControl|Delay 2.0)
    (Game|SetGamePaused true)
    (else
      (Default|EventonPauseMenuRemoved _pausemenu_widget)
      (Utilities|FlowControl|Delay 0.5)
      (Widget|RemovefromParent _pausemenu_widget)
      (Input|SetInputModeGameOnly self false)
      (Variables|Default|SetbShowMouseCursor false)
      (bind _outactors_2 (Actor|GetAllActorswithTag "Soundtrack"))
      (for _array_element_2 _outactors_2
        (Class|BPIntActorProps|SoundtrackPlayerPauseMenu(Message) _array_element_2 false))
      (Utilities|FlowControl|Delay 1.5)
      (Game|SetGamePaused false)
      (CallFunction|EventCheckandSetFSR3))))

(event EventCreateSubtitleWidget
  (params (CharacterName :type E_CharacterNames%20Enum :default "NewEnumerator0") (SubtitleText :type Text) (AudioDuration :type Float%20%28double-precision%29))
  ;[1 1 1] Subtitle Widget
  (Default|EventUpdateSubtitleText (Variables|Default|GetSubtitleWidget) CharacterName SubtitleText AudioDuration) ; custom event inside HUD Widget
)

(fn ConstructionScript)

(fn JackGetFollowCam
  (return 0))

(fn SetDesiredOptic
  (return "NewEnumerator0"))