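; BP_TowerStation_Plank is a ladder-related tower station plank that tells characters when they enter or leave its trigger Box.
; Box begin and end overlaps send a true or false ladder-state message, using actor tags to pick the player message for "Jack" or the NPC message for "NPC".
; The vehicle seat, trunk arrow, name/location and player-dependent light functions are stubs returning defaults, and the construction script is empty.
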(event OnComponentBeginOverlap(Box)
  (params (OverlappedComponent :type Primitive%20Component%20Object%20Reference) (OtherActor :type Actor%20Object%20Reference) (OtherComp :type Primitive%20Component%20Object%20Reference) (OtherBodyIndex :type Integer) (bFromSweep :type Boolean) (SweepResult :type Hit%20Result%20Structure%20%28by%20ref%29))
  (if (Actor|ActorHasTag OtherActor "Jack")
    (Class|BPIntJack|PlayeronLadder(Message) OtherActor true)
    (elif (Actor|ActorHasTag OtherActor "NPC")
      (Class|BPIntNPC|NPCLadderState(Message) OtherActor true))))

(event OnComponentEndOverlap(Box)
  (params (OverlappedComponent :type Primitive%20Component%20Object%20Reference) (OtherActor :type Actor%20Object%20Reference) (OtherComp :type Primitive%20Component%20Object%20Reference) (OtherBodyIndex :type Integer))
  (if (Actor|ActorHasTag OtherActor "Jack")
    (Class|BPIntJack|PlayeronLadder(Message) OtherActor false)
    (elif (Actor|ActorHasTag OtherActor "NPC")
      (Class|BPIntNPC|NPCLadderState(Message) OtherActor false))))

(fn ConstructionScript)

(fn FetchArrowsfromVehicles
  (params (Seat :type E_VehicleSeat%20Enum :default "NewEnumerator0"))
  (return "0, 0, 0" "0, 0, 0"))

(fn GetVehicleNameandLoc
  (return "NewEnumerator0" "0, 0, 0"))

(fn ObtainTrunkArrowsPickup
  (params (Seat%281-6%29 :type Integer))
  (return "0, 0, 0" "0, 0, 0"))

(fn PlayerDependentLight?
  (return false))