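; Configurable swinging door that the player opens by interacting and NPCs open automatically, with sound, a panel material change and optional timed auto-close.
; Front and back overlap boxes set the swing direction while the door is closed and toggle the player's interact prompt.
; A FlipFlop plays or reverses a timeline that rotates the door from its placed yaw, guarded against mid-swing triggers.
; The construction script configures panel and handles.
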(event OnComponentBeginOverlap(BoxCollisionFront)
  (params (OverlappedComponent :type Primitive%20Component%20Object%20Reference) (OtherActor :type Actor%20Object%20Reference) (OtherComp :type Primitive%20Component%20Object%20Reference) (OtherBodyIndex :type Integer) (bFromSweep :type Boolean) (SweepResult :type Hit%20Result%20Structure%20%28by%20ref%29))
  ;[0.2292 0.09774 0.09546] In and Out decider
  ; + Auto Open for NPCs
  (if (Actor|ActorHasTag OtherActor "Jack")
    (if (not (Variables|Default|GetPlayerNotAllowed?))
      (Utilities|DoorRotationState?
        (:DoorClosed
          (Variables|Default|SetInOrOut 1.0)
          (Class|BPIntJack|ToggleInteractPromptPlayer(Message) OtherActor true))))
    (elif (Actor|ActorHasTag OtherActor "NPC")
      (Utilities|DoorRotationState?
        (:DoorClosed
          (Variables|Default|SetInOrOut 1.0)
          (CallFunction|DoorOpenClose))))))

(event OnComponentBeginOverlap(BoxCollisionBack)
  (params (OverlappedComponent :type Primitive%20Component%20Object%20Reference) (OtherActor :type Actor%20Object%20Reference) (OtherComp :type Primitive%20Component%20Object%20Reference) (OtherBodyIndex :type Integer) (bFromSweep :type Boolean) (SweepResult :type Hit%20Result%20Structure%20%28by%20ref%29))
  ;[0.2292 0.09774 0.09546] In and Out decider
  ; + Auto Open for NPCs
  (if (Actor|ActorHasTag OtherActor "Jack")
    (if (not (Variables|Default|GetPlayerNotAllowed?))
      (Utilities|DoorRotationState?
        (:DoorClosed
          (Variables|Default|SetInOrOut -1.0)
          (Class|BPIntJack|ToggleInteractPromptPlayer(Message) OtherActor true))))
    (elif (Actor|ActorHasTag OtherActor "NPC")
      (Utilities|DoorRotationState?
        (:DoorClosed
          (Variables|Default|SetInOrOut -1.0)
          (CallFunction|DoorOpenClose))))))

(event OnComponentEndOverlap(BoxCollisionFront)
  (params (OverlappedComponent :type Primitive%20Component%20Object%20Reference) (OtherActor :type Actor%20Object%20Reference) (OtherComp :type Primitive%20Component%20Object%20Reference) (OtherBodyIndex :type Integer))
  (Class|BPIntJack|ToggleInteractPromptPlayer(Message) OtherActor false))

(event OnComponentEndOverlap(BoxCollisionBack)
  (params (OverlappedComponent :type Primitive%20Component%20Object%20Reference) (OtherActor :type Actor%20Object%20Reference) (OtherComp :type Primitive%20Component%20Object%20Reference) (OtherBodyIndex :type Integer))
  (Class|BPIntJack|ToggleInteractPromptPlayer(Message) OtherActor false))

(event Custom|DoorAutomaticClose
  (bind _zaxisrotation_old (Variables|Default|GetZAxisRotation_Old))
  ;[0.03646 0.03646 0.03646 1 12] Auto Close
  (Utilities|DoorRotationState?
    (:DoorClosed
      (Utilities|Time|ClearandInvalidateTimerbyHandle (Variables|Default|GetDoorAutoCloseTimer)) ; necessary
    )
    (:DoorOpen
      (Utilities|FlowControl|FlipFlop
        (:A
          (Audio|PlaySoundatLocation (select (Variables|Default|GetIsWoodenDoor?) "/Game/_Main/Sounds/Doors/WoodenDoor_Open.WoodenDoor_Open" (Utilities|Select :Index (Variables|Default|GetMetalSoundIndex_Open) :Option%200 "/Game/_Main/Sounds/Doors/MetalDoor_Open_1.MetalDoor_Open_1" :Option%201 "/Game/_Main/Sounds/Doors/MetalDoor_Open_2.MetalDoor_Open_2" :Option%202 "/Game/_Main/Sounds/Doors/MetalDoor_Open_3.MetalDoor_Open_3")) (Transformation|GetActorLocation) "0, 0, 0" 1.0 1.0 0.0 "/Game/_Main/Sounds/Doors/DoorSoundAttentuation.DoorSoundAttentuation" 0 0 0) ; Door Open Sound
          (Variables|Default|SetDoorClosing? false)
          ;[0 0 0] Animation
          (bind _dooralpha (Timeline|DoorAnimFw PlayFromStart) ; 0 to 1 in 1.5seconds
            (:Update
              (Variables|Default|SetTimelineAlpha _dooralpha)
              (Transformation|SetRelativeRotation (Variables|Default|GetDoorMesh) (Math|Rotator|MakeRotator 0.0 0.0 (Math|Float|Lerp (.yaw _zaxisrotation_old) (+ (.yaw _zaxisrotation_old) (* (Variables|Default|GetInOrOut) (Variables|Default|GetDoorAngle))) _dooralpha)) false false)
              ;[0.1727 0.3012 0.3073 1 14] Updating Panel Material
              (Rendering|Material|SetMaterial (Variables|Default|GetPanelMesh) 0 "/Game/_Main/Assets/Annexe/Props/Panel/Mat/MI_Panel_True.MI_Panel_True")
              (if (Variables|Default|GetAutoCloseEnable?) ; Toggle
                (bind _returnvalue (Utilities|Time|SetTimerbyEvent (delegate Custom|DoorAutomaticClose) (Variables|Default|GetAutoCloseTimer))) ; how much to wait
                (Variables|Default|SetDoorAutoCloseTimer _returnvalue)))
            (:Finished
              ;[0.1875 0.1875 0.1875] Panel Material switch after door anim
              (Rendering|Material|SetMaterial (Variables|Default|GetPanelMesh) 0 "/Game/_Main/Assets/Annexe/Props/Panel/Mat/Panel_Mat.Panel_Mat")
              (if (Variables|Default|GetDoorClosing?)
                (Audio|PlaySoundatLocation (select (Variables|Default|GetIsWoodenDoor?) "/Game/_Main/Sounds/Doors/WoodenDoor_Close.WoodenDoor_Close" (Utilities|Select :Index (Variables|Default|GetMetalSoundIndex_Close) :Option%200 "/Game/_Main/Sounds/Doors/MetalDoor_Close_1.MetalDoor_Close_1" :Option%201 "/Game/_Main/Sounds/Doors/MetalDoor_Close_2.MetalDoor_Close_2" :Option%202 "/Game/_Main/Sounds/Doors/MetalDoor_Close_3.MetalDoor_Close_3")) (Transformation|GetActorLocation) "0, 0, 0" 1.0 1.0 0.0 "/Game/_Main/Sounds/Doors/DoorSoundAttentuation.DoorSoundAttentuation" 0 0 0) ; Door Closing Sound
                (Variables|Default|SetDoorClosing? false)))))
        (:B
          (Variables|Default|SetDoorClosing? true)
          (Timeline|DoorAnimFw ReverseFromEnd))))))

(event Custom|DoorOpenClose
  (bind _zaxisrotation_old (Variables|Default|GetZAxisRotation_Old))
  (if (not (== (Variables|Default|GetInOrOut) 0.0)) ; Prevents hitching when\nyou suddenly enter collision\nbox to tell orientation
    ;[0.1146 0.1146 0.1146 1 14] Premature Cancel avoidance
    (if (Utilities|Time|IsTimerActivebyHandle (Variables|Default|GetDoorAutoCloseTimer))
      (Utilities|Time|ClearandInvalidateTimerbyHandle (Variables|Default|GetDoorAutoCloseTimer)))
    (if (== (Variables|Default|GetTimelineAlpha) 0.0) ; prevents premature cancellation
      (Utilities|FlowControl|FlipFlop :!label _label
        (:A
          (Audio|PlaySoundatLocation (select (Variables|Default|GetIsWoodenDoor?) "/Game/_Main/Sounds/Doors/WoodenDoor_Open.WoodenDoor_Open" (Utilities|Select :Index (Variables|Default|GetMetalSoundIndex_Open) :Option%200 "/Game/_Main/Sounds/Doors/MetalDoor_Open_1.MetalDoor_Open_1" :Option%201 "/Game/_Main/Sounds/Doors/MetalDoor_Open_2.MetalDoor_Open_2" :Option%202 "/Game/_Main/Sounds/Doors/MetalDoor_Open_3.MetalDoor_Open_3")) (Transformation|GetActorLocation) "0, 0, 0" 1.0 1.0 0.0 "/Game/_Main/Sounds/Doors/DoorSoundAttentuation.DoorSoundAttentuation" 0 0 0) ; Door Open Sound
          (Variables|Default|SetDoorClosing? false)
          ;[0 0 0] Animation
          (bind _dooralpha (Timeline|DoorAnimFw PlayFromStart) ; 0 to 1 in 1.5seconds
            (:Update
              (Variables|Default|SetTimelineAlpha _dooralpha)
              (Transformation|SetRelativeRotation (Variables|Default|GetDoorMesh) (Math|Rotator|MakeRotator 0.0 0.0 (Math|Float|Lerp (.yaw _zaxisrotation_old) (+ (.yaw _zaxisrotation_old) (* (Variables|Default|GetInOrOut) (Variables|Default|GetDoorAngle))) _dooralpha)) false false)
              ;[0.1727 0.3012 0.3073 1 14] Updating Panel Material
              (Rendering|Material|SetMaterial (Variables|Default|GetPanelMesh) 0 "/Game/_Main/Assets/Annexe/Props/Panel/Mat/MI_Panel_True.MI_Panel_True")
              ;[0.03646 0.03646 0.03646 1 12] Auto Close
              (if (Variables|Default|GetAutoCloseEnable?) ; Toggle
                (bind _returnvalue (Utilities|Time|SetTimerbyEvent (delegate Custom|DoorAutomaticClose) (Variables|Default|GetAutoCloseTimer))) ; how much to wait
                (Variables|Default|SetDoorAutoCloseTimer _returnvalue)))
            (:Finished
              ;[0.1875 0.1875 0.1875] Panel Material switch after door anim
              (Rendering|Material|SetMaterial (Variables|Default|GetPanelMesh) 0 "/Game/_Main/Assets/Annexe/Props/Panel/Mat/Panel_Mat.Panel_Mat")
              (if (Variables|Default|GetDoorClosing?)
                (Audio|PlaySoundatLocation (select (Variables|Default|GetIsWoodenDoor?) "/Game/_Main/Sounds/Doors/WoodenDoor_Close.WoodenDoor_Close" (Utilities|Select :Index (Variables|Default|GetMetalSoundIndex_Close) :Option%200 "/Game/_Main/Sounds/Doors/MetalDoor_Close_1.MetalDoor_Close_1" :Option%201 "/Game/_Main/Sounds/Doors/MetalDoor_Close_2.MetalDoor_Close_2" :Option%202 "/Game/_Main/Sounds/Doors/MetalDoor_Close_3.MetalDoor_Close_3")) (Transformation|GetActorLocation) "0, 0, 0" 1.0 1.0 0.0 "/Game/_Main/Sounds/Doors/DoorSoundAttentuation.DoorSoundAttentuation" 0 0 0) ; Door Closing Sound
                (Variables|Default|SetDoorClosing? false)))))
        (:B
          (Variables|Default|SetDoorClosing? true)
          (Timeline|DoorAnimFw ReverseFromEnd)))
      (elif (== (Variables|Default|GetTimelineAlpha) 1.0) ; yeah this too
        (goto _label)))))

(event EventBeginPlay
  (Variables|Default|SetZAxisRotation_Old (Variables|/Script/Engine.SceneComponent|GetRelativeRotation (Variables|Default|GetDoorMesh))))

(event EventInteractwithActor
  (if (not (Variables|Default|GetPlayerNotAllowed?))
    (CallFunction|DoorOpenClose)))

(fn ConstructionScript
  (bind _panelmesh (Variables|Default|GetPanelMesh))
  (bind _doorhandlef (Variables|Default|GetDoorHandleF))
  (bind _doorhandleb (Variables|Default|GetDoorHandleB))
  ;[0.2031 0.2031 0.2031] Panel
  (Transformation|SetRelativeLocationAndRotation _panelmesh (Variables|Default|GetPanelLocation) (Variables|Default|GetPanelRotation) false false)
  (Transformation|SetRelativeScale3D _panelmesh (Variables|Default|GetPanelScale))
  (Rendering|SetVisibility _panelmesh (Variables|Default|GetPanelVisible?) true)
  ;[0.4635 0.4094 0.3254] Door Handles
  (Components|StaticMesh|SetStaticMesh _doorhandlef (Variables|Default|GetHandleFront))
  (Components|StaticMesh|SetStaticMesh _doorhandleb (Variables|Default|GetHandleBack))
  (Transformation|SetRelativeLocation _doorhandlef (Variables|Default|GetFrontHandleLoc) false false)
  (Transformation|SetRelativeRotation _doorhandlef (Variables|Default|GetFrontHandleRot) false false)
  (Transformation|SetRelativeLocation _doorhandleb (Variables|Default|GetBackHandleLoc) false false)
  (Transformation|SetRelativeRotation _doorhandleb (Variables|Default|GetBackHandleRot) false false))

(fn FetchArrowsfromVehicles
  (params (Seat :type E_VehicleSeat%20Enum :default "NewEnumerator0"))
  (return "0, 0, 0" "0, 0, 0"))

(fn GetVehicleNameandLoc
  (return "NewEnumerator0" "0, 0, 0" "0, 0, 0"))

(fn IsVehicleMoving?
  (return false))

(fn JackGetFollowCam
  (return 0))

(fn ObtainTrunkArrowsPickup
  (params (Seat%281-6%29 :type Integer))
  (return "0, 0, 0" "0, 0, 0"))

(fn PlayerDependentLight?
  (return false))

(fn SetDesiredOptic
  (return "NewEnumerator0"))