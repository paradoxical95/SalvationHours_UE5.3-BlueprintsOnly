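; Mortar shell actor that flies along a referenced spline and explodes at the end of its path.
; LaunchProjectileMortar plays a timeline scaled by TimeToTravel, setting location and yaw-offset rotation from the spline.
; On finish it applies radial falloff damage, plays a sound and selected explosion effect, hides the mesh and destroys itself after a delay.
; The decal spawn is unconnected, and the vehicle-related functions are empty stubs.
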(event EventLaunchProjectileMortar
  (bind _splineref (Variables|Default|GetSplineRef))
  (bind _spline (Variables|/Game/_Main/Blueprints/Vehicles/BP_Spline_Vehicle.BP_Spline_Vehicle_C|GetSpline _splineref))
  (Components|Activation|Activate (Variables|Default|GetSmokeFX) false)
  (Components|Timeline|SetPlayRate (Variables|Default|GetTimelineMoveMortarProjectile) (/ 1.0 (Variables|Default|GetTimeToTravel))) ; How fast
  (bind _float (Timeline|TimelineMoveMortarProjectile PlayFromStart)
    (:Update
      (Transformation|SetActorTransform (Math|Transform|MakeTransform (.location (Spline|GetTransformatDistanceAlongSpline _spline (Math|Float|Lerp 0.0 (Spline|GetSplineLength _spline) _float) "World" false)) (Math|Rotator|MakeRotator (.Roll (Math|Rotator|BreakRotator (Spline|GetRotationatDistanceAlongSpline _spline (Math|Float|Lerp 0.0 (Spline|GetSplineLength _spline) _float) "Local"))) (.Pitch (Math|Rotator|BreakRotator (Spline|GetRotationatDistanceAlongSpline _spline (Math|Float|Lerp 0.0 (Spline|GetSplineLength _spline) _float) "Local"))) (+ (.Yaw (Math|Rotator|BreakRotator (Spline|GetRotationatDistanceAlongSpline _spline (Math|Float|Lerp 0.0 (Spline|GetSplineLength _spline) _float) "Local"))) (Variables|Default|GetOffset_Z_RotationSpline))) "1.000000,1.000000,1.000000")))
    (:Finished
      (Class|GameplayStatics|ApplyRadialDamagewithFalloff 105.0 85.0 (.location (Spline|GetTransformatDistanceAlongSpline _spline (Math|Float|Lerp 0.0 (Spline|GetSplineLength _spline) _float) "World" false)) 1.5e+02 6e+02 1.0 0 0 self 0 "ECC_Visibility")
      (Audio|PlaySoundatLocation "/Game/Warfare_SFX_Bundle/Explosion_Sounds_Pro/Wavs/Explosion_C4_01.Explosion_C4_01" (.location (Spline|GetTransformatDistanceAlongSpline _spline (Math|Float|Lerp 0.0 (Spline|GetSplineLength _spline) _float) "World" false)) "0, 0, 0" 2.0 1.0 0.0 "/Game/_Main/Blueprints/NPCs/AudioFX/ExplosionAttenuation.ExplosionAttenuation" 0 0 0)
      (Niagara|SpawnSystematLocation (Utilities|Select :Index (Variables|Default|GetExplosionFX_Int) :Option%200 "/Game/M5VFXVOL2/Niagara/Explosion/NFire_Exp_00.NFire_Exp_00" :Option%201 "/Game/M5VFXVOL2/Niagara/Explosion/NFire_Exp_01.NFire_Exp_01" :Option%202 "/Game/M5VFXVOL2/Niagara/Explosion/NFire_Exp_03.NFire_Exp_03") (.location (Spline|GetTransformatDistanceAlongSpline _spline (Math|Float|Lerp 0.0 (Spline|GetSplineLength _spline) _float) "World" false)) "0, 0, 0" "1.500000,1.500000,1.500000")
      (Rendering|SetVisibility (Variables|Default|GetStaticMesh) false false)
      (Utilities|FlowControl|Delay 5.0)
      (Actor|DestroyActor))))

(fn ConstructionScript)

(fn FetchArrowsfromVehicles
  (params (Seat :type E_VehicleSeat%20Enum :default "NewEnumerator0"))
  (return "0, 0, 0" "0, 0, 0"))

(fn GetVehicleNameandLoc
  (return "NewEnumerator0" "0, 0, 0" "0, 0, 0"))

(fn IsVehicleMoving?
  (return false))

(fn ObtainTrunkArrowsPickup
  (params (Seat%281-6%29 :type Integer))
  (return "0, 0, 0" "0, 0, 0"))

(fn PlayerDependentLight?
  (return false))