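; Fire hazard actor that switches a randomly chosen Niagara fire effect, fading audio and a point light on or off, and damages the player.
; ActivateFireSMC also randomizes actor scale and sets a looping timer, whichever way it toggles.
; The timer applies periodic damage while the fire is active and the "Jack"-tagged actor is inside the collision sphere.
; Vehicle and light query functions are stubs returning defaults.
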(event OnComponentBeginOverlap(SphereCollision)
  (params (OverlappedComponent :type Primitive%20Component%20Object%20Reference) (OtherActor :type Actor%20Object%20Reference) (OtherComp :type Primitive%20Component%20Object%20Reference) (OtherBodyIndex :type Integer) (bFromSweep :type Boolean) (SweepResult :type Hit%20Result%20Structure%20%28by%20ref%29))
  (if (Actor|ActorHasTag OtherActor "Jack")
    (Variables|Default|SetPlayerInRadius? true)
    (Variables|Default|SetJackRef OtherActor)))

(event OnComponentEndOverlap(SphereCollision)
  (params (OverlappedComponent :type Primitive%20Component%20Object%20Reference) (OtherActor :type Actor%20Object%20Reference) (OtherComp :type Primitive%20Component%20Object%20Reference) (OtherBodyIndex :type Integer))
  (if (Actor|ActorHasTag OtherActor "Jack")
    (Variables|Default|SetPlayerInRadius? false)))

(event Custom|DamageByFire
  (bind _jackref (Variables|Default|GetJackRef))
  (if (and (Variables|Default|GetIsFireActive?) (Variables|Default|GetPlayerInRadius?))
    (Utilities|IsValid _jackref
      (:Is%20Valid
        (Game|Damage|ApplyDamage _jackref 3.0 0 self)))))

(event EventActivateFireSMC
  (params (Toggle? :type Boolean))
  (bind _returnvalue (Math|Random|RandomFloatinRange 0.5 1.25))
  (bind _fireeffect (Variables|Default|GetFireEffect))
  (bind _audio (Variables|Default|GetAudio))
  (Class|NiagaraComponent|SetAsset (Variables|Default|GetFireEffect) (Utilities|Array|Get(acopy) (Variables|Default|GetEffect_Type) (Math|Random|RandomIntegerinRange 0 8)) true)
  (if Toggle?
    (Audio|Components|Audio|FadeIn _audio 1.0 1.0 0.0 "Linear" :!class /Script/Engine.AudioComponent)
    (Components|Activation|Activate _fireeffect true)
    (Variables|Default|SetIsFireActive? true)
    (else
      (Audio|Components|Audio|FadeOut _audio 1.0 0.0 "Linear" :!class /Script/Engine.AudioComponent)
      (Components|Activation|Deactivate _fireeffect)
      (Variables|Default|SetIsFireActive? false)))
  (Rendering|SetVisibility (Variables|Default|GetPointLight) Toggle? false)
  (Transformation|SetActorScale3D (Math|Vector|MakeVector _returnvalue _returnvalue _returnvalue))
  (bind _returnvalue_2 (Utilities|Time|SetTimerbyEvent (delegate Custom|DamageByFire) 2.0 true))
  (Variables|Default|SetTimer _returnvalue_2))

(fn ConstructionScript)

(fn FetchArrowsfromVehicles
  (params (Seat :type E_VehicleSeat%20Enum :default "NewEnumerator0"))
  (return "0, 0, 0" "0, 0, 0"))

(fn GetVehicleNameandLoc
  (return "NewEnumerator0" "0, 0, 0" "0, 0, 0"))

(fn IsVehicleMoving?
  (return false))

(fn ObtainTrunkArrowsPickup
  (params (Seat%281-6%29 :type Integer))
  (return "0, 0, 0" "0, 0, 0"))

(fn PlayerDependentLight?
  (return false))