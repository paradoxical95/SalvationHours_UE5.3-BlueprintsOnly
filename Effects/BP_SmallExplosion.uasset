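; Small bomb explosion effect actor that plays its visuals and sound, then removes itself.
; StartSmallBombExplosion fires the explosion effect and audio together, activates smoke after a short delay, then destroys the actor after a further delay.
; The vehicle seat, arrow, movement and light query functions are empty stubs returning default values and play no part in the effect.
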(event EventStartSmallBombExplosion
  (Components|Activation|Activate (Variables|Default|GetExplosion) false)
  (Audio|Components|Audio|Play (Variables|Default|GetAudio) 0.0)
  (Utilities|FlowControl|Delay 1.0)
  (Components|Activation|Activate (Variables|Default|GetSmoke) false)
  (Utilities|FlowControl|Delay 2.0)
  (Actor|DestroyActor))

(fn ConstructionScript)

(fn FetchArrowsfromVehicles
  (params (Seat :type E_VehicleSeat%20Enum :default "NewEnumerator0"))
  (return "0, 0, 0" "0, 0, 0"))

(fn GetVehicleNameandLoc
  (return "NewEnumerator0" "0, 0, 0" "0, 0, 0"))

(fn IsVehicleMoving?
  (return false))

(fn ObtainTrunkArrowsPickup
  (params (Seat%281-6%29 :type Integer))
  (return "0, 0, 0" "0, 0, 0"))

(fn PlayerDependentLight?
  (return false))