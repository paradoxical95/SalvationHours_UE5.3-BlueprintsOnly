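; Soundtrack actor that plays the game's music, switching between main theme, chapter and other tracks, plus a pause menu theme.
; The SoundtrackList selection picks a sound asset, which is async-loaded into the Audio component.
; Events toggle playback, change tracks (intended for GameInstance chapter updates) and swap the pause theme in and out.
; Transitions use fades and delays, often starting at randomized offsets, with IsSoundtrackPlaying tracking whether to resume.
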(event EventBeginPlay
  (Variables|/Script/Engine.AudioComponent|SetbAllowSpatialization (Variables|Default|GetAudio) (Variables|Default|GetAllowSpatialization?))
  (bind _output_get (Variables|Default|SetSoundAsset (Utilities|MFetchSoundtrack)))
  (bind _object (Utilities|AsyncLoadAsset _output_get)
    (:Completed
      (bind _assound_wave (Utilities|Casting|CastToSoundWave _object))
      (Audio|Components|Audio|SetSound (Variables|Default|GetAudio) _assound_wave)
      (if (Variables|Default|GetAutoActivate?)
        (Audio|Components|Audio|FadeIn (Variables|Default|GetAudio) 0.0 1.0 0.0 "Linear" :!class /Script/Engine.AudioComponent)
        (Variables|Default|SetIsSoundtrackPlaying? true)
        (else
          (Variables|Default|SetIsSoundtrackPlaying? false))))))

(event EventSoundtrackPlayerPauseMenu
  (params (TogglePauseMenuTheme? :type Boolean))
  (bind _audio (Variables|Default|GetAudio))
  (bind _audio_2 (Variables|Default|GetAudio))
  ;[1 1 1] Pause Menu Code
  (if TogglePauseMenuTheme?
    (if (Variables|Default|GetIsSoundtrackPlaying?)
      (Audio|Components|Audio|FadeOut (Variables|Default|GetAudio) 1.0 0.0 "Linear" :!class /Script/Engine.AudioComponent)
      (Utilities|FlowControl|Delay 1.0))
    (bind _output_get (Variables|Default|SetSoundAsset "/Game/_Main/MusicTracks/PauseMenuTheme_Trimmed.PauseMenuTheme_Trimmed"))
    (bind _object (Utilities|AsyncLoadAsset _output_get)
      (:Completed
        (bind _assound_wave (Utilities|Casting|CastToSoundWave _object))
        (Audio|Components|Audio|SetSound _audio_2 _assound_wave)
        (Audio|Components|Audio|FadeIn _audio_2 1.0 0.5 (Math|Random|RandomFloatinRange 2.0 14.0) "Linear" :!class /Script/Engine.AudioComponent)
        (Audio|Components|Audio|SetVolumeMultiplier _audio_2 0.75 :!class /Script/Engine.AudioComponent)))
    (else
      (Audio|Components|Audio|FadeOut (Variables|Default|GetAudio) 1.0 0.0 "Linear" :!class /Script/Engine.AudioComponent)
      (Utilities|FlowControl|Delay 1.0)
      (bind _output_get_2 (Variables|Default|SetSoundAsset (Utilities|MFetchSoundtrack)))
      (bind _object_2 (Utilities|AsyncLoadAsset _output_get_2)
        (:Completed
          (bind _assound_wave_2 (Utilities|Casting|CastToSoundWave _object_2))
          (Audio|Components|Audio|SetSound _audio _assound_wave_2)
          (if (Variables|Default|GetIsSoundtrackPlaying?)
            (Audio|Components|Audio|FadeIn _audio 1.0 1.0 (Math|Random|RandomFloatinRange 2.0 12.0) "Linear" :!class /Script/Engine.AudioComponent)))))))

(event EventSoundtrackPlayerSetNewSound
  (params (WhichTrack :type E_SoundtrackList%20Enum :default "NewEnumerator12") (PlayAfterChange? :type Boolean))
  (bind _fadeduration (Variables|Default|GetFadeDuration))
  ;[1 1 1] Change Track and Play
  (Variables|Default|SetSoundtrackList WhichTrack)
  (if (Variables|Default|GetIsSoundtrackPlaying?)
    (Audio|Components|Audio|FadeOut (Variables|Default|GetAudio) _fadeduration 0.0 "Linear" :!class /Script/Engine.AudioComponent)
    (Utilities|FlowControl|Delay _fadeduration))
  (bind _output_get (Variables|Default|SetSoundAsset (Utilities|MFetchSoundtrack)))
  (bind _object (Utilities|AsyncLoadAsset _output_get)
    (:Completed
      (bind _assound_wave (Utilities|Casting|CastToSoundWave _object))
      (Audio|Components|Audio|SetSound (Variables|Default|GetAudio) _assound_wave)
      (Development|PrintString "New Soundtrack Set" true true "(R=1.000000,G=0.176134,B=0.000000,A=1.000000)")
      (if PlayAfterChange?
        (Audio|Components|Audio|FadeIn (Variables|Default|GetAudio) (Variables|Default|GetFadeDuration) 1.0 (Math|Random|RandomFloatinRange 1.0 6.0) "Linear" :!class /Script/Engine.AudioComponent)
        (Variables|Default|SetIsSoundtrackPlaying? true)
        (else
          (Variables|Default|SetIsSoundtrackPlaying? false))))))

(event EventSoundtrackPlayerToggleSound
  (params (Play? :type Boolean))
  (bind _fadeduration (Variables|Default|GetFadeDuration))
  (bind _audio (Variables|Default|GetAudio))
  ;[1 1 1] Only Play/Pause Track
  (if Play?
    (if (not (Audio|Components|Audio|IsPlaying _audio))
      (Audio|Components|Audio|FadeIn _audio _fadeduration 1.0 0.0 "Linear" :!class /Script/Engine.AudioComponent)
      (Variables|Default|SetIsSoundtrackPlaying? true))
    (elif (Audio|Components|Audio|IsPlaying _audio)
      (Audio|Components|Audio|FadeOut _audio _fadeduration 0.0 "Linear" :!class /Script/Engine.AudioComponent)
      (Variables|Default|SetIsSoundtrackPlaying? false))))

(fn ConstructionScript)

(fn FetchArrowsfromVehicles
  (params (Seat :type E_VehicleSeat%20Enum :default "NewEnumerator0"))
  (return "0, 0, 0" "0, 0, 0"))

(fn GetVehicleNameandLoc
  (return "NewEnumerator0" "0, 0, 0"))

(fn ObtainTrunkArrowsPickup
  (params (Seat%281-6%29 :type Integer))
  (return "0, 0, 0" "0, 0, 0"))

(fn PlayerDependentLight?
  (return false))