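; Ambient gunfire sound actor that plays distant-combat audio only during certain story segments.
; On BeginPlay a looping timer fires every few seconds and, if the Play flag is set, queries the GameInstance for the current chapter and segment.
; The Audio component restarts only in one chapter and four specific CH4 segments.
; A SetLifeSpan call exists but is never executed.
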(event Custom|PlayAmbientGunfire
  (if (Variables|Default|GetPlay?)
    (bind _chsegstruct (Class|BPIntGameInstance|GIFetchChapterSegment(Message) (Game|GetGameInstance)))
    (if (Utilities|Enum|Equal(Enum) (.ChapterNumber? (Utilities|Struct|BreakS_ChapterSegmentData _chsegstruct)) "NewEnumerator3")
      (if (Math|Boolean|ORBoolean (Utilities|Enum|Equal(Enum) (.CH4_Segment (Utilities|Struct|BreakS_ChapterSegmentData _chsegstruct)) "NewEnumerator10") (Utilities|Enum|Equal(Enum) (.CH4_Segment (Utilities|Struct|BreakS_ChapterSegmentData _chsegstruct)) "NewEnumerator11") (Utilities|Enum|Equal(Enum) (.CH4_Segment (Utilities|Struct|BreakS_ChapterSegmentData _chsegstruct)) "NewEnumerator12") (Utilities|Enum|Equal(Enum) (.CH4_Segment (Utilities|Struct|BreakS_ChapterSegmentData _chsegstruct)) "NewEnumerator13"))
        (Audio|Components|Audio|Play (Variables|Default|GetAudio) 0.0)))))

(event EventBeginPlay
  (Utilities|Time|SetTimerbyEvent (delegate Custom|PlayAmbientGunfire) 3.0 true))

(fn ConstructionScript)